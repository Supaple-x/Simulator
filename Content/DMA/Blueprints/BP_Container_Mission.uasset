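; BP_Container_Mission is a mission path container that owns navigation points, a spawned BP_Moving_Actor with a child drone, and a timeline widget.
; It derives point enter times from distance, speed and waits; retiming a point clamps against neighbors and adjusts segment speeds.
; Scrubbing linearly interpolates position between points by time.
; Parent overrides propagate highlighting, color, visibility, pause, danger-zone updates and removal to points, actor, widget or shared dynamic material.
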(event EventBeginPlay
  (bind _returnvalue (Game|SpawnActorfromClass "/Game/DMA/Blueprints/Core/BP_Moving_Actor.BP_Moving_Actor_C" (Math|Transform|MakeTransform "0, 0, 0" "0, 0, 0" "1,1,1") "AlwaysSpawn" 0 0))
  (Variables|/Game/DMA/Blueprints/Core/BP_Moving_Actor.BP_Moving_Actor_C|SetAttachedToContainer _returnvalue self)
  (Variables|Default|SetMovingActor _returnvalue)
  (bind _returnvalue_2 (Rendering|Material|CreateDynamicMaterialInstance "/Game/DMA/MaterialLibrary/M_Metal_Brushed_Nickel.M_Metal_Brushed_Nickel" "None" :!class /Script/Engine.KismetMaterialLibrary))
  (Variables|Default|SetPathMaterialInstance _returnvalue_2))

(event Collision|EventActorBeginOverlap
  (params (OtherActor :type Actor%20Object%20Reference)))

(event EventTick
  (params (DeltaSeconds :type Float%20%28single-precision%29)))

(fn ConstructionScript)

(fn UpdateFirstLastPoint
  (bind _navipointsactors (Variables|Default|GetNaviPointsActors))
  (for (_array_element _array_index) _navipointsactors
    (if (== _array_index 0)
      (Default|SetFirst _array_element)
      (elif (== _array_index (Utilities|Array|LastIndex _navipointsactors))
        (Default|SetLast _array_element)
        (else
          (Default|SetNormal _array_element))))))

(fn CalculatePointsTimes
  (bind _navipointsactors (Variables|Default|GetNaviPointsActors))
  (bind _navipointsactors_2 (Variables|Default|GetNaviPointsActors))
  (if (Utilities|Array|IsValidIndex (Variables|Default|GetNaviPointsActors))
    (Variables|/Game/DMA/Blueprints/BP_Point_Mission.BP_Point_Mission_C|SetEnterTime (Utilities|Array|Get(acopy) (Variables|Default|GetNaviPointsActors)) 0.0)
    (for _index (range 1 (Utilities|Array|LastIndex (Variables|Default|GetNaviPointsActors)))
      (bind _output_get (Variables|/Game/DMA/Blueprints/BP_Point_Mission.BP_Point_Mission_C|SetEnterTime (Utilities|Array|Get(acopy) _navipointsactors_2 _index) (+ (Default|GetLeaveTime (Utilities|Array|Get(acopy) _navipointsactors_2 (- _index 1))) (/ (Transformation|GetDistanceTo (Utilities|Array|Get(acopy) _navipointsactors_2 (- _index 1)) (Utilities|Array|Get(acopy) _navipointsactors_2 _index)) (CallFunction|GetTargetSpeed (Transformation|GetActorLocation (Utilities|Array|Get(acopy) _navipointsactors_2 (- _index 1))) (Utilities|Array|Get(acopy) _navipointsactors_2 _index)))))))
    (Variables|Default|SetTotalTime (Variables|/Game/DMA/Blueprints/BP_Point_Mission.BP_Point_Mission_C|GetEnterTime (Utilities|Array|Get(acopy) _navipointsactors (Utilities|Array|LastIndex _navipointsactors))))
    (CallFunction|UpdateTimeline)
    (return)))

(fn UpdatePointTime
  (params (Point :type BP%20Point%20Mission%20Object%20Reference) (NewTime :type Float%20%28single-precision%29))
  (Utilities|IsValid Point
    (:Is%20Valid
      (LocalVariables|SetLocalPoint Point)
      (LocalVariables|SetLocalNewTime NewTime)
      (if (Utilities|Array|IsValidIndex (Variables|Default|GetNaviPointsActors))
        (if (and (Default|IsFirst (LocalVariables|GetLocalPoint)) (Default|IsLast (LocalVariables|GetLocalPoint)))
          (CallFunction|UpdateTimeline)
          (elif (Default|IsFirst (LocalVariables|GetLocalPoint))
            (bind _output_get (LocalVariables|SetLocalNewTime (Math|Float|Min(Float) (LocalVariables|GetLocalNewTime) (Variables|/Game/DMA/Blueprints/BP_Point_Mission.BP_Point_Mission_C|GetEnterTime (Default|GetNext (LocalVariables|GetLocalPoint))))))
            (Default|UpdateSpeed (Default|GetNext (LocalVariables|GetLocalPoint)) (- (Variables|/Game/DMA/Blueprints/BP_Point_Mission.BP_Point_Mission_C|GetEnterTime (Default|GetNext (LocalVariables|GetLocalPoint))) _output_get))
            (CallFunction|CalculatePointsTimes)
            (elif (Default|IsLast (LocalVariables|GetLocalPoint))
              (bind _output_get_2 (LocalVariables|SetLocalNewTime (Math|Float|Max(Float) (LocalVariables|GetLocalNewTime) (Default|GetLeaveTime (Default|GetPrevious (LocalVariables|GetLocalPoint))))))
              (Default|UpdateSpeed (LocalVariables|GetLocalPoint) (- _output_get_2 (Default|GetLeaveTime (Default|GetPrevious (LocalVariables|GetLocalPoint)))))
              (CallFunction|CalculatePointsTimes)
              (else
                (bind _output_get_3 (LocalVariables|SetLocalNewTime (Math|Float|Clamp(Float) (LocalVariables|GetLocalNewTime) (Default|GetLeaveTime (Default|GetPrevious (LocalVariables|GetLocalPoint))) (- (Variables|/Game/DMA/Blueprints/BP_Point_Mission.BP_Point_Mission_C|GetEnterTime (Default|GetNext (LocalVariables|GetLocalPoint))) (Default|GetWaitTime (LocalVariables|GetLocalPoint))))))
                (Default|UpdateSpeed (LocalVariables|GetLocalPoint) (- _output_get_3 (Default|GetLeaveTime (Default|GetPrevious (LocalVariables|GetLocalPoint)))))
                (Default|UpdateSpeed (Default|GetNext (LocalVariables|GetLocalPoint)) (- (Variables|/Game/DMA/Blueprints/BP_Point_Mission.BP_Point_Mission_C|GetEnterTime (Default|GetNext (LocalVariables|GetLocalPoint))) (+ (LocalVariables|GetLocalNewTime) (Default|GetWaitTime (LocalVariables|GetLocalPoint)))))
                (CallFunction|CalculatePointsTimes)))))
        (else
          (CallFunction|UpdateTimeline :!label _label))))
    (:Is%20Not%20Valid
      (goto _label))))

(fn UpdateTimeline
  (bind _asw_mission_timeline (Utilities|Casting|CastToW_Mission_Timeline (Variables|Default|GetTimelineWidget)))
  (Default|UpdateTimeline _asw_mission_timeline)
  (bind _asbp_main_pawn (Utilities|Casting|CastToBP_Main_Pawn (Game|Player|GetPlayerPawn 0)))
  (Default|CalculateZoom (Variables|/Game/DMA/UI/Widgets/MenuWidget.MenuWidget_C|GetMissionsScroll (Variables|/Game/DMA/Blueprints/Core/BP_Main_Pawn.BP_Main_Pawn_C|GetMenuWidget _asbp_main_pawn)))
  (Default|CalculateMaxTime (Variables|/Game/DMA/UI/Widgets/MenuWidget.MenuWidget_C|GetMissionsScroll (Variables|/Game/DMA/Blueprints/Core/BP_Main_Pawn.BP_Main_Pawn_C|GetMenuWidget _asbp_main_pawn))))

(fn UpdateLinks)

(fn GetTargetPointat
  (params (InTime :type Float%20%28single-precision%29))
  (return (Default|GetNext (CallFunction|GetPointat InTime))))

(fn GetMovingActorRotationat
  (params (InTime :type Float%20%28single-precision%29))
  (bind _point (CallFunction|GetPointat InTime))
  (Utilities|IsValid (Default|GetNext _point)
    (:Is%20Valid
      (return (Math|Rotator|MakeRotator 0.0 0.0 (.poiHeading (Utilities|Struct|BreakMissionPoint (Variables|/Game/DMA/Blueprints/BP_Point_Mission.BP_Point_Mission_C|GetPointStruct _point))))))
    (:Is%20Not%20Valid
      (return (Math|Rotator|MakeRotator 0.0 0.0 (.poiHeading (Utilities|Struct|BreakMissionPoint (Variables|/Game/DMA/Blueprints/BP_Point_Mission.BP_Point_Mission_C|GetPointStruct _point))))))))

(fn GetPointat
  (params (InTime :type Float%20%28single-precision%29))
  (return (Utilities|Array|Get(acopy) (Variables|Default|GetNaviPointsActors) (CallFunction|GetPointIndexat InTime))))

(fn GetPointIndexat
  (params (InTime :type Float%20%28single-precision%29))
  (bind _navipointsactors (Variables|Default|GetNaviPointsActors))
  (bind _navipointsactors_2 (Variables|Default|GetNaviPointsActors))
  (bind _returnvalue (Utilities|Array|LastIndex _navipointsactors))
  (for _index (range 0 (- _returnvalue 1))
    (if (and (>= InTime (Variables|/Game/DMA/Blueprints/BP_Point_Mission.BP_Point_Mission_C|GetEnterTime (Utilities|Array|Get(acopy) _navipointsactors_2 _index))) (< InTime (Variables|/Game/DMA/Blueprints/BP_Point_Mission.BP_Point_Mission_C|GetEnterTime (Utilities|Array|Get(acopy) _navipointsactors_2 (+ _index 1)))))
      (return _index)))
  (return _returnvalue))

(fn SetWorldTrackIsHighlighted
  (params (bNewIsHighlighted :type Boolean))
  (|CallParentFunction bNewIsHighlighted)
  (Rendering|Material|SetScalarParameterValue (Variables|Default|GetPathMaterialInstance) "Lines" (Math|Float|SelectFloat 1.0 0.0 bNewIsHighlighted) :!class /Script/Engine.MaterialInstanceDynamic)
  (return bNewIsHighlighted))

(fn SetTimelineIsHighlighted
  (params (bNewIsHighlighted :type Boolean))
  (|CallParentFunction bNewIsHighlighted)
  (bind _asw_mission_timeline (Utilities|Casting|CastToW_Mission_Timeline (Variables|Default|GetTimelineWidget))
    (:then
      (bind _output_get (Variables|/Game/DMA/UI/Widgets/W_Mission_Timeline.W_Mission_Timeline_C|SetbIsHighlighted _asw_mission_timeline bNewIsHighlighted))
      (return _output_get))
    (:CastFailed
      (return false))))

(fn StartMoving
  (bind _movingactor (Variables|Default|GetMovingActor))
  (|CallParentFunction)
  (Utilities|IsValid _movingactor
    (:Is%20Valid
      (Default|StartMoving _movingactor)
      (return true))
    (:Is%20Not%20Valid
      (return false))))

(fn SetPointsMaterial
  (|CallParentFunction)
  (for _array_element (Variables|Default|GetNaviPointsActors)
    (Class|MapperPointBase|SetMaterial _array_element (Variables|Default|GetPathMaterialInstance)))
  (return true))

(fn SetPointsColor
  (params (NewColor :type Linear%20Color%20Structure))
  (|CallParentFunction NewColor)
  (Rendering|Material|SetVectorParameterValue (Variables|Default|GetPathMaterialInstance) "Color" NewColor :!class /Script/Engine.MaterialInstanceDynamic)
  (return true))

(fn SetMovingActor
  (params (NewTime :type Float%20%28single-precision%29))
  (bind _navipointsactors (Variables|Default|GetNaviPointsActors))
  (bind _navipointsactors_2 (Variables|Default|GetNaviPointsActors))
  (|CallParentFunction 0.0)
  (LocalVariables|SetCurrentTime NewTime)
  (for _index (range 1 (Utilities|Array|LastIndex _navipointsactors))
    (if (< (LocalVariables|GetCurrentTime) (Variables|/Game/DMA/Blueprints/BP_Point_Mission.BP_Point_Mission_C|GetEnterTime (Utilities|Array|Get(acopy) _navipointsactors_2 _index)))
      (Variables|/Game/DMA/Blueprints/Core/BP_Moving_Actor.BP_Moving_Actor_C|SetTargetPoint (Variables|Default|GetMovingActor) (Utilities|Array|Get(acopy) _navipointsactors_2 _index))
      (Transformation|SetActorLocation (Variables|Default|GetMovingActor) (Math|Interpolation|Ease "Linear" (Math|Float|Absolute(Float) (/ (- (Variables|/Game/DMA/Blueprints/BP_Point_Mission.BP_Point_Mission_C|GetEnterTime (Utilities|Array|Get(acopy) _navipointsactors_2 _index)) (LocalVariables|GetCurrentTime)) (- (Default|GetLeaveTime (Utilities|Array|Get(acopy) _navipointsactors_2 (- _index 1))) (Variables|/Game/DMA/Blueprints/BP_Point_Mission.BP_Point_Mission_C|GetEnterTime (Utilities|Array|Get(acopy) _navipointsactors_2 _index))))) (Transformation|GetActorLocation (Utilities|Array|Get(acopy) _navipointsactors_2 _index)) (Transformation|GetActorLocation (Utilities|Array|Get(acopy) _navipointsactors_2 (- _index 1)))) false false)
      (Transformation|SetActorRotation (Variables|Default|GetMovingActor) (CallFunction|GetMovingActorRotationat (LocalVariables|GetCurrentTime)) :!label _label)
      (Variables|/Game/DMA/Blueprints/Core/BP_Moving_Actor.BP_Moving_Actor_C|SetCurrentPoint (Variables|Default|GetMovingActor) (+ (CallFunction|GetPointIndexat (LocalVariables|GetCurrentTime)) 1))
      (Variables|/Game/DMA/Blueprints/Core/BP_Moving_Actor.BP_Moving_Actor_C|SetTargetPoint (Variables|Default|GetMovingActor) (CallFunction|GetTargetPointat (LocalVariables|GetCurrentTime)))
      (return false)
      (elif (and (>= (LocalVariables|GetCurrentTime) (Variables|/Game/DMA/Blueprints/BP_Point_Mission.BP_Point_Mission_C|GetEnterTime (Utilities|Array|Get(acopy) _navipointsactors_2 _index))) (<= (LocalVariables|GetCurrentTime) (Default|GetLeaveTime (Utilities|Array|Get(acopy) _navipointsactors_2 _index))))
        (Variables|/Game/DMA/Blueprints/Core/BP_Moving_Actor.BP_Moving_Actor_C|SetTargetPoint (Variables|Default|GetMovingActor) (Utilities|Array|Get(acopy) _navipointsactors_2 _index))
        (Transformation|SetActorLocation (Variables|Default|GetMovingActor) (Transformation|GetActorLocation (Utilities|Array|Get(acopy) _navipointsactors_2 _index)) false false)
        (goto _label))))
  (Transformation|SetActorLocation (Variables|Default|GetMovingActor) (Transformation|GetActorLocation (Utilities|Array|Get(acopy) _navipointsactors)) false false)
  (Transformation|SetActorRotation (Variables|Default|GetMovingActor) (CallFunction|GetMovingActorRotationat (LocalVariables|GetCurrentTime)))
  (Variables|/Game/DMA/Blueprints/Core/BP_Moving_Actor.BP_Moving_Actor_C|SetCurrentPoint (Variables|Default|GetMovingActor) (+ (CallFunction|GetPointIndexat (LocalVariables|GetCurrentTime)) 1))
  (Variables|/Game/DMA/Blueprints/Core/BP_Moving_Actor.BP_Moving_Actor_C|SetTargetPoint (Variables|Default|GetMovingActor) (CallFunction|GetTargetPointat (LocalVariables|GetCurrentTime)))
  (return false))

(fn SetPaused
  (params (bNewIsPaused :type Boolean))
  (bind _returnvalue (|CallParentFunction bNewIsPaused))
  (bind _output_get (Variables|/Game/DMA/Blueprints/Core/BP_Moving_Actor.BP_Moving_Actor_C|SetPaused? (Variables|Default|GetMovingActor) _returnvalue))
  (return _output_get))

(fn SetPathVisibility
  (params (bNewIsVisible :type Boolean))
  (|CallParentFunction bNewIsVisible)
  (for _array_element (Variables|Default|GetNaviPointsActors)
    (Default|UpdatePathVisibility _array_element))
  (return (Variables|Default|GetbIsPathVisible)))

(fn RemovePath
  (bind _returnvalue (Class|KulaginStatics|GetMapperGameMode))
  (bind _pointcontainers (Variables|/Script/Kulagin.MapperGameMode|GetPointContainers _returnvalue))
  (|CallParentFunction)
  (Utilities|IsValid (Variables|Default|GetTimelineWidget)
    (:Is%20Valid
      (Widget|RemovefromParent (Variables|Default|GetTimelineWidget)))
    (:Is%20Not%20Valid
      _))
  (Variables|Default|SetTimelineWidget 0)
  (Utilities|Array|RemoveIndex _pointcontainers (Utilities|Array|FindItem _pointcontainers self))
  (for _array_element (Variables|Default|GetNaviPointsActors)
    (Actor|DestroyActor _array_element))
  (Actor|DestroyActor (Variables|Default|GetMovingActor))
  (Actor|DestroyActor)
  (return true))

(fn GetTotalTime
  (return (Variables|Default|GetTotalTime)))

(fn GetLocationatTime
  (params (TimeIn :type Float%20%28single-precision%29))
  (bind _navipointsactors (Variables|Default|GetNaviPointsActors))
  (bind _navipointsactors_2 (Variables|Default|GetNaviPointsActors))
  (for _index (range 1 (Utilities|Array|LastIndex _navipointsactors_2))
    (if (< TimeIn (Variables|/Game/DMA/Blueprints/BP_Point_Mission.BP_Point_Mission_C|GetEnterTime (Utilities|Array|Get(acopy) _navipointsactors _index)))
      (return (Math|Interpolation|Ease "Linear" (Math|Float|Absolute(Float) (/ (- (Variables|/Game/DMA/Blueprints/BP_Point_Mission.BP_Point_Mission_C|GetEnterTime (Utilities|Array|Get(acopy) _navipointsactors _index)) TimeIn) (- (Default|GetLeaveTime (Utilities|Array|Get(acopy) _navipointsactors (- _index 1))) (Variables|/Game/DMA/Blueprints/BP_Point_Mission.BP_Point_Mission_C|GetEnterTime (Utilities|Array|Get(acopy) _navipointsactors _index))))) (Transformation|GetActorLocation (Utilities|Array|Get(acopy) _navipointsactors _index)) (Transformation|GetActorLocation (Utilities|Array|Get(acopy) _navipointsactors (- _index 1)))))
      (elif (and (>= TimeIn (Variables|/Game/DMA/Blueprints/BP_Point_Mission.BP_Point_Mission_C|GetEnterTime (Utilities|Array|Get(acopy) _navipointsactors _index))) (<= TimeIn (Default|GetLeaveTime (Utilities|Array|Get(acopy) _navipointsactors _index))))
        (return (Transformation|GetActorLocation (Utilities|Array|Get(acopy) _navipointsactors _index))))))
  (return (Transformation|GetActorLocation (Utilities|Array|Get(acopy) _navipointsactors_2))))

(fn UpdateDangerZones
  (bind _returnvalue (|CallParentFunction))
  (if _returnvalue
    (for _array_element (Variables|Default|GetNaviPointsActors)
      (Default|UpdateCrossCylinder _array_element))
    (return true)
    (else
      (return false))))

(fn GetMissionPoint
  (params (Index :type Integer))
  (bind _asbp_point_mission (Utilities|Casting|CastToBP_Point_Mission (Utilities|Array|Get(acopy) (Variables|Default|GetPointActors) Index))
    (:then
      (return _asbp_point_mission))
    (:CastFailed
      (return 0))))

(fn GetActorsIgnoreCrossing
  (bind _output_get (LocalVariables|SetIgnoreLocal (|CallParentFunction)))
  (Utilities|Array|AppendArray _output_get (Variables|Default|GetNaviPointsActors))
  (Utilities|Array|Add (LocalVariables|GetIgnoreLocal) (Variables|Default|GetMovingActor))
  (Utilities|Array|Add (LocalVariables|GetIgnoreLocal) (Variables|/Game/DMA/Blueprints/Core/BP_Moving_Actor.BP_Moving_Actor_C|GetChildDrone (Variables|Default|GetMovingActor)))
  (return (LocalVariables|GetIgnoreLocal)))

(fn GetActualPointData
  (for _array_element (Variables|Default|GetNaviPointsActors)
    (Utilities|Array|Add (LocalVariables|GetLocalMissionPoints) (Variables|/Game/DMA/Blueprints/BP_Point_Mission.BP_Point_Mission_C|GetPointStruct _array_element)))
  (return (LocalVariables|GetLocalMissionPoints)))

(fn UpdateCrossRadius
  (for _array_element (Variables|Default|GetNaviPointsActors)
    (Default|UpdateCrossRadius _array_element)))

(fn SetDangerZoneVisibility
  (params (bNewIsVisible :type Boolean))
  (|CallParentFunction bNewIsVisible)
  (for _array_element (Variables|Default|GetNaviPointsActors)
    (Default|UpdateCrossVisibility _array_element))
  (return (Variables|Default|GetbIsDangerZoneVisible)))

(fn SetMovingActorVisibility
  (params (bNewIsVisible :type Boolean))
  (|CallParentFunction bNewIsVisible)
  (Default|SetMovingActorVisible (Variables|Default|GetMovingActor) (Variables|Default|GetbIsMovingActorVisible))
  (return (Variables|Default|GetbIsMovingActorVisible)))

(fn DropMovingActor
  (|CallParentFunction)
  (bind _returnvalue (Class|MapperDroneBase|DropMovingActor (Variables|Default|GetMovingActor)))
  (return _returnvalue))

(fn RiseMovingActor
  (|CallParentFunction)
  (bind _returnvalue (Class|MapperDroneBase|RiseMovingActor (Variables|Default|GetMovingActor)))
  (return _returnvalue))