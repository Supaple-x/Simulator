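; Log point actor that marks one point of a recorded log in the world and draws the path segment to the next point.
; SetPointStruct stores the point and moves the actor to its converted Unreal position, using a start altitude.
; SetNextPointBP aims the PathNormal pivot at the next point, then centers, stretches and unhides the Path component to span the gap.
; SetMaterial extends the parent's version to also apply the material to Path.
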(event EventBeginPlay)

(event Collision|EventActorBeginOverlap
  (params (OtherActor :type Actor%20Object%20Reference)))

(event EventTick
  (params (DeltaSeconds :type Float%20%28single-precision%29)))

(fn ConstructionScript)

(fn SetPointStruct
  (params (LogPoint :type Log%20Point%20Structure))
  (bind _output_get (Variables|Default|SetLogPointStruct LogPoint))
  (bind _returnvalue (Class|KulaginStatics|LogPointtoUE _output_get (Variables|Default|GetStartAlt)))
  (Transformation|SetActorLocation _returnvalue false false))

(fn SetMaterial
  (params (NewMaterial :type Material%20Interface%20Object%20Reference))
  (|CallParentFunction NewMaterial)
  (Rendering|Material|SetMaterial (Variables|Default|GetPath) 0 NewMaterial)
  (return true))

(fn SetNextPointBP
  (params (NextPoint :type Mapper%20Point%20Base%20Object%20Reference))
  (bind _returnvalue (Transformation|GetActorLocation))
  (bind _returnvalue_2 (Transformation|GetActorLocation NextPoint))
  (bind _returnvalue_3 (Math|Vector|Distance(Vector) _returnvalue_2 _returnvalue))
  (Utilities|IsValid NextPoint
    (:Is%20Valid
      (Transformation|SetRelativeRotation (Variables|Default|GetPathNormal) (Math|Rotator|FindLookatRotation _returnvalue _returnvalue_2) false false)
      (Transformation|SetRelativeLocation (Variables|Default|GetPath) (Math|Vector|MakeVector (* _returnvalue_3 0.5) 0.0 0.0) false false)
      (Transformation|SetRelativeScale3D (Variables|Default|GetPath) (Math|Vector|MakeVector (* _returnvalue_3 0.01) 0.1 0.1))
      (Development|SetHiddeninGame (Variables|Default|GetPath) false false))))