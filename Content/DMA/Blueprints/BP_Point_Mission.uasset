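; BP_Point_Mission is a waypoint actor in a timed mission path, syncing its world position with lat/lon/alt point data.
; Moves update that data and ask the parent container to recalculate times.
; Tick stretches a plane and cylinder toward TargetActor and line-traces projection beams with decals, including colored takeoff/landing markers.
; A per-instance render target feeds the cylinder material, masking danger zones over the time window from the previous point.
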(event Custom|DisableArrow
  (bind _arrowmesh (Variables|Default|GetArrowMesh))
  (Rendering|SetVisibility _arrowmesh false false)
  (Collision|SetCollisionProfileName _arrowmesh "NoCollision" :!class /Script/Engine.PrimitiveComponent))

(event Custom|ShowArrow
  (bind _arrowmesh (Variables|Default|GetArrowMesh))
  (Rendering|SetVisibility _arrowmesh true false)
  (Collision|SetCollisionProfileName _arrowmesh "BlockAll" :!class /Script/Engine.PrimitiveComponent))

(event EventBeginPlay
  (bind _returnvalue (Rendering|CreateRenderTarget2D 512 512 "RTF_RGBA16f"))
  (bind _output_get (Variables|Default|SetCrossRenderTarget _returnvalue))
  (Rendering|ClearRenderTarget2D _output_get)
  (bind _returnvalue_2 (Rendering|Material|CreateDynamicMaterialInstance "/Game/DMA/MaterialLibrary/M_Cross_01.M_Cross_01" "None" :!class /Script/Engine.KismetMaterialLibrary))
  (bind _output_get_2 (Variables|Default|SetCrossMaterial _returnvalue_2))
  (Rendering|Material|SetTextureParameterValue _output_get_2 "RenderTarget" (Variables|Default|GetCrossRenderTarget))
  (Rendering|Material|SetMaterial (Variables|Default|GetCylinder) 0 (Variables|Default|GetCrossMaterial)))

(event Collision|EventActorBeginOverlap
  (params (OtherActor :type Actor%20Object%20Reference)))

(event EventTick
  (params (DeltaSeconds :type Float%20%28single-precision%29))
  (bind _returnvalue (Transformation|GetActorLocation))
  (if (Variables|Default|GetbIsFirstLast)
    (CallFunction|UpdateFirstLast))
  (if (Variables|Default|GetbIsProjectionEnabled)
    (CallFunction|UpdateProjection))
  (if (Math|Vector|NotEqual(Vector) (Variables|Default|GetPrevLocation) _returnvalue 0.1)
    (Variables|Default|SetPrevLocation _returnvalue)
    (CallFunction|ChangePointStruct))
  (bind _targetactor (Variables|Default|GetTargetActor)
    (:then
      (if (Math|Vector|NotEqual(Vector) (Variables|Default|GetTargetPrevLocation) (Transformation|GetActorLocation _targetactor) 0.1)
        (Variables|Default|SetTargetPrevLocation (Variables|Default|GetTargetPrevLocation))
        (CallFunction|CreatePlane)))
    (:else
      (Rendering|SetVisibility (Variables|Default|GetPlane) false false))))

(fn ConstructionScript)

(fn CreatePlane
  (bind _returnvalue (Transformation|GetActorLocation))
  (bind _planeroot (Variables|Default|GetPlaneRoot))
  (bind _targetactor (Variables|Default|GetTargetActor))
  (bind _returnvalue_2 (Transformation|GetActorLocation _targetactor))
  (bind _returnvalue_3 (Math|Vector|Distance(Vector) _returnvalue _returnvalue_2))
  (bind _returnvalue_4 (Math|Rotator|FindLookatRotation _returnvalue _returnvalue_2))
  (bind (_roll _pitch _yaw) (Math|Rotator|BreakRotator _returnvalue_4))
  (bind _returnvalue_5 (/ _returnvalue_3 1e+02))
  (Rendering|SetVisibility (Variables|Default|GetPlane) true false)
  (Transformation|SetWorldScale3D _planeroot (Math|Vector|MakeVector 1.0 1.0 _returnvalue_5))
  (Transformation|SetWorldRotation _planeroot (Math|Rotator|MakeRotator 0.0 _pitch _yaw) false false)
  (Transformation|SetRelativeLocation (Variables|Default|GetCylinder) (Math|Vector|MakeVector (* _returnvalue_5 5e+01) 0.0 0.0) false false))

(fn IntBacktoMap
  (params (SourceString :type String) (InInt :type Integer))
  (bind _returnvalue (Utilities|String|Left SourceString 1))
  (bind _returnvalue_2 (Utilities|String|ToString(Integer) InInt))
  (bind _returnvalue_3 (Utilities|String|Left _returnvalue_2 1))
  (bind _returnvalue_4 (Utilities|String|RightChop _returnvalue_2 1))
  (bind _returnvalue_5 (Utilities|String|Append _returnvalue _returnvalue_3 "." _returnvalue_4))
  (bind _returnvalue_6 (Utilities|String|Reverse _returnvalue_5))
  (bind _returnvalue_7 (Utilities|String|GetCharacterArrayfromString _returnvalue_6))
  (bind _array_element (Utilities|Array|ForEachLoopwithBreak _returnvalue_7 :!label _label)
    (:LoopBody
      (if (Utilities|Enum|Equal(Enum) _array_element "0")
        (Math|Integer|IncrementInt (LocalVariables|GetZeroCount))
        (else
          (goto _label Break))))
    (:Completed
      (return (Utilities|String|LeftChop (Utilities|String|Reverse (Utilities|String|JoinStringArray _returnvalue_7 "")) (LocalVariables|GetZeroCount))))))

(fn ChangePointStruct
  ;[1 1 1] If location changed laclulate new Lat and Lon
  (if (not (Variables|Default|GetbStaticPointStruct))
    (CallFunction|CoordBacktoMap (Variables|Default|GetPointStruct) (Variables|Default|GetReferenceLatLon) (Transformation|GetActorLocation) (Variables|Default|GetStartAlt))
    (Default|CalculatePointsTimes (Variables|Default|GetParentContainer))))

(fn SetPointID
  (params (Value :type Integer%20%28by%20ref%29))
  (bind _output_get (Variables|Default|SetPointID Value))
  (Rendering|Components|TextRender|SetText (Variables|Default|GetTextRender) (Utilities|Text|ToText(Integer) _output_get)))

(fn OnPointStructUpdated
  (Development|PrintString "Kulagin: On Point Struct Updated")
  (Transformation|SetActorLocation (CallFunction|MaptoCoord (Variables|Default|GetPointStruct) (Variables|Default|GetReferenceLatLon) (Variables|Default|GetStartAlt)) false false)
  (Variables|Default|SetPrevLocation (Transformation|GetActorLocation)))

(fn SetMaterialBp
  (params (NewMaterial :type Material%20Interface%20Object%20Reference)))

(fn UpdateProjection
  (for (_array_element _array_index) (Utilities|Array|MakeArray (Variables|Default|GetProjectionZMinusRoot) (Variables|Default|GetProjectionXMinusRoot) (Variables|Default|GetProjectionXPlusRoot) (Variables|Default|GetProjectionYMinusRoot) (Variables|Default|GetProjectionYPlusRoot))
    (CallFunction|UpdateProjectionComponents _array_element (Utilities|Array|Get(acopy) (Utilities|Array|MakeArray (Variables|Default|GetProjectionZMinusDecal) (Variables|Default|GetProjectionXMinusDecal) (Variables|Default|GetProjectionXPlusDecal) (Variables|Default|GetProjectionYMinusDecal) (Variables|Default|GetProjectionYPlusDecal)) _array_index))))

(fn ToggleProjection
  (params (bEnabled :type Boolean))
  (Class|MapperContainerBase|SetTimelineIsHighlighted (Variables|Default|GetParentContainer) bEnabled)
  (if (Math|Boolean|NotEqual(Boolean) bEnabled (Variables|Default|GetbIsProjectionEnabled))
    (Variables|Default|SetbIsProjectionEnabled bEnabled)
    (for (_array_element _array_index) (Utilities|Array|MakeArray (Variables|Default|GetProjectionZMinusRoot) (Variables|Default|GetProjectionXMinusRoot) (Variables|Default|GetProjectionXPlusRoot) (Variables|Default|GetProjectionYMinusRoot) (Variables|Default|GetProjectionYPlusRoot))
      (Development|SetHiddeninGame _array_element (not (Variables|Default|GetbIsProjectionEnabled)) true)
      (Development|SetHiddeninGame (Utilities|Array|Get(acopy) (Utilities|Array|MakeArray (Variables|Default|GetProjectionZMinusDecal) (Variables|Default|GetProjectionXMinusDecal) (Variables|Default|GetProjectionXPlusDecal) (Variables|Default|GetProjectionYMinusDecal) (Variables|Default|GetProjectionYPlusDecal)) _array_index) (not (Variables|Default|GetbIsProjectionEnabled)) true))))

(fn UpdateFirstLast
  (CallFunction|UpdateProjectionComponents (Variables|Default|GetProjectionFirstLastRoot) (Variables|Default|GetProjectionFirstLastDecal)))

(fn UpdateProjectionComponents
  (params (Root :type Scene%20Component%20Object%20Reference) (Decal :type Scene%20Component%20Object%20Reference))
  (bind _returnvalue (Transformation|GetActorLocation))
  (bind (_outhit _returnvalue_2) (Collision|LineTraceForObjects _returnvalue (+ _returnvalue (* (Math|Vector|GetForwardVector Root) 1e+05)) (Utilities|Array|MakeArray "ObjectTypeQuery1") true 0 "None"))
  (Transformation|SetWorldScale3D Root (Math|Vector|MakeVector (Math|Float|SelectFloat (/ (Math|Vector|Distance(Vector) (.ImpactPoint (Collision|BreakHitResult _outhit)) (Transformation|GetActorLocation)) 1e+02) 1e+03 _returnvalue_2) 1.0 1.0))
  (Development|SetHiddeninGame Decal (not _returnvalue_2) false)
  (if _returnvalue_2
    (Transformation|SetWorldLocation Decal (.ImpactPoint (Collision|BreakHitResult _outhit)) false false)))

(fn SetFirst
  (Variables|Default|SetbIsFirstLast true)
  (Rendering|Material|SetMaterial (Variables|Default|GetProjectionFirstLast) 0 "/Game/DMA/MaterialLibrary/MI_Projection_01_Red.MI_Projection_01_Red")
  (Development|SetHiddeninGame (Variables|Default|GetProjectionFirstLast) false false)
  (Rendering|Components|Decal|SetDecalMaterial (Variables|Default|GetProjectionFirstLastDecal) "/Game/DMA/MaterialLibrary/MI_Projection_Decal_01_Red.MI_Projection_Decal_01_Red")
  (Development|SetHiddeninGame (Variables|Default|GetProjectionFirstLastDecal) false false)
  (Utilities|Struct|SetmembersinMissionPoint (Variables|Default|GetPointStruct) "NAVI_POINT_TAKEOFF"))

(fn SetLast
  (Variables|Default|SetbIsFirstLast true)
  (Rendering|Material|SetMaterial (Variables|Default|GetProjectionFirstLast) 0 "/Game/DMA/MaterialLibrary/MI_Projection_01_Yellow.MI_Projection_01_Yellow")
  (Development|SetHiddeninGame (Variables|Default|GetProjectionFirstLast) false false)
  (Rendering|Components|Decal|SetDecalMaterial (Variables|Default|GetProjectionFirstLastDecal) "/Game/DMA/MaterialLibrary/MI_Projection_Decal_01_Yellow.MI_Projection_Decal_01_Yellow")
  (Development|SetHiddeninGame (Variables|Default|GetProjectionFirstLastDecal) false false)
  (Utilities|Struct|SetmembersinMissionPoint (Variables|Default|GetPointStruct) "NAVI_POINT_TO_LAND"))

(fn SetNormal
  (bind _pointstruct (Variables|Default|GetPointStruct))
  (bind _type (Utilities|Struct|BreakMissionPoint _pointstruct))
  (Variables|Default|SetbIsFirstLast false)
  (Development|SetHiddeninGame (Variables|Default|GetProjectionFirstLast) true false)
  (Development|SetHiddeninGame (Variables|Default|GetProjectionFirstLastDecal) true false)
  (if (Math|Boolean|ORBoolean (== _type 5) (== _type 2) (== _type 0) (> _type 8))
    (Utilities|Struct|SetmembersinMissionPoint (Variables|Default|GetPointStruct) "NAVI_POINT_SIMPLE")))

(fn GetWaitTime
  (return (/ (Math|Conversions|ToFloat(Integer) (.loitertime (Variables|Default|GetPointStruct))) 1e+03)))

(fn GetLeaveTime
  (bind _entertime (Variables|Default|GetEnterTime))
  (return (Math|Float|SelectFloat _entertime (+ _entertime (CallFunction|GetWaitTime)) (Variables|Default|GetbIsFirstLast))))

(fn IsFirst
  (return (== (Variables|Default|GetPointID) 0)))

(fn IsLast
  (return (== (Variables|Default|GetPointID) (Utilities|Array|LastIndex (Variables|/Game/DMA/Blueprints/BP_Container_Mission.BP_Container_Mission_C|GetNaviPointsActors (Variables|Default|GetParentContainer))))))

(fn GetPrevious
  (bind _pointid (Variables|Default|GetPointID))
  (bind _parentcontainer (Variables|Default|GetParentContainer))
  (bind _returnvalue (- _pointid 1))
  (bind _navipointsactors (Variables|/Game/DMA/Blueprints/BP_Container_Mission.BP_Container_Mission_C|GetNaviPointsActors _parentcontainer))
  (if (Utilities|Array|IsValidIndex _navipointsactors _returnvalue)
    (return (Utilities|Array|Get(acopy) _navipointsactors _returnvalue))
    (else
      (return 0))))

(fn GetNext
  (bind _pointid (Variables|Default|GetPointID))
  (bind _parentcontainer (Variables|Default|GetParentContainer))
  (bind _returnvalue (+ _pointid 1))
  (bind _navipointsactors (Variables|/Game/DMA/Blueprints/BP_Container_Mission.BP_Container_Mission_C|GetNaviPointsActors _parentcontainer))
  (Utilities|IsValid _parentcontainer
    (:Is%20Valid
      (if (Utilities|Array|IsValidIndex _navipointsactors _returnvalue)
        (return (Utilities|Array|Get(acopy) _navipointsactors _returnvalue))
        (else
          _)))
    (:Is%20Not%20Valid
      _))
  (return 0))

(fn UpdateSpeed
  (params (NewTargetTime :type Float%20%28single-precision%29))
  (bind _previous (CallFunction|GetPrevious))
  (bind _pointstruct (Variables|Default|GetPointStruct))
  (bind (_targetlatlon _targetalt _targetradius _loitertime _maxhorizspeed _maxvertspeed) (Utilities|Struct|BreakMissionPoint _pointstruct))
  (if (not (CallFunction|IsFirst))
    (bind _output_get (LocalVariables|SetOldTime (/ (Transformation|GetDistanceTo _previous) (CallFunction|GetTargetSpeed (Transformation|GetActorLocation _previous) self))))
    (LocalVariables|SetSpeedMultiplier (/ _output_get NewTargetTime))
    (Utilities|Struct|SetmembersinMissionPoint _pointstruct (* _maxhorizspeed (LocalVariables|GetSpeedMultiplier)) (* _maxvertspeed (LocalVariables|GetSpeedMultiplier)))))

(fn SetMaterial
  (params (NewMaterial :type Material%20Interface%20Object%20Reference))
  (|CallParentFunction NewMaterial)
  (Rendering|Material|SetMaterial (Variables|Default|GetSphere) 0 NewMaterial)
  (Rendering|Material|SetMaterial (Variables|Default|GetPlane) 0 NewMaterial)
  (return true))

(fn UpdateCrossRadius
  (bind _parentcontainer (Variables|Default|GetParentContainer))
  (bind _returnvalue (Class|MapperContainerBase|GetDangerZoneRadiusUU _parentcontainer))
  (bind _returnvalue_2 (/ _returnvalue 1e+02))
  (Transformation|SetRelativeScale3D (Variables|Default|GetCylinder) (Math|Vector|MakeVector _returnvalue_2 _returnvalue_2 1.0)))

(fn UpdateCrossCylinder
  (Utilities|IsValid (Variables|Default|GetParentContainer)
    (:Is%20Valid
      (bind _output_get (LocalVariables|SetPrevLocal (CallFunction|GetPrevious)))
      (Utilities|IsValid _output_get
        (:Is%20Valid
          (LocalVariables|SetStartTimeLocal (CallFunction|GetLeaveTime _output_get))
          (LocalVariables|SetEndTimeLocal (Variables|Default|GetEnterTime))
          (Class|MapperPointBase|SetDangerZoneMask (Variables|Default|GetCrossRenderTarget) (LocalVariables|GetStartTimeLocal) (LocalVariables|GetEndTimeLocal) (Variables|/Script/Kulagin.MapperContainerBase|GetDangerZones (Variables|Default|GetParentContainer))))))))

(fn UpdateCrossVisibility
  (Development|SetHiddeninGame (Variables|Default|GetCylinder) (not (Variables|/Game/DMA/Blueprints/BP_Container_Mission.BP_Container_Mission_C|GetDangerZoneVisible (Variables|Default|GetParentContainer))) false))