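; Drone mission waypoint actor that wraps a PointData struct and maps it between WGS84 coordinates and world location.
; First, last and normal setters adjust the point type to takeoff, landing or simple.
; Moving the actor rewrites its data unless static and has the parent container recalculate point times.
; It also copies data from mission lists or other points, reports loiter time, and picks travel speed from the slower horizontal or vertical leg.
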(fn ConstructionScript)

(fn SetFirst
  (bind _returnvalue (|CallParentFunction))
  (Utilities|Struct|SetmembersinMissionPoint (Variables|Default|GetPointData) "NAVI_POINT_TAKEOFF")
  (return _returnvalue))

(fn SetLast
  (bind _returnvalue (|CallParentFunction))
  (Utilities|Struct|SetmembersinMissionPoint (Variables|Default|GetPointData) "NAVI_POINT_TO_LAND")
  (return _returnvalue))

(fn SetNormal
  (bind _pointdata (Variables|Default|GetPointData))
  (bind _type (Utilities|Struct|BreakMissionPoint _pointdata))
  (bind _returnvalue (|CallParentFunction))
  (if (Math|Boolean|ORBoolean (== _type 5) (== _type 2) (== _type 0) (> _type 8))
    (Utilities|Struct|SetmembersinMissionPoint (Variables|Default|GetPointData) "NAVI_POINT_SIMPLE"))
  (return _returnvalue))

(fn GetWaitTime
  (return (/ (Math|Conversions|ToFloat(Integer) (.loitertime (Variables|Default|GetPointData))) 1e+03)))

(fn UpdateActorfromData
  (Development|PrintString "Kulagin: UpdateActorFromData for Drone Point")
  (bind _returnvalue (Class|KulaginStatics|WGS84toUE (Variables|Default|GetPointData) (Variables|Default|GetStartAlt)))
  (Transformation|SetActorLocation _returnvalue false false)
  (Variables|Default|SetPrevLocation (Transformation|GetActorLocation))
  (return true))

(fn UpdateDatafromActor
  (if (not (Variables|Default|GetbStaticPointStruct))
    (Class|KulaginStatics|UEtoWGS84 (Variables|Default|GetPointData) (Transformation|GetActorLocation) (Variables|Default|GetStartAlt))
    (bind _asbp_container_interactive (Utilities|Casting|CastToBP_Container_Interactive (Variables|Default|GetParentContainer)))
    (Default|CalculatePointsTimes _asbp_container_interactive)
    (return true)))

(fn SetDatafromList
  (params (List :type Mission%20Point%20List%20Structure%20%28by%20ref%29) (Index :type Integer))
  (if (and (Utilities|Enum|Equal(Enum) (.type List) "PCT_Mission") (Utilities|Array|IsValidIndex (.dronepoints List) Index))
    (Variables|Default|SetPointData (Utilities|Array|Get(acopy) (.dronepoints List) Index))
    (return true)
    (else
      (return false))))

(fn SetDatafromPoint
  (params (Point :type Mapper%20Point%20Base%20Object%20Reference))
  (bind _asbp_point_drone_mission (Utilities|Casting|CastToBP_Point_Drone_Mission Point)
    (:then
      (Variables|Default|SetPointData (Variables|BP_Point_Drone_Mission_C|GetPointData _asbp_point_drone_mission))
      (return true))
    (:CastFailed
      (return false))))

(fn GetSpeedtoPoint
  (params (CurrentLocation :type Vector%20%28by%20ref%29 :default "0, 0, 0"))
  (bind _returnvalue (Transformation|GetActorLocation))
  (bind _pointdata (Variables|Default|GetPointData))
  (bind (_targetlatlon _maxhorizspeed _maxvertspeed) (Utilities|Struct|BreakMissionPoint _pointdata))
  (bind (_x _y _z) (Math|Vector|BreakVector CurrentLocation))
  (LocalVariables|SetHorSpeed (Math|Float|SelectFloat 1e+03 (* _maxhorizspeed 1e+01) (== _maxhorizspeed 0.0)))
  (LocalVariables|SetVertSpeed (Math|Float|SelectFloat 1e+03 (* _maxvertspeed 1e+01) (== 0.0 _maxvertspeed)))
  (LocalVariables|SetHorDistance (Math|Vector|Distance2D(Vector) (Math|Vector2D|MakeVector2D _x _y) (Math|Vector2D|MakeVector2D (.x _returnvalue) (.y _returnvalue))))
  (LocalVariables|SetVertDistance (Math|Float|Absolute(Float) (- _z (.z _returnvalue))))
  (return (Math|Float|SelectFloat (LocalVariables|GetVertSpeed) (LocalVariables|GetHorSpeed) (> (/ (LocalVariables|GetVertDistance) (LocalVariables|GetVertSpeed)) (/ (LocalVariables|GetHorDistance) (LocalVariables|GetHorSpeed))))))