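; Interactive path point actor that draws its segment to a target point and shows danger zones along a path.
; Tick stretches and aims the segment at TargetPoint, and line-traces projection beams and decals onto static world geometry, including red/yellow first/last markers.
; A per-point render target feeds the cylinder's material, masked by danger zones between the previous point's leave time and this point's enter time.
; ParentContainer supplies visibility flags and danger radius.
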(event EventBeginPlay
  (bind _returnvalue (Rendering|CreateRenderTarget2D 512 512 "RTF_RGBA16f"))
  (bind _output_get (Variables|Default|SetCrossRenderTarget _returnvalue))
  (Rendering|ClearRenderTarget2D _output_get)
  (bind _returnvalue_2 (Rendering|Material|CreateDynamicMaterialInstance "/Game/DMA/MaterialLibrary/M_Cross_01.M_Cross_01" "None" :!class /Script/Engine.KismetMaterialLibrary))
  (bind _output_get_2 (Variables|Default|SetCrossMaterial _returnvalue_2))
  (Rendering|Material|SetTextureParameterValue _output_get_2 "RenderTarget" (Variables|Default|GetCrossRenderTarget))
  (Rendering|Material|SetMaterial (Variables|Default|GetCylinder) 0 (Variables|Default|GetCrossMaterial)))

(event EventTick
  (params (DeltaSeconds :type Float%20%28single-precision%29))
  (bind _returnvalue (Transformation|GetActorLocation))
  (if (Variables|Default|GetbIsFirstLast)
    (CallFunction|UpdateFirstLast))
  (if (Variables|Default|GetbIsProjectionEnabled)
    (CallFunction|UpdateProjection))
  (if (Math|Vector|NotEqual(Vector) (Variables|Default|GetPrevLocation) _returnvalue 0.1)
    (Variables|Default|SetPrevLocation _returnvalue)
    (Class|MapperPointInteractive|UpdateDatafromActor))
  (bind _targetpoint (Variables|Default|GetTargetPoint)
    (:then
      (if (Math|Vector|NotEqual(Vector) (Variables|Default|GetTargetPrevLocation) (Transformation|GetActorLocation _targetpoint) 0.1)
        (Variables|Default|SetTargetPrevLocation (Variables|Default|GetTargetPrevLocation))
        (CallFunction|UpdatePlane)))
    (:else
      (Rendering|SetVisibility (Variables|Default|GetPlane) false false))))

(fn ConstructionScript)

(fn UpdatePlane
  (bind _returnvalue (Transformation|GetActorLocation))
  (bind _planeroot (Variables|Default|GetPlaneRoot))
  (bind _targetpoint (Variables|Default|GetTargetPoint))
  (bind _returnvalue_2 (Transformation|GetActorLocation _targetpoint))
  (bind _returnvalue_3 (Math|Vector|Distance(Vector) _returnvalue _returnvalue_2))
  (bind _returnvalue_4 (Math|Rotator|FindLookatRotation _returnvalue _returnvalue_2))
  (bind (_roll _pitch _yaw) (Math|Rotator|BreakRotator _returnvalue_4))
  (bind _returnvalue_5 (/ _returnvalue_3 1e+02))
  (Rendering|SetVisibility (Variables|Default|GetPlane) true false)
  (Transformation|SetWorldScale3D _planeroot (Math|Vector|MakeVector 1.0 1.0 _returnvalue_5))
  (Transformation|SetWorldRotation _planeroot (Math|Rotator|MakeRotator 0.0 _pitch _yaw) false false)
  (Transformation|SetRelativeLocation (Variables|Default|GetCylinder) (Math|Vector|MakeVector (* _returnvalue_5 5e+01) 0.0 0.0) false false)
  (return true))

(fn SetPointIndex
  (params (IndexIn :type Integer))
  (bind _output_get (Variables|Default|SetPointIndex IndexIn))
  (Rendering|Components|TextRender|SetText (Variables|Default|GetTextRender) (Utilities|Text|ToText(Integer) _output_get))
  (return true))

(fn UpdateProjection
  (for (_array_element _array_index) (Utilities|Array|MakeArray (Variables|Default|GetProjectionZMinusRoot) (Variables|Default|GetProjectionXMinusRoot) (Variables|Default|GetProjectionXPlusRoot) (Variables|Default|GetProjectionYMinusRoot) (Variables|Default|GetProjectionYPlusRoot))
    (CallFunction|UpdateProjectionComponents _array_element (Utilities|Array|Get(acopy) (Utilities|Array|MakeArray (Variables|Default|GetProjectionZMinusDecal) (Variables|Default|GetProjectionXMinusDecal) (Variables|Default|GetProjectionXPlusDecal) (Variables|Default|GetProjectionYMinusDecal) (Variables|Default|GetProjectionYPlusDecal)) _array_index)))
  (return true))

(fn SetProjectionEnabled
  (params (bEnabledIn :type Boolean))
  (Class|MapperContainerBase|SetTimelineIsHighlighted (Variables|Default|GetParentContainer) bEnabledIn)
  (if (Math|Boolean|NotEqual(Boolean) bEnabledIn (Variables|Default|GetbIsProjectionEnabled))
    (Variables|Default|SetbIsProjectionEnabled bEnabledIn)
    (for (_array_element _array_index) (Utilities|Array|MakeArray (Variables|Default|GetProjectionZMinusRoot) (Variables|Default|GetProjectionXMinusRoot) (Variables|Default|GetProjectionXPlusRoot) (Variables|Default|GetProjectionYMinusRoot) (Variables|Default|GetProjectionYPlusRoot))
      (Development|SetHiddeninGame _array_element (not (and (Variables|/Script/Kulagin.MapperContainerBase|GetbIsPathVisible (Variables|Default|GetParentContainer)) (Variables|Default|GetbIsProjectionEnabled))) true)
      (Development|SetHiddeninGame (Utilities|Array|Get(acopy) (Utilities|Array|MakeArray (Variables|Default|GetProjectionZMinusDecal) (Variables|Default|GetProjectionXMinusDecal) (Variables|Default|GetProjectionXPlusDecal) (Variables|Default|GetProjectionYMinusDecal) (Variables|Default|GetProjectionYPlusDecal)) _array_index) (not (and (Variables|/Script/Kulagin.MapperContainerBase|GetbIsPathVisible (Variables|Default|GetParentContainer)) (Variables|Default|GetbIsProjectionEnabled))) true)
      (return true))))

(fn UpdateFirstLast
  (CallFunction|UpdateProjectionComponents (Variables|Default|GetProjectionFirstLastRoot) (Variables|Default|GetProjectionFirstLastDecal)))

(fn UpdateProjectionComponents
  (params (Root :type Scene%20Component%20Object%20Reference) (Decal :type Scene%20Component%20Object%20Reference))
  (bind _returnvalue (Transformation|GetActorLocation))
  (bind (_outhit _returnvalue_2) (Collision|LineTraceForObjects _returnvalue (+ _returnvalue (* (Math|Vector|GetForwardVector Root) 1e+05)) (Utilities|Array|MakeArray "ObjectTypeQuery1") true 0 "None"))
  (Transformation|SetWorldScale3D Root (Math|Vector|MakeVector (Math|Float|SelectFloat (/ (Math|Vector|Distance(Vector) (.ImpactPoint (Collision|BreakHitResult _outhit)) (Transformation|GetActorLocation)) 1e+02) 1e+03 _returnvalue_2) 1.0 1.0))
  (Development|SetHiddeninGame Decal (not _returnvalue_2) false)
  (if _returnvalue_2
    (Transformation|SetWorldLocation Decal (.ImpactPoint (Collision|BreakHitResult _outhit)) false false)
    (return true)))

(fn SetFirst
  (Variables|Default|SetbIsFirstLast true)
  (Rendering|Material|SetMaterial (Variables|Default|GetProjectionFirstLast) 0 "/Game/DMA/MaterialLibrary/MI_Projection_01_Red.MI_Projection_01_Red")
  (Development|SetHiddeninGame (Variables|Default|GetProjectionFirstLast) false false)
  (Rendering|Components|Decal|SetDecalMaterial (Variables|Default|GetProjectionFirstLastDecal) "/Game/DMA/MaterialLibrary/MI_Projection_Decal_01_Red.MI_Projection_Decal_01_Red")
  (Development|SetHiddeninGame (Variables|Default|GetProjectionFirstLastDecal) false false)
  (return true))

(fn SetLast
  (Variables|Default|SetbIsFirstLast true)
  (Rendering|Material|SetMaterial (Variables|Default|GetProjectionFirstLast) 0 "/Game/DMA/MaterialLibrary/MI_Projection_01_Yellow.MI_Projection_01_Yellow")
  (Development|SetHiddeninGame (Variables|Default|GetProjectionFirstLast) false false)
  (Rendering|Components|Decal|SetDecalMaterial (Variables|Default|GetProjectionFirstLastDecal) "/Game/DMA/MaterialLibrary/MI_Projection_Decal_01_Yellow.MI_Projection_Decal_01_Yellow")
  (Development|SetHiddeninGame (Variables|Default|GetProjectionFirstLastDecal) false false)
  (return true))

(fn SetNormal
  (Variables|Default|SetbIsFirstLast false)
  (Development|SetHiddeninGame (Variables|Default|GetProjectionFirstLast) true false)
  (Development|SetHiddeninGame (Variables|Default|GetProjectionFirstLastDecal) true false)
  (return true))

(fn UpdateCrossRadius
  (bind _parentcontainer (Variables|Default|GetParentContainer))
  (bind _returnvalue (Class|MapperContainerBase|GetDangerZoneRadiusUU _parentcontainer))
  (bind _returnvalue_2 (/ _returnvalue 1e+02))
  (Transformation|SetRelativeScale3D (Variables|Default|GetCylinder) (Math|Vector|MakeVector _returnvalue_2 _returnvalue_2 1.0))
  (return true))

(fn UpdateCrossCylinder
  (Utilities|IsValid (Variables|Default|GetParentContainer)
    (:Is%20Valid
      (bind _output_get (LocalVariables|SetPrevLocal (Class|MapperPointInteractive|GetPreviousOfClass "/Script/Kulagin.MapperPointInteractive")))
      (Utilities|IsValid _output_get
        (:Is%20Valid
          (LocalVariables|SetStartTimeLocal (Class|MapperPointInteractive|GetLeaveTime _output_get))
          (LocalVariables|SetEndTimeLocal (Variables|Default|GetEnterTime))
          (Class|MapperPointBase|SetDangerZoneMask (Variables|Default|GetCrossRenderTarget) (LocalVariables|GetStartTimeLocal) (LocalVariables|GetEndTimeLocal) (Variables|/Script/Kulagin.MapperContainerBase|GetDangerZones (Variables|Default|GetParentContainer)))
          (return true))))))

(fn UpdateCrossVisibility
  (Development|SetHiddeninGame (Variables|Default|GetCylinder) (not (Variables|/Script/Kulagin.MapperContainerBase|GetbIsDangerZoneVisible (Variables|Default|GetParentContainer))) false)
  (return true))

(fn UpdatePathVisibility
  (Development|SetHiddeninGame (Variables|Default|GetSphere) (not (Variables|/Script/Kulagin.MapperContainerBase|GetbIsPathVisible (Variables|Default|GetParentContainer))) true)
  (return true))

(fn SetMaterial
  (params (NewMaterial :type Material%20Interface%20Object%20Reference))
  (Rendering|Material|SetMaterial (Variables|Default|GetSphere) 0 NewMaterial)
  (Rendering|Material|SetMaterial (Variables|Default|GetPlane) 0 NewMaterial)
  (return false))

(fn HideArrow
  (bind _arrowmesh (Variables|Default|GetArrowMesh))
  (Rendering|SetVisibility _arrowmesh false false)
  (Collision|SetCollisionProfileName _arrowmesh "NoCollision" :!class /Script/Engine.PrimitiveComponent)
  (return true))

(fn ShowArrow
  (bind _arrowmesh (Variables|Default|GetArrowMesh))
  (Rendering|SetVisibility _arrowmesh true false)
  (Collision|SetCollisionProfileName _arrowmesh "BlockAll" :!class /Script/Engine.PrimitiveComponent)
  (return true))