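; Main scene actor of the drone mapper, holding either imported procedural meshes or web map tiles, and georeferencing them.
; After import it enables query collision and spawns two orientation points seeded with lat/lon from NaviPoints.
; Orient converts both points to map coordinates, derives uniform scale and yaw from them, repositions the scene and passes the reference to the pawn.
; Helpers apply texture and heightmap materials and refresh MapperTile components.
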(event Custom|Orient
  (bind _returnvalue (Class|KulaginStatics|GetMapperGameMode))
  (bind _scene01 (Variables|Default|GetScene01))
  (bind _worldlocations (Variables|Default|GetWorldLocations))
  (bind _scene01_2 (Variables|Default|GetScene01))
  (bind _scene02 (Variables|Default|GetScene02))
  (bind _pointsactors (Variables|Default|GetPointsActors))
  (bind _worldlocations_2 (Variables|Default|GetWorldLocations))
  (bind _scene01_3 (Variables|Default|GetScene01))
  (bind _scene02_2 (Variables|Default|GetScene02))
  (bind _returnvalue_2 (Transformation|GetWorldLocation _scene01))
  (bind _returnvalue_3 (Transformation|GetWorldLocation _scene01_2))
  (bind _returnvalue_4 (Transformation|GetWorldLocation _scene02))
  (bind _output (Utilities|Array|Get(acopy) _worldlocations_2))
  (bind _output_2 (Utilities|Array|Get(acopy) _worldlocations_2 1))
  (bind _output_3 (Utilities|Array|Get(acopy) _pointsactors))
  (bind _output_4 (Utilities|Array|Get(acopy) _worldlocations))
  (bind _output_5 (Utilities|Array|Get(acopy) _worldlocations 1))
  (bind _pointcontainers (Variables|/Script/Kulagin.MapperGameMode|GetPointContainers _returnvalue))
  (bind _relativelocation (Variables|/Script/Engine.SceneComponent|GetRelativeLocation _scene02_2))
  (bind _relativelocation_2 (Variables|/Script/Engine.SceneComponent|GetRelativeLocation _scene01_3))
  (bind _returnvalue_5 (* _returnvalue_2 -1))
  (bind _returnvalue_6 (Math|Vector|Distance2D(Vector) (Math|Vector2D|MakeVector2D (.x _relativelocation) (.y _relativelocation)) (Math|Vector2D|MakeVector2D (.x _relativelocation_2) (.y _relativelocation_2))))
  (bind _returnvalue_7 (Math|Vector|Distance2D(Vector) (Math|Vector2D|MakeVector2D (.x _output) (.y _output)) (Math|Vector2D|MakeVector2D (.x _output_2) (.y _output_2))))
  (bind _returnvalue_8 (- _output_4 _output_5))
  (bind _returnvalue_9 (- _returnvalue_3 _returnvalue_4))
  (bind _pointstruct (Variables|/Game/DMA/Blueprints/BP_Point_Mission.BP_Point_Mission_C|GetPointStruct _output_3))
  (bind _returnvalue_10 (Math|Vector|Normalize (Math|Vector|MakeVector (.x _returnvalue_8) (.y _returnvalue_8) 0.0)))
  (bind _returnvalue_11 (Math|Vector|Normalize (Math|Vector|MakeVector (.x _returnvalue_9) (.y _returnvalue_9) 0.0)))
  (bind _returnvalue_12 (/ _returnvalue_7 _returnvalue_6))
  (bind _returnvalue_13 (Math|Vector|DotProduct _returnvalue_11 _returnvalue_10))
  (bind _returnvalue_14 (Class|KismetMathLibrary|DegAcos _returnvalue_13))
  (Development|PrintString "ORIENT START" true true "(R=1.000000,G=0.043376,B=0.000000,A=1.000000)")
  (Transformation|SetWorldLocation (Variables|Default|GetScene01) (Transformation|GetActorLocation (Utilities|Array|Get(acopy) (Variables|Default|GetPointsActors))) false false)
  (Transformation|SetWorldLocation (Variables|Default|GetScene02) (Transformation|GetActorLocation (Utilities|Array|Get(acopy) (Variables|Default|GetPointsActors) 1)) false false)
  (for _array_element (Variables|Default|GetPointsActors)
    _)
  (Variables|Default|SetReferenceLatLon (Class|KulaginStatics|GetReferenceLatLon _pointstruct))
  (Class|KulaginStatics|SetReference (.TargetLatLon (Utilities|Struct|BreakMissionPoint _pointstruct)))
  (for _array_element_2 (Variables|Default|GetPointsActors)
    (Utilities|Array|Add (Variables|Default|GetWorldLocations) (CallFunction|MaptoCoord (Variables|/Game/DMA/Blueprints/BP_Point_Mission.BP_Point_Mission_C|GetPointStruct _array_element_2) (Variables|Default|GetReferenceLatLon) 0.0)))
  (Transformation|SetActorRelativeScale3D (Math|Conversions|ToVector(Float) _returnvalue_12))
  (Development|PrintString (Utilities|String|Append "Scale: X = " (Utilities|String|ToString(Float) _returnvalue_7) "; Y = " (Utilities|String|ToString(Float) _returnvalue_6) "; Z = " (Utilities|String|ToString(Float) 0.0) "; Total = " (Utilities|String|ToString(Float) _returnvalue_12) "; dot = " (Utilities|String|ToString(Float) _returnvalue_13) "; ACosD = " (Utilities|String|ToString(Float) _returnvalue_14) "; v1 = " (Utilities|String|ToString(Vector) _returnvalue_11) "; v2 = " (Utilities|String|ToString(Vector) _returnvalue_10)))
  (Transformation|SetActorRotation (Math|Rotator|MakeRotator 0.0 0.0 (* _returnvalue_14 (Math|Float|Sign(Float) _returnvalue_13))))
  (Transformation|SetActorLocation (Math|Vector|MakeVector (.x _returnvalue_5) (.y _returnvalue_5) 0.0) false false)
  (Transformation|SetActorLocation (Game|Player|GetPlayerPawn 0) (+ (Transformation|GetWorldLocation (Variables|Default|GetScene01)) "0, 0,500.000000") false false)
  (bind _asbp_main_pawn (Utilities|Casting|CastToBP_Main_Pawn (Game|Player|GetPlayerPawn 0)))
  (Variables|/Game/DMA/Blueprints/Core/BP_Main_Pawn.BP_Main_Pawn_C|SetReferenceLatLon _asbp_main_pawn (Variables|Default|GetReferenceLatLon))
  (for _array_element_3 _pointcontainers
    (Class|MapperContainerBase|RemovePath _array_element_3))
  (Utilities|Array|Clear _pointcontainers)
  (Transformation|SetActorLocation (Game|Player|GetPlayerPawn 0) (+ (Transformation|GetWorldLocation (Variables|Default|GetScene01)) "0, 0,500.000000") false false))

(event Custom|OnEndImporting
  (bind _pointsactors (Variables|Default|GetPointsActors))
  (Variables|Default|SetbIsReadyToOrient true)
  (for _array_element (Actor|GetComponentsByClass "/Script/ProceduralMeshComponent.ProceduralMeshComponent")
    (Components|Activation|Deactivate _array_element)
    (Collision|SetCollisionEnabled _array_element "QueryOnly")
    (Collision|SetCollisionResponsetoAllChannels _array_element "ECR_Block")
    (Collision|SetCollisionObjectType _array_element "ECC_WorldStatic")
    (Components|Activation|Activate _array_element true))
  (Transformation|SetActorLocation (Game|Player|GetPlayerPawn 0) (+ (Transformation|GetWorldLocation (Variables|Default|GetScene01)) "0, 0,500.000000") false false)
  (for (_array_element_2 _array_index) (Utilities|Array|MakeArray (Transformation|GetWorldLocation (Variables|Default|GetScene01)) (Transformation|GetWorldLocation (Variables|Default|GetScene02)))
    (bind _returnvalue (Game|SpawnActorfromClass "/Game/DMA/Blueprints/BP_Point_Orient.BP_Point_Orient_C" (Math|Transform|MakeTransform _array_element_2 "0, 0, 0" "1,1,1") "AlwaysSpawn" 0 0))
    (Variables|/Game/DMA/Blueprints/BP_Point_Mission.BP_Point_Mission_C|SetbStaticPointStruct _returnvalue true)
    (Utilities|Array|Add (Variables|Default|GetPointsActors) _returnvalue)
    (Class|KulaginStatics|SetTargetLat (Variables|/Game/DMA/Blueprints/BP_Point_Mission.BP_Point_Mission_C|GetPointStruct _returnvalue) (.Lat (Utilities|Struct|BreakNaviPointStruct (Utilities|Array|Get(acopy) (Variables|Default|GetNaviPoints) _array_index))))
    (Class|KulaginStatics|SetTargetLon (Variables|/Game/DMA/Blueprints/BP_Point_Mission.BP_Point_Mission_C|GetPointStruct _returnvalue) (.Lon (Utilities|Struct|BreakNaviPointStruct (Utilities|Array|Get(acopy) (Variables|Default|GetNaviPoints) _array_index)))))
  (bind _returnvalue_2 (Game|SpawnActorfromClass "/Game/DMA/Blueprints/BP_Container_Orient.BP_Container_Orient_C" (Transformation|GetWorldTransform (Variables|Default|GetRoot)) "AlwaysSpawn" 0 0))
  (Utilities|Array|Add (Variables|/Game/DMA/Blueprints/BP_Container_Mission.BP_Container_Mission_C|GetNaviPointsActors _returnvalue_2) (Utilities|Array|Get(acopy) _pointsactors))
  (Utilities|Array|Add (Variables|/Game/DMA/Blueprints/BP_Container_Mission.BP_Container_Mission_C|GetNaviPointsActors _returnvalue_2) (Utilities|Array|Get(acopy) _pointsactors 1))
  (Utilities|Array|Add (Variables|/Script/Kulagin.MapperGameMode|GetPointContainers (Class|KulaginStatics|GetMapperGameMode)) _returnvalue_2))

(event EventBeginPlay
  (bind _gamemode (CallFunction|GetDroneMapperGamemode))
  (bind _tile (Variables|Default|GetTile))
  (Components|Tick|SetComponentTickEnabled (Variables|Default|GetTile) false)
  (Development|SetHiddeninGame (Variables|Default|GetTile) true false)
  (Default|SetMainScene _gamemode self)
  (if (Utilities|Enum|Equal(Enum) (Variables|/Game/DMA/Blueprints/Core/BP_Drone_Mapper_Gamemode.BP_Drone_Mapper_Gamemode_C|GetSceneType (CallFunction|GetDroneMapperGamemode)) "ST_Web")
    (bind _returnvalue (Class|KulaginStatics|UEtoLatLon (Transformation|GetActorLocation)))
    (bind _returnvalue_2 (Class|KulaginStatics|GetMapTile _returnvalue (Class|KulaginStatics|GetMaxZoom)))
    (Class|MapperGameMode|SetMaxZoomImages _gamemode (Utilities|Set|MakeSet (Utilities|Struct|MakeIntPoint (.GoogleX (Class|KulaginStatics|GetGoogleTile _returnvalue_2)) (.GoogleY (Class|KulaginStatics|GetGoogleTile _returnvalue_2)))))
    (Rendering|SetCastShadow _tile false)
    (Development|SetHiddeninGame _tile false false)
    (Class|MapperTileComponent|GetMapTileMaxZoom _tile)))

(event EventDestroyed
  (bind _asbp_main_pawn (Utilities|Casting|CastToBP_Main_Pawn (Game|Player|GetPlayerPawn 0)))
  (Variables|/Game/DMA/Blueprints/Core/BP_Main_Pawn.BP_Main_Pawn_C|SetReferenceLatLon _asbp_main_pawn (Utilities|Struct|MakeReferenceLatLon)))

(event EventTick
  (params (DeltaSeconds :type Float%20%28single-precision%29)))

(fn ConstructionScript
  (Transformation|SetRelativeScale3D (Variables|Default|GetTile) "1.005000,1.005000,1.005000"))

(fn SetTexture
  (params (Texture :type Texture%20Object%20Reference))
  (bind _astexture_2ddynamic (Utilities|Casting|CastToTexture2DDynamic Texture))
  (bind _output_get (LocalVariables|SetPlaneScale (Math|Vector2D|MakeVector2D (Math|Conversions|ToFloat(Integer) (Class|KulaginStatics|GetTexture2DDynamicSizeX _astexture_2ddynamic)) (Math|Conversions|ToFloat(Integer) (Class|KulaginStatics|GetTexture2DDynamicSizeY _astexture_2ddynamic)))))
  (bind _output_get_2 (LocalVariables|SetPlaneScale (/ _output_get (Math|Float|Max(Float) (.X (Math|Vector2D|BreakVector2D _output_get)) (.Y (Math|Vector2D|BreakVector2D _output_get))))))
  (Transformation|SetRelativeScale3D (Variables|Default|GetTile) (Math|Conversions|ToVector(Vector2D) _output_get_2 1.0))
  (bind _returnvalue (Rendering|Material|CreateDynamicMaterialInstance "/Game/DMA/MaterialLibrary/M_Test_Texture_01.M_Test_Texture_01" "None" :!class /Script/Engine.KismetMaterialLibrary))
  (Rendering|Material|SetTextureParameterValue _returnvalue "Tex" Texture)
  (Rendering|Material|SetMaterial (Variables|Default|GetTile) 0 _returnvalue)
  (Development|SetHiddeninGame (Variables|Default|GetTile) false false))

(fn SetHighmap
  (params (Highmap :type Texture%20Object%20Reference))
  (Utilities|IsValid Highmap
    (:Is%20Valid
      (bind _asmaterial_instance_dynamic (Utilities|Casting|CastToMaterialInstanceDynamic (Rendering|Material|GetMaterial (Variables|Default|GetTile) 0)))
      (Rendering|Material|SetTextureParameterValue _asmaterial_instance_dynamic "Highmap" Highmap))))

(fn GetCorners
  (return (Utilities|Array|MakeArray (Variables|Default|GetCornerTopLeft) (Variables|Default|GetCornerTopRight) (Variables|Default|GetCornerBottomLeft) (Variables|Default|GetCornerBottomRight))))

(fn OrientTopLeftBottomRight
  (params (TopLeft :type Mission%20Point%20Structure) (BottomRight :type Mission%20Point%20Structure))
  (for _index (range 0 1)
    (Variables|/Game/DMA/Blueprints/BP_Point_Mission.BP_Point_Mission_C|SetPointStruct (Utilities|Array|Get(acopy) (Variables|Default|GetPointsActors) _index) (Utilities|Array|Get(acopy) (Utilities|Array|MakeArray TopLeft BottomRight) _index))
    (Transformation|SetActorLocation (Utilities|Array|Get(acopy) (Variables|Default|GetPointsActors) _index) (Transformation|GetWorldLocation (Utilities|Array|Get(acopy) (Utilities|Array|MakeArray (Variables|Default|GetCornerTopLeft) (Variables|Default|GetCornerBottomRight)) _index)) false false))
  (CallFunction|Orient))

(fn SetTileMaterial
  (params (Tile :type Mapper%20Tile%20Component%20Object%20Reference))
  (bind _returnvalue (Rendering|Material|CreateDynamicMaterialInstance "/Game/DMA/MaterialLibrary/M_MapTile.M_MapTile" "None" :!class /Script/Engine.KismetMaterialLibrary))
  (Rendering|Material|SetMaterial Tile 0 _returnvalue))

(fn SetVisibleTilesMaxZoom
  (for _array_element (Actor|GetComponentsByClass "/Script/Kulagin.MapperTileComponent")
    (if (Class|MapperTileComponent|IsinRenderDistance _array_element)
      (Class|MapperTileComponent|GetMapTileMaxZoom _array_element))))

(fn UpdateAllTiles
  (bind _output_get (LocalVariables|SetCurrentTiles (Actor|GetComponentsByClass "/Script/Kulagin.MapperTileComponent")))
  (for _array_element _output_get
    (Class|MapperTileComponent|UpdateTile _array_element))
  (Development|PrintString (Utilities|String|Append "UpdateTile: Final number of tiles: " (Utilities|String|ToString(Integer) (Utilities|Array|Length (Actor|GetComponentsByClass "/Script/Kulagin.MapperTileComponent"))))))

(fn SetWebTiles
  (params (TopLeft :type Boolean) (NewParam1 :type Boolean)))