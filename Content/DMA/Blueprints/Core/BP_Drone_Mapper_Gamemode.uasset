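; Game mode for a drone mission mapper that manages the georeferenced scene, mission routes and scene lighting.
; Scenes come from FBX, image or web map tiles, or from preset levels oriented by data-table reference points with level actors attached.
; Selected mission and log files are parsed by extension into containers of point actors with menu widgets, and their bounds can size web imports.
; Tagged sky and light actors drive time-of-day and lighting toggles.
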(event Custom|ImportImage
  (params (FilePath :type Binary%20File%20Path%20Structure%20%28by%20ref%29))
  (Variables|Default|SetSceneType "ST_Image")
  (bind _texture (|DownloadImage (Utilities|String|Append "file://" (Class|KulaginStatics|GetBinaryFullPath FilePath)))
    (:OnSuccess
      (CallFunction|CreateScenewithImage _texture))))

(event Custom|ImportHighmap
  (bind (_path _returnvalue) (Class|KulaginStatics|AskUserforFile "Select highmap" "Image scene|*.jpg;*.jpeg;*.png"))
  (if _returnvalue
    (bind _texture (|DownloadImage (Utilities|String|Append "file://" (Class|KulaginStatics|GetBinaryFullPath _path)))
      (:OnSuccess
        (Default|SetHighmap (Variables|Default|GetMainScene) _texture)))))

(event Custom|ImportFromWeb
  (params (bLoadMission :type Boolean) (bProvidedCenter :type Boolean) (Radius :type Float%20%28single-precision%29) (Center :type Lat%20Lon%20Structure))
  (if bLoadMission
    (bind (_bsuccess _topleft _bottomright _missionlists _loglists) (CallFunction|SelectFiles))
    (bind _returnvalue (Class|KulaginStatics|LatLontoUE _topleft 0.0))
    (bind _returnvalue_2 (Class|KulaginStatics|LatLontoUE _bottomright 0.0))
    (CallFunction|ImportfromWebFunc _missionlists _loglists (select bProvidedCenter Center (Class|KulaginStatics|LatLonCenter _topleft _bottomright)) (Math|Float|Max(Float) (Class|KulaginStatics|UUtoLife (Math|Vector|Distance(Vector) _returnvalue_2 _returnvalue)) Radius))
    (elif bProvidedCenter
      (CallFunction|ImportfromWebFunc (Utilities|Array|MakeArray) (Utilities|Array|MakeArray) Center Radius))))

(event Custom|SetDroneSize
  (params (Size :type Float%20%28single-precision%29))
  (bind _outactors (Actor|GetAllActorsOfClass "/Game/DMA/Blueprints/Core/BP_Moving_Actor.BP_Moving_Actor_C"))
  (for _array_element _outactors
    (Transformation|SetActorScale3D _array_element (Math|Conversions|ToVector(Float) Size))))

(event Custom|MakeIgnore
  (Utilities|Array|Clear (Variables|Default|GetActorsToIgnore))
  (for _array_element (Utilities|Array|MakeArray "/Script/Engine.PlanarReflection" "/Game/AGameAssets/Maps/UPN/Details/Vishka/Vishka_BP.Vishka_BP_C" "/Game/AGameAssets/Maps/UPN/Details/Trubu/fire.fire_C" "/Game/AGameAssets/Maps/UPN/Details/Fanar_Stolb1/Fanar_Stolb1_BP.Fanar_Stolb1_BP_C" "/Script/Engine.Emitter" "/Script/Kulagin.MapperPointBase" "/Script/Kulagin.MapperDroneBase")
    (bind _outactors (Actor|GetAllActorsOfClass _array_element))
    (Utilities|Array|AppendArray (Variables|Default|GetActorsToIgnore) _outactors))
  (Development|PrintString "DONE"))

(event EventBeginPlay
  (bind _outactors (Actor|GetAllActorsOfClass "/Game/Blueprints/DronesGroup_Blueprints/TargetPoints/TargetPoint_Actor.TargetPoint_Actor_C"))
  (for _array_element _outactors
    (Rendering|SetActorHiddenInGame _array_element true))
  (bind _outactors_2 (Actor|GetAllActorswithTag "DirectLight"))
  (for _array_element_2 _outactors_2
    (bind _asdirectional_light (Utilities|Casting|CastToDirectionalLight _array_element_2))
    (Variables|Default|SetDirectLight _asdirectional_light))
  (bind _outactors_3 (Actor|GetAllActorswithTag "SkyLight"))
  (for _array_element_3 _outactors_3
    (bind _assky_light (Utilities|Casting|CastToSkyLight _array_element_3))
    (Variables|Default|SetSkyLight _assky_light))
  (bind _outactors_4 (Actor|GetAllActorswithTag "SkySphere"))
  (for _array_element_4 _outactors_4
    (bind _asbp_sky_sphere (Utilities|Casting|CastToBP_Sky_Sphere _array_element_4))
    (Variables|Default|SetSkySphere _asbp_sky_sphere)))

(event EventTick
  (params (DeltaSeconds :type Float%20%28single-precision%29)))

(event EventHandleStartingNewPlayer
  (params (NewPlayer :type Player%20Controller%20Object%20Reference))
  (Variables|Default|SetSceneType "ST_Empty")
  (Variables|Default|SetImportStage "ST_Ready")
  (bind _returnvalue (Class|DataTableFunctionLibrary|DoesDataTableRowExist "/Game/DMA/Data/DT_MapperLevelData.DT_MapperLevelData" (Variables|/Script/Kulagin.MapperGameInstance|GetLevelName (Class|KulaginStatics|GetMapperGameInstance))))
  (if _returnvalue
    (bind _returnvalue_2 (Game|SpawnActorfromClass "/Game/DMA/Blueprints/Core/BP_Main_Scene.BP_Main_Scene_C" (Math|Transform|MakeTransform "0, 0, 0" "0, 0, 0" "1,1,1") "AlwaysSpawn" 0 0))
    (Variables|Default|SetMainScene _returnvalue_2)
    (Default|OnEndImporting (Variables|Default|GetMainScene))
    (CallFunction|SetMainSceneLevelValue)
    (for _array_element (Utilities|Array|MakeArray "/Script/Engine.StaticMeshActor" "/Script/Engine.PlanarReflection" "/Game/AGameAssets/Maps/UPN/Details/Vishka/Vishka_BP.Vishka_BP_C" "/Game/AGameAssets/Maps/UPN/Details/Trubu/fire.fire_C" "/Game/AGameAssets/Maps/UPN/Details/Fanar_Stolb1/Fanar_Stolb1_BP.Fanar_Stolb1_BP_C" "/Script/Engine.Emitter")
      (bind _outactors (Actor|GetAllActorsOfClass _array_element))
      (for _array_element_2 _outactors
        (Transformation|AttachActorToActor _array_element_2 (Variables|Default|GetMainScene) "None" "KeepRelative" "KeepRelative" "KeepRelative" true)))
    (bind _outactors_2 (Actor|GetAllActorsOfClass "/Script/Foliage.InstancedFoliageActor"))
    (for _array_element_3 _outactors_2
      (Transformation|SetMobility (Variables|/Script/Engine.Actor|GetRootComponent _array_element_3) "Movable")
      (for _array_element_4 (Components|GetChildrenComponents (Variables|/Script/Engine.Actor|GetRootComponent _array_element_3) true)
        (Transformation|SetMobility _array_element_4 "Movable"))
      (Transformation|AttachActorToActor _array_element_3 (Variables|Default|GetMainScene) "None" "KeepRelative" "KeepRelative" "KeepRelative" true))
    (Default|Orient (Variables|Default|GetMainScene))))

(fn ConstructionScript)

(fn SetMainScene
  (params (MainScene :type BP%20Main%20Scene%20Object%20Reference))
  (Variables|Default|SetMainScene MainScene))

(fn SetFBXImportManager
  (params (ImportManager :type BP%20Kulagin%20Import%20Manager%20Object%20Reference))
  (Variables|Default|SetFBXImportManager ImportManager))

(fn ImportMesh
  (params (FilePath :type Binary%20File%20Path%20Structure%20%28by%20ref%29))
  (Variables|Default|SetSceneType "ST_Mesh")
  (Default|ImportFBX (Variables|Default|GetFBXImportManager) FilePath "0, 0, 0"))

(fn Orient
  (Default|Orient (Variables|Default|GetMainScene))
  (Variables|Default|SetImportStage "ST_Ready"))

(fn ImportScene
  (bind (_path _returnvalue) (Class|KulaginStatics|AskUserforFile "Select scene" "Mesh scene|*.fbx|Image scene|*.jpg;*.jpeg;*.png"))
  (if _returnvalue
    (CallFunction|CleanScene)
    (Variables|Default|SetImportStage "ST_ImportingScene")
    (if (Utilities|Enum|Equal(Enum) (.Extension (Utilities|Struct|BreakBinaryFilePath _path)) "fbx")
      (CallFunction|ImportMesh _path)
      (else
        (CallFunction|ImportImage _path)))))

(fn CleanScene
  (Utilities|IsValid (Variables|Default|GetMainScene)
    (:Is%20Valid
      (Actor|DestroyActor (Variables|Default|GetMainScene)))
    (:Is%20Not%20Valid
      _))
  (Widget|Panel|ClearChildren (Variables|/Game/DMA/UI/Widgets/MenuWidget.MenuWidget_C|GetContainersHolder (Variables|/Game/DMA/Blueprints/Core/BP_Main_Pawn.BP_Main_Pawn_C|GetMenuWidget (CallFunction|GetDroneMapperPawn))))
  (bind _arrayelement (Utilities|Array|ReverseforEachLoop (Variables|/Script/Kulagin.MapperGameMode|GetPointContainers (Class|KulaginStatics|GetMapperGameMode)))
    (:LoopBody
      (Class|MapperContainerBase|RemovePath _arrayelement))))

(fn OnImportSceneDone
  (params (MainScene :type BP%20Main%20Scene%20Object%20Reference))
  (CallFunction|SetMainScene MainScene)
  (Variables|Default|SetImportStage "ST_Orientating")
  (Default|OnEndImporting (Variables|Default|GetMainScene)))

(fn OrientfromFile
  (bind _mainscene (Variables|Default|GetMainScene))
  (bind _pointsactors (Variables|/Game/DMA/Blueprints/Core/BP_Main_Scene.BP_Main_Scene_C|GetPointsActors _mainscene))
  (for _array_element _pointsactors
    (Utilities|Array|Add (LocalVariables|GetLocalPoints) (Variables|/Game/DMA/Blueprints/BP_Point_Drone_Mission.BP_Point_Drone_Mission_C|GetPointData _array_element)))
  (bind _returnvalue (Class|KulaginStatics|SetOrientActorsfromFile (LocalVariables|GetLocalPoints) _pointsactors (Variables|Default|GetTexture) (Default|GetCorners _mainscene)))
  (if _returnvalue
    (for (_array_element_2 _array_index) (Variables|/Game/DMA/Blueprints/Core/BP_Main_Scene.BP_Main_Scene_C|GetPointsActors (Variables|Default|GetMainScene))
      (Variables|/Game/DMA/Blueprints/BP_Point_Drone_Mission.BP_Point_Drone_Mission_C|SetPointData _array_element_2 (Utilities|Array|Get(acopy) (LocalVariables|GetLocalPoints) _array_index)))
    (CallFunction|Orient)))

(fn CreateScenewithImage
  (params (Texture :type Texture%202D%20Dynamic%20Object%20Reference))
  (Variables|Default|SetTexture Texture)
  (bind _returnvalue (Game|SpawnActorfromClass "/Game/DMA/Blueprints/Core/BP_Main_Scene.BP_Main_Scene_C" (Math|Transform|MakeTransform "0, 0, 0" "0, 0, 0" "1,1,1") "AlwaysSpawn" 0 0))
  (Default|SetTexture _returnvalue (Variables|Default|GetTexture))
  (Transformation|SetActorScale3D _returnvalue (Math|Vector|MakeVector (/ 1.25e+03 (Math|Float|Max(Float) (.x (.BoxExtent (Collision|GetActorBounds _returnvalue false))) (.y (.BoxExtent (Collision|GetActorBounds _returnvalue false))) (.z (.BoxExtent (Collision|GetActorBounds _returnvalue false))))) (/ 1.25e+03 (Math|Float|Max(Float) (.x (.BoxExtent (Collision|GetActorBounds _returnvalue false))) (.y (.BoxExtent (Collision|GetActorBounds _returnvalue false))) (.z (.BoxExtent (Collision|GetActorBounds _returnvalue false))))) (/ 1.25e+03 (Math|Float|Max(Float) (.x (.BoxExtent (Collision|GetActorBounds _returnvalue false))) (.y (.BoxExtent (Collision|GetActorBounds _returnvalue false))) (.z (.BoxExtent (Collision|GetActorBounds _returnvalue false)))))))
  (CallFunction|OnImportSceneDone _returnvalue))

(fn LoadLog
  (params (List :type Log%20Point%20List%20Structure%20%28by%20ref%29))
  (bind (_filepath _points) (Utilities|Struct|BreakLogPointList List))
  (bind _output_get (LocalVariables|SetPointsLocal _points))
  (if (Utilities|Array|IsValidIndex _output_get 1)
    (bind _returnvalue (Game|SpawnActorfromClass "/Game/DMA/Blueprints/BP_Container_Log.BP_Container_Log_C" (Math|Transform|MakeTransform "0, 0, 0" "0, 0, 0" "1,1,1") "AlwaysSpawn" 0 0))
    (bind _output_get_2 (LocalVariables|SetCurrentContainer _returnvalue))
    (Utilities|Array|Add (Variables|/Script/Kulagin.MapperGameMode|GetPointContainers (Class|KulaginStatics|GetMapperGameMode)) _output_get_2)
    (bind _returnvalue_2 (Class|KulaginStatics|LogPointtoUE (Utilities|Array|Get(acopy) (LocalVariables|GetPointsLocal)) 0.0))
    (Variables|/Game/DMA/Blueprints/BP_Container_Log.BP_Container_Log_C|SetStartAlt (LocalVariables|GetCurrentContainer) (CallFunction|GetStartAlt _returnvalue_2))
    (for _array_element (LocalVariables|GetPointsLocal)
      (bind _returnvalue_3 (Game|SpawnActorfromClass "/Game/DMA/Blueprints/BP_Point_Log.BP_Point_Log_C" (Math|Transform|MakeTransform "0, 0, 0" "0, 0, 0" "1,1,1") "AlwaysSpawn" 0 0))
      (Utilities|Array|Add (Variables|/Script/Kulagin.MapperContainerBase|GetPointActors (LocalVariables|GetCurrentContainer)) _returnvalue_3)
      (Variables|/Game/DMA/Blueprints/BP_Point_Log.BP_Point_Log_C|SetStartAlt_0 _returnvalue_3 (Variables|/Game/DMA/Blueprints/BP_Container_Log.BP_Container_Log_C|GetStartAlt (LocalVariables|GetCurrentContainer)))
      (Default|SetPointStruct _returnvalue_3 _array_element)
      (Utilities|IsValid (LocalVariables|GetTempPoint)
        (:Is%20Valid
          (Default|SetNextPointBP (LocalVariables|GetTempPoint) _returnvalue_3))
        (:Is%20Not%20Valid
          _))
      (LocalVariables|SetTempPoint _returnvalue_3))
    (Variables|/Script/Kulagin.MapperContainerBase|SetFilePath (LocalVariables|GetCurrentContainer) _filepath)
    (Class|MapperContainerBase|SetPointsMaterial (LocalVariables|GetCurrentContainer))
    (Class|MapperContainerBase|SetPointsColor (LocalVariables|GetCurrentContainer) "(R=0.007843,G=0.007843,B=0.007843,A=1.000000)")
    (Default|CreateNaviPointsWidget (Variables|/Game/DMA/Blueprints/Core/BP_Main_Pawn.BP_Main_Pawn_C|GetMenuWidget (CallFunction|GetDroneMapperPawn)) (LocalVariables|GetCurrentContainer))
    (return "" "")))

(fn LoadHighRes
  (Default|SetVisibleTilesMaxZoom (Variables|Default|GetMainScene)))

(fn SelectFiles
  (LocalVariables|SetTopLeftLocal (Class|KulaginStatics|GetLatLonBottomRight))
  (LocalVariables|SetBottomRightLocal (Class|KulaginStatics|GetLatLonTopLeft))
  (bind _returnvalue (Class|KulaginStatics|AskUserforFiles "Select Mission Files" (Utilities|String|Append "All|*.bin;*.txt;*plane;*car;*human" "|" "Binary Files|*.bin" "|" "Log Files|*.txt" "|" "Plane mission|*.plane" "|" "Car mission|*.car" "|" "Human mission|*.human")))
  (for _array_element _returnvalue
    (bind _output_get (LocalVariables|SetCurrentFileLocal _array_element))
    (switch string (Utilities|Struct|BreakBinaryFilePath _output_get)
      (:Default
        (bind _returnvalue_2 (Class|KulaginStatics|GetLogPointsfromFile (LocalVariables|GetCurrentFileLocal)))
        (Utilities|Array|Add (LocalVariables|GetLogListsLocal) _returnvalue_2)
        (LocalVariables|SetTopLeftLocal (Class|KulaginStatics|LatLonTopLeft (LocalVariables|GetTopLeftLocal) (.TopLeft (Utilities|Struct|BreakLogPointList _returnvalue_2))))
        (LocalVariables|SetBottomRightLocal (Class|KulaginStatics|LatLonBottomRight (.BottomRight (Utilities|Struct|BreakLogPointList _returnvalue_2)) (LocalVariables|GetBottomRightLocal)))
        (LocalVariables|SetbSuccessLocal true))
      (:bin
        (bind _returnvalue_3 (Class|KulaginStatics|GetPointsfromFile (LocalVariables|GetCurrentFileLocal)))
        (Utilities|Array|Add (LocalVariables|GetMissionListsLocal) _returnvalue_3)
        (LocalVariables|SetTopLeftLocal (Class|KulaginStatics|LatLonTopLeft (LocalVariables|GetTopLeftLocal) (.TopLeft (Utilities|Struct|BreakMissionPointList _returnvalue_3))))
        (LocalVariables|SetBottomRightLocal (Class|KulaginStatics|LatLonBottomRight (.BottomRight (Utilities|Struct|BreakMissionPointList _returnvalue_3)) (LocalVariables|GetBottomRightLocal)))
        (LocalVariables|SetbSuccessLocal true))
      (:plane
        (bind _returnvalue_4 (Class|KulaginStatics|GetPlanePointsfromFile (LocalVariables|GetCurrentFileLocal)))
        (Utilities|Array|Add (LocalVariables|GetMissionListsLocal) _returnvalue_4)
        (LocalVariables|SetTopLeftLocal (Class|KulaginStatics|LatLonTopLeft (LocalVariables|GetTopLeftLocal) (.TopLeft (Utilities|Struct|BreakMissionPointList _returnvalue_4))))
        (LocalVariables|SetBottomRightLocal (Class|KulaginStatics|LatLonBottomRight (.BottomRight (Utilities|Struct|BreakMissionPointList _returnvalue_4)) (LocalVariables|GetBottomRightLocal)))
        (LocalVariables|SetbSuccessLocal true))
      (:car
        (bind _returnvalue_5 (Class|KulaginStatics|GetCarPointsfromFile (LocalVariables|GetCurrentFileLocal)))
        (Utilities|Array|Add (LocalVariables|GetMissionListsLocal) _returnvalue_5)
        (LocalVariables|SetTopLeftLocal (Class|KulaginStatics|LatLonTopLeft (LocalVariables|GetTopLeftLocal) (.TopLeft (Utilities|Struct|BreakMissionPointList _returnvalue_5))))
        (LocalVariables|SetBottomRightLocal (Class|KulaginStatics|LatLonBottomRight (.BottomRight (Utilities|Struct|BreakMissionPointList _returnvalue_5)) (LocalVariables|GetBottomRightLocal)))
        (LocalVariables|SetbSuccessLocal true))
      (:human
        (bind _returnvalue_6 (Class|KulaginStatics|GetHumanPointsfromFile (LocalVariables|GetCurrentFileLocal)))
        (Utilities|Array|Add (LocalVariables|GetMissionListsLocal) _returnvalue_6)
        (LocalVariables|SetTopLeftLocal (Class|KulaginStatics|LatLonTopLeft (LocalVariables|GetTopLeftLocal) (.TopLeft (Utilities|Struct|BreakMissionPointList _returnvalue_6))))
        (LocalVariables|SetBottomRightLocal (Class|KulaginStatics|LatLonBottomRight (.BottomRight (Utilities|Struct|BreakMissionPointList _returnvalue_6)) (LocalVariables|GetBottomRightLocal)))
        (LocalVariables|SetbSuccessLocal true))))
  (return (LocalVariables|GetbSuccessLocal) (LocalVariables|GetTopLeftLocal) (LocalVariables|GetBottomRightLocal) (LocalVariables|GetMissionListsLocal) (LocalVariables|GetLogListsLocal)))

(fn LoadDroneMission
  (params (List :type Mission%20Point%20List%20Structure%20%28by%20ref%29))
  (bind (_filepath _type _topleft _bottomright _dronepoints) (Utilities|Struct|BreakMissionPointList List))
  (bind _asbp_main_pawn (Utilities|Casting|CastToBP_Main_Pawn (Game|Player|GetPlayerPawn 0)))
  (Default|OpenandLoadFile _asbp_main_pawn _dronepoints _filepath)
  (return))

(fn LoadAllMissions
  (params (MissionLists :type Array%20of%20Mission%20Point%20List%20Structures))
  (for _array_element MissionLists
    (CallFunction|LoadMission _array_element)))

(fn LoadAllLogs
  (params (LogLists :type Array%20of%20Log%20Point%20List%20Structures))
  (for _array_element LogLists
    (CallFunction|LoadLog _array_element)))

(fn SelectandLoadFiles
  (bind (_bsuccess _topleft _bottomright _missionlists _loglists) (CallFunction|SelectFiles))
  (if _bsuccess
    (CallFunction|LoadAllLists _missionlists _loglists)))

(fn SetMainSceneLevelValue
  (bind _returnvalue (Utilities|GetDataTableRow "/Game/DMA/Data/DT_MapperLevelData.DT_MapperLevelData" (Variables|/Script/Kulagin.MapperGameInstance|GetLevelName (Class|KulaginStatics|GetMapperGameInstance)))
    (:then
      (LocalVariables|SetLatLonCurrent (.latlon _returnvalue))
      (LocalVariables|SetLocationsCurrent (.locations _returnvalue))
      (for (_array_element _array_index) (Variables|/Game/DMA/Blueprints/Core/BP_Main_Scene.BP_Main_Scene_C|GetPointsActors (Variables|Default|GetMainScene))
        (Utilities|Struct|SetmembersinMissionPoint (Variables|/Game/DMA/Blueprints/BP_Point_Drone_Mission.BP_Point_Drone_Mission_C|GetPointData _array_element) (Class|KulaginStatics|LatLonfromFloat (.X (Math|Vector2D|BreakVector2D (Utilities|Array|Get(acopy) (LocalVariables|GetLatLonCurrent) _array_index))) (.Y (Math|Vector2D|BreakVector2D (Utilities|Array|Get(acopy) (LocalVariables|GetLatLonCurrent) _array_index)))))
        (Transformation|SetActorLocation _array_element (Utilities|Array|Get(acopy) (LocalVariables|GetLocationsCurrent) _array_index) false false))
      (return))
    (:RowNotFound
      (return))))

(fn GetSceneActor
  (return (Variables|Default|GetMainScene)))

(fn UpdateAllDangerZones
  (|CallParentFunction)
  (for _array_element (Variables|Default|GetPointContainers)
    (bind _asw_mission_timeline (Utilities|Casting|CastToW_Mission_Timeline (Variables|/Script/Kulagin.MapperContainerBase|GetTimelineWidget _array_element)))
    (Default|UpdateTimeline _asw_mission_timeline))
  (return false))

(fn LoadPlaneMissionsAll
  (params (PlaneMissionLists :type Array%20of%20Mission%20Point%20List%20Structures))
  (for _array_element PlaneMissionLists
    (CallFunction|LoadMission _array_element)))

(fn LoadAllLists
  (params (MissionLists :type Array%20of%20Mission%20Point%20List%20Structures) (LogLists :type Array%20of%20Log%20Point%20List%20Structures))
  (CallFunction|LoadAllMissions MissionLists)
  (CallFunction|LoadAllLogs LogLists))

(fn LoadMission
  (params (List :type Mission%20Point%20List%20Structure))
  (LocalVariables|SetLastIndexLocal (- (Class|KulaginStatics|GetListLength List) 1))
  (bind _returnvalue (Game|SpawnActorfromClass (CallFunction|GetContainerClass (.type List)) (Math|Transform|MakeTransform "0, 0, 0" "0, 0, 0" "1,1,1") "AlwaysSpawn" 0 0))
  (bind _asbp_container_interactive (Utilities|Casting|CastToBP_Container_Interactive _returnvalue))
  (bind _output_get (LocalVariables|SetLocalContainer _asbp_container_interactive))
  (Variables|/Script/Kulagin.MapperContainerBase|SetFilePath _output_get (.filepath List))
  (bind _returnvalue_2 (Class|KulaginStatics|LatLontoUE (Class|KulaginStatics|GetListLatLon List) 0.0))
  (bind _output_get_2 (LocalVariables|SetFirstLocationLocal _returnvalue_2))
  (LocalVariables|SetLocalStartAlt (CallFunction|GetStartAlt _output_get_2))
  (for _index (range 0 (LocalVariables|GetLastIndexLocal))
    (bind _returnvalue_3 (Game|SpawnActorfromClass (CallFunction|GetPointClass (.type List)) (Math|Transform|MakeTransform (LocalVariables|GetFirstLocationLocal) "0, 0, 0" "1,1,1") "AlwaysSpawn" 0 0))
    (bind _asbp_point_interactive (Utilities|Casting|CastToBP_Point_Interactive _returnvalue_3))
    (bind _output_get_3 (LocalVariables|SetSpawnedPoint _asbp_point_interactive))
    (Variables|/Script/Kulagin.MapperPointInteractive|SetParentContainer _output_get_3 (LocalVariables|GetLocalContainer))
    (Variables|/Script/Kulagin.MapperPointInteractive|SetTargetPoint (LocalVariables|GetSpawnedPoint) (Utilities|Array|Get(acopy) (Variables|/Script/Kulagin.MapperContainerBase|GetPointActors (LocalVariables|GetLocalContainer)) (Utilities|Array|LastIndex (Variables|/Script/Kulagin.MapperContainerBase|GetPointActors (LocalVariables|GetLocalContainer)))))
    (Class|MapperPointBase|SetDatafromList (LocalVariables|GetSpawnedPoint) List _index)
    (Variables|/Script/Kulagin.MapperPointBase|SetStartAlt (LocalVariables|GetSpawnedPoint) (LocalVariables|GetLocalStartAlt))
    (Class|MapperPointBase|UpdateActorfromData (LocalVariables|GetSpawnedPoint))
    (Class|MapperPointInteractive|SetPointIndex (LocalVariables|GetSpawnedPoint) _index)
    (Utilities|Array|Add (Variables|/Script/Kulagin.MapperContainerBase|GetPointActors (LocalVariables|GetLocalContainer)) (LocalVariables|GetSpawnedPoint)))
  (Class|MapperContainerBase|SetPointsMaterial (LocalVariables|GetLocalContainer))
  (Class|MapperContainerBase|SetPointsColor (LocalVariables|GetLocalContainer) "(R=0.007843,G=0.007843,B=0.007843,A=1.000000)")
  (Default|UpdateFirstLastPoint (LocalVariables|GetLocalContainer))
  (Default|CalculatePointsTimes (LocalVariables|GetLocalContainer))
  (bind _asbp_main_pawn (Utilities|Casting|CastToBP_Main_Pawn (Game|Player|GetPlayerPawn 0)))
  (Default|CreateNaviPointsWidget (Variables|/Game/DMA/Blueprints/Core/BP_Main_Pawn.BP_Main_Pawn_C|GetMenuWidget _asbp_main_pawn) (LocalVariables|GetLocalContainer))
  (Default|UpdateCrossRadius (LocalVariables|GetLocalContainer))
  (Utilities|Array|Add (Variables|/Script/Kulagin.MapperGameMode|GetPointContainers (Class|KulaginStatics|GetMapperGameMode)) (LocalVariables|GetLocalContainer)))

(fn OnTimeOfDayChanged
  (params (TimeOfDay :type Float%20%28single-precision%29))
  (Transformation|SetActorRotation (Variables|Default|GetDirectLight) (Math|Rotator|MakeRotator 0.0 TimeOfDay 0.0))
  (Default|RefreshMaterial (Variables|Default|GetSkySphere)))

(fn OnSceneLightChanged
  (params (bEnable :type Boolean))
  (bind _directlight (Variables|Default|GetDirectLight))
  (bind _skylight (Variables|Default|GetSkyLight))
  (Utilities|IsValid _directlight
    (:Is%20Valid
      (Rendering|Components|Light|SetIntensity (Variables|/Script/Engine.Light|GetLightComponent _directlight) (select bEnable 2.75 0.0)))
    (:Is%20Not%20Valid
      _))
  (Utilities|IsValid _skylight
    (:Is%20Valid
      (Rendering|Components|Light|SetIntensity (Variables|/Script/Engine.SkyLight|GetLightComponent _skylight) (select bEnable 4.0 0.5)))))

(fn ImportfromWebFunc
  (params (MissionLists :type Array%20of%20Mission%20Point%20List%20Structures) (LogLists :type Array%20of%20Log%20Point%20List%20Structures) (Center :type Lat%20Lon%20Structure) (Radius :type Float%20%28single-precision%29))
  (bind _returnvalue (Class|KulaginStatics|LifetoUU Radius))
  (CallFunction|CleanScene)
  (Variables|Default|SetSceneType "ST_Web")
  (Variables|Default|SetImportStage "ST_Ready")
  (bind _returnvalue_2 (Class|KulaginStatics|GetMapTile Center (Class|KulaginStatics|GetMaxZoom)))
  (Development|PrintString (Utilities|String|Append "google x: " (Utilities|String|ToString(Integer) (.GoogleX (Class|KulaginStatics|GetGoogleTile _returnvalue_2))) ",, y: " (Utilities|String|ToString(Integer) (.GoogleY (Class|KulaginStatics|GetGoogleTile _returnvalue_2)))))
  (Class|KulaginStatics|SetReference (.Center (Utilities|Struct|BreakMapTileInfo _returnvalue_2)))
  (bind _returnvalue_3 (Class|KulaginStatics|LatLontoUE (.Center (Utilities|Struct|BreakMapTileInfo _returnvalue_2)) 0.0))
  (bind _returnvalue_4 (Game|SpawnActorfromClass "/Game/DMA/Blueprints/Core/BP_Main_Scene.BP_Main_Scene_C" (Math|Transform|MakeTransform "0, 0, 0" "0,90.000000, 0" (Math|Vector|MakeVector (/ (.SizeX (Class|KulaginStatics|GetMapTileSize _returnvalue_2)) 1e+02) (/ (.SizeY (Class|KulaginStatics|GetMapTileSize _returnvalue_2)) 1e+02) 1.0)) "AlwaysSpawn" 0 0))
  (bind _returnvalue_5 (Class|KulaginStatics|UEtoLatLon (+ _returnvalue_3 (Math|Vector|MakeVector _returnvalue _returnvalue 0.0))))
  (bind _returnvalue_6 (Class|KulaginStatics|UEtoLatLon (- _returnvalue_3 (Math|Vector|MakeVector _returnvalue _returnvalue 0.0))))
  (Class|KulaginStatics|SpawnDefaultTiles (Variables|/Script/Engine.Actor|GetRootComponent _returnvalue_4) (Class|KulaginStatics|LatLonTopLeft _returnvalue_6 _returnvalue_5) (Class|KulaginStatics|LatLonBottomRight _returnvalue_6 _returnvalue_5))
  (CallFunction|LoadAllLists MissionLists LogLists))