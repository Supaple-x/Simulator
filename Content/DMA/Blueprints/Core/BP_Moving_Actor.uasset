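; Moving drone actor that flies the mission points of its attached container, using the look chosen by the game instance's drone name.
; BeginPlay reads DT_DroneData to show a skeletal or static mesh or spawn an attached child actor.
; Tick interpolates at constant, point-supplied speed unless paused; SetTarget handles loiter delays and heading turns, then advances the point.
; Drop and Rise toggle mesh physics or forward to a BP_Drone_01 child.
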(event Custom|StartMoving
  (Variables|Default|SetCurrentPoint 0)
  (Variables|Default|SetTargetPoint 0)
  (CallFunction|SetTarget)
  (Utilities|IsValid 0
    (:Is%20Valid
      (bind _outpoints (Class|MapperContainerBase|GetPointsOfClass (Variables|Default|GetAttachedToContainer) "/Game/DMA/Blueprints/BP_Point_Drone_Mission.BP_Point_Drone_Mission_C"))
      (if (Utilities|Array|IsValidIndex _outpoints)
        (Transformation|SetRelativeRotation (Variables|Default|GetMeshAttachRoot) (Math|Rotator|MakeRotator 0.0 0.0 (.poiHeading (Utilities|Struct|BreakMissionPoint (Variables|/Game/DMA/Blueprints/BP_Point_Drone_Mission.BP_Point_Drone_Mission_C|GetPointData (Utilities|Array|Get(acopy) _outpoints))))) false false)))))

(event Custom|SetTarget
  (switch Utilities|FlowControl|Switch|SwitchonEPointContainerType (Variables|/Script/Kulagin.MapperContainerBase|GetContainerType (Variables|Default|GetAttachedToContainer))
    (:PCT_Mission
      (bind _asbp_point_drone_mission (Utilities|Casting|CastToBP_Point_Drone_Mission (Variables|Default|GetTargetPoint))
        (:then
          (CallFunction|UpdateRotation (+ (Variables|Default|GetCurrentPoint) 1))
          (Utilities|FlowControl|Delay (* (Math|Float|Absolute(Float) (Math|Conversions|ToFloat(Integer) (.loiterTime (Utilities|Struct|BreakMissionPoint (Variables|/Game/DMA/Blueprints/BP_Point_Drone_Mission.BP_Point_Drone_Mission_C|GetPointData _asbp_point_drone_mission))))) 0.001)))
        (:CastFailed
          _))
      (bind _outpoints (Class|MapperContainerBase|GetPointsOfClass (Variables|Default|GetAttachedToContainer) "/Game/DMA/Blueprints/BP_Point_Interactive.BP_Point_Interactive_C"))
      (Transformation|SetActorLocation (Transformation|GetActorLocation (Utilities|Array|Get(acopy) _outpoints (Variables|Default|GetCurrentPoint))) false false)
      (if (not (> (+ (Variables|Default|GetCurrentPoint) 1) (Utilities|Array|LastIndex _outpoints)))
        (Variables|Default|SetTargetPoint (Utilities|Array|Get(acopy) _outpoints (+ (Variables|Default|GetCurrentPoint) 1)))
        (Variables|Default|SetCurrentPoint (+ (Variables|Default|GetCurrentPoint) 1))))))

(event Custom|UpdateRotation
  (params (CurrentPointIndex :type Integer))
  (bind _returnvalue (+ CurrentPointIndex 1))
  (bind _attachedtocontainer (Variables|Default|GetAttachedToContainer))
  (Utilities|IsValid _attachedtocontainer
    (:Is%20Valid
      (bind _outpoints (Class|MapperContainerBase|GetPointsOfClass _attachedtocontainer "/Game/DMA/Blueprints/BP_Point_Drone_Mission.BP_Point_Drone_Mission_C"))
      (if (and (Utilities|Array|IsValidIndex _outpoints CurrentPointIndex) (Utilities|Array|IsValidIndex _outpoints _returnvalue))
        (Components|MoveComponentTo (Variables|Default|GetMeshAttachRoot) "0, 0, 0" (Math|Rotator|MakeRotator 0.0 0.0 (.poiHeading (Utilities|Struct|BreakMissionPoint (Variables|/Game/DMA/Blueprints/BP_Point_Drone_Mission.BP_Point_Drone_Mission_C|GetPointData (Utilities|Array|Get(acopy) _outpoints _returnvalue))))) false false (/ (Math|Conversions|ToFloat(Integer) (.loiterTime (Utilities|Struct|BreakMissionPoint (Variables|/Game/DMA/Blueprints/BP_Point_Drone_Mission.BP_Point_Drone_Mission_C|GetPointData (Utilities|Array|Get(acopy) _outpoints CurrentPointIndex))))) 1e+03) true)))))

(event Custom|StartDropMoving)

(event Custom|StartRiseMoving)

(event EventBeginPlay
  (bind _returnvalue (Class|KulaginStatics|GetMapperGameInstance))
  (bind _dronename (Variables|/Script/Kulagin.MapperGameInstance|GetDroneName _returnvalue))
  (Utilities|IsValid _returnvalue
    (:Is%20Valid
      (bind _returnvalue_2 (Class|DataTableFunctionLibrary|DoesDataTableRowExist "/Game/DMA/Data/DT_DroneData.DT_DroneData" _dronename))
      (if _returnvalue_2
        (bind _returnvalue_3 (Utilities|GetDataTableRow "/Game/DMA/Data/DT_DroneData.DT_DroneData" _dronename)
          (:then
            (if (Class|KulaginStatics|IsValidDroneData _returnvalue_3)
              (switch Utilities|FlowControl|Switch|SwitchonEDroneActorType (.ActorType (Utilities|Struct|BreakDroneData _returnvalue_3))
                (:DAT_Skeletal
                  (Class|SkinnedMeshComponent|SetSkeletalMesh (Variables|Default|GetSkeletalMesh) (.SkeletalMesh (Utilities|Struct|BreakDroneData _returnvalue_3)) true)
                  (Development|SetHiddeninGame (Variables|Default|GetSkeletalMesh) false false))
                (:DAT_Static
                  (Components|StaticMesh|SetStaticMesh (Variables|Default|GetStaticMesh) (.StaticMesh (Utilities|Struct|BreakDroneData _returnvalue_3)))
                  (Development|SetHiddeninGame (Variables|Default|GetStaticMesh) false false))
                (:DAT_Class
                  (bind _returnvalue_4 (Game|SpawnActorfromClass (.Class (Utilities|Struct|BreakDroneData _returnvalue_3)) (Math|Transform|MakeTransform "0, 0, 0" "0, 0, 0" "1,1,1") "AlwaysSpawn" 0 0))
                  (bind _output_get (Variables|Default|SetChildDrone _returnvalue_4))
                  (Transformation|AttachComponentToComponent _output_get (Variables|Default|GetMeshAttachRoot) "None" "KeepRelative" "KeepRelative" "KeepRelative" true)))
              (else
                (Development|SetHiddeninGame (Variables|Default|GetSkeletalMesh) false false :!label _label)))))
        (else
          (goto _label))))
    (:Is%20Not%20Valid
      (goto _label))))

(event Collision|EventActorBeginOverlap
  (params (OtherActor :type Actor%20Object%20Reference)))

(event EventTick
  (params (DeltaSeconds :type Float%20%28single-precision%29))
  (bind _returnvalue (Transformation|GetActorLocation))
  (bind _targetpoint (Variables|Default|GetTargetPoint))
  (bind _returnvalue_2 (Transformation|GetActorLocation _targetpoint))
  (Variables|Default|GetTargetPoint
    (:then
      (if (not (CallFunction|IsPaused))
        (Variables|Default|SetHorDistance (Math|Vector|Distance2D(Vector) (Math|Vector2D|MakeVector2D (.x _returnvalue) (.y _returnvalue)) (Math|Vector2D|MakeVector2D (.x _returnvalue_2) (.y _returnvalue_2))))
        (Variables|Default|SetVertDistance (Math|Float|Absolute(Float) (- (.z _returnvalue) (.z _returnvalue_2))))
        (if (and (<= (Variables|Default|GetHorDistance) 0.1) (<= (Variables|Default|GetVertDistance) 0.1))
          _
          (else
            (Transformation|SetActorLocation (Math|Interpolation|VInterptoConstant (Transformation|GetActorLocation) (Transformation|GetActorLocation (Variables|Default|GetTargetPoint)) DeltaSeconds (Class|MapperPointBase|GetSpeedtoPoint (Variables|Default|GetTargetPoint) (Transformation|GetActorLocation))) false false)
            (Utilities|FlowControl|DoOnce false ; enters at Reset
              (:Completed
                _))))
        (CallFunction|SetTarget)))
    (:else)))

(event EventEndPlay
  (params (EndPlayReason :type EEndPlayReason%20Enum :default "Destroyed"))
  (Utilities|IsValid (Variables|Default|GetChildDrone)
    (:Is%20Valid
      (Actor|DestroyActor (Variables|Default|GetChildDrone)))))

(fn ConstructionScript)

(fn SetMovingActorVisible
  (params (bNewVisible :type Boolean))
  (Rendering|SetActorHiddenInGame (not bNewVisible))
  (Utilities|IsValid (Variables|Default|GetChildDrone)
    (:Is%20Valid
      (Rendering|SetActorHiddenInGame (Variables|Default|GetChildDrone) (not bNewVisible)))))

(fn RiseMovingActor
  (|CallParentFunction)
  (Utilities|IsValid (Variables|Default|GetChildDrone)
    (:Is%20Valid
      (bind _asbp_drone_01 (Utilities|Casting|CastToBP_Drone_01 (Variables|Default|GetChildDrone))
        (:then
          (bind _bsuccess (Default|RiseMovingActor _asbp_drone_01))
          (return _bsuccess))
        (:CastFailed
          _)))
    (:Is%20Not%20Valid
      _))
  (if (not (Variables|/Script/Engine.SceneComponent|GetbHiddenInGame (Variables|Default|GetSkeletalMesh)))
    (Physics|SetSimulatePhysics (Variables|Default|GetSkeletalMesh) false)
    (Transformation|SetRelativeLocationAndRotation (Variables|Default|GetSkeletalMesh) "0, 0, 0" "0, 0, 0" false false)
    (Transformation|AttachComponentToComponent (Variables|Default|GetSkeletalMesh) (Variables|Default|GetMeshAttachRoot) "None" "KeepRelative" "KeepRelative" "KeepRelative" true)
    (return true)
    (elif (not (Variables|/Script/Engine.SceneComponent|GetbHiddenInGame (Variables|Default|GetStaticMesh)))
      (Physics|SetSimulatePhysics (Variables|Default|GetStaticMesh) false)
      (Transformation|SetRelativeLocationAndRotation (Variables|Default|GetStaticMesh) "0, 0, 0" "0, 0, 0" false false)
      (Transformation|AttachComponentToComponent (Variables|Default|GetStaticMesh) (Variables|Default|GetMeshAttachRoot) "None" "KeepRelative" "KeepRelative" "KeepRelative" true)
      (return true)
      (else
        (return false)))))

(fn DropMovingActor
  (|CallParentFunction)
  (Utilities|IsValid (Variables|Default|GetChildDrone)
    (:Is%20Valid
      (bind _asbp_drone_01 (Utilities|Casting|CastToBP_Drone_01 (Variables|Default|GetChildDrone))
        (:then
          (bind _bsuccess (Default|DropMovingActor _asbp_drone_01))
          (return _bsuccess))
        (:CastFailed
          _)))
    (:Is%20Not%20Valid
      _))
  (if (not (Variables|/Script/Engine.SceneComponent|GetbHiddenInGame (Variables|Default|GetSkeletalMesh)))
    (Physics|SetSimulatePhysics (Variables|Default|GetSkeletalMesh) true)
    (return true)
    (elif (not (Variables|/Script/Engine.SceneComponent|GetbHiddenInGame (Variables|Default|GetStaticMesh)))
      (Physics|SetSimulatePhysics (Variables|Default|GetStaticMesh) true)
      (return true)
      (else
        (return false)))))

(fn IsPaused
  (bind _attachedtocontainer (Variables|Default|GetAttachedToContainer))
  (Utilities|IsValid _attachedtocontainer
    (:Is%20Valid
      (return (Variables|/Script/Kulagin.MapperContainerBase|GetbIsPaused _attachedtocontainer)))
    (:Is%20Not%20Valid
      (return (|CallParentFunction)))))