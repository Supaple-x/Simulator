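; BP_Moving_Actor_Human is a moving actor, apparently a human, that travels along the interactive mapper points of its attached container.
; StartMoving places it at the first point and targets the second; ResumeMoving faces along the segment and drives a MoveComponentTo timed by the point.
; Each completed move advances to the next point, pausing the container at the path's end.
; SetPaused stops or resumes movement, while the SetMovingActorRotation override flattens rotation to horizontal.
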(event Custom|ResumeMoving
  (if (not (Class|MapperDroneBase|IsPaused))
    (Utilities|IsValid (Variables|Default|GetTargetPoint)
      (:Is%20Valid
        (Utilities|IsValid (Class|MapperPointInteractive|GetPrevious (Variables|Default|GetTargetPoint))
          (:Is%20Valid
            (Transformation|SetActorRotation (Math|Rotator|FindLookatRotation (Transformation|GetActorLocation (Class|MapperPointInteractive|GetPrevious (Variables|Default|GetTargetPoint))) (Transformation|GetActorLocation (Variables|Default|GetTargetPoint))))
            (Variables|Default|SetTargetLocation (Transformation|GetActorLocation (Variables|Default|GetTargetPoint)))
            (Variables|Default|SetTargetRotation (Math|Rotator|FindLookatRotation (Transformation|GetActorLocation (Class|MapperPointInteractive|GetPrevious (Variables|Default|GetTargetPoint))) (Transformation|GetActorLocation (Variables|Default|GetTargetPoint))))
            (Variables|Default|SetTargetTime (Class|MapperPointBase|GetTimetoPoint (Variables|Default|GetTargetPoint) (Transformation|GetActorLocation)))
            (Components|MoveComponentTo (Variables|Default|GetDefaultSceneRoot) (Variables|Default|GetTargetLocation) (Variables|Default|GetTargetRotation) false false (Variables|Default|GetTargetTime) true)
            (if (not (Class|MapperDroneBase|IsPaused))
              (Utilities|IsValid (Variables|Default|GetTargetPoint)
                (:Is%20Valid
                  (Utilities|IsValid (Class|MapperPointInteractive|GetNextOfClass (Variables|Default|GetTargetPoint) "/Script/Kulagin.MapperPointInteractive")
                    (:Is%20Valid
                      (Variables|Default|SetTargetPoint (Class|MapperPointInteractive|GetNextOfClass (Variables|Default|GetTargetPoint) "/Script/Kulagin.MapperPointInteractive"))
                      (CallFunction|ResumeMoving))
                    (:Is%20Not%20Valid
                      (Class|MapperContainerBase|SetPaused (Variables|Default|GetAttachedToContainer) true))))))))))))

(event Custom|StopMoving
  (Components|MoveComponentTo (Variables|Default|GetDefaultSceneRoot) (Variables|Default|GetTargetLocation) (Variables|Default|GetTargetRotation) false false (Variables|Default|GetTargetTime) true) ; enters at Stop
)

(event EventBeginPlay
  (Development|PrintString "Hello"))

(event EventStartMoving
  (if (not (Class|MapperDroneBase|IsPaused))
    (Utilities|IsValid (Variables|Default|GetAttachedToContainer)
      (:Is%20Valid
        (bind _outpoints (Class|MapperContainerBase|GetPointsOfClass (Variables|Default|GetAttachedToContainer) "/Script/Kulagin.MapperPointInteractive"))
        (if (Utilities|Array|IsValidIndex _outpoints 1)
          (Variables|Default|SetTargetPoint (Utilities|Array|Get(acopy) _outpoints 1))
          (Transformation|SetActorLocation (Transformation|GetActorLocation (Utilities|Array|Get(acopy) _outpoints)) false false)
          (CallFunction|ResumeMoving))))))

(fn ConstructionScript
  (|CallParentFunction))

(fn SetMovingActorRotation
  (params (Rot :type Rotator%20%28by%20ref%29 :default "0, 0, 0") (bTeleport :type Boolean))
  (bind _returnvalue (Math|Vector|GetForwardVector Rot))
  (bind _returnvalue_2 (|CallParentFunction (Math|Rotator|MakeRotfromX (Math|Vector|MakeVector (.x _returnvalue) (.y _returnvalue) 0.0)) bTeleport))
  (return _returnvalue_2))

(fn SetPaused
  (params (bIsPausedIn :type Boolean))
  (if bIsPausedIn
    (CallFunction|StopMoving)
    (return true)
    (else
      (CallFunction|ResumeMoving)
      (return false))))