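; Plane mission path container for the drone mapper, holding the route's points and handling saving and copying of that path.
; It gathers point data from its BP_Point_Plane_Mission points, and SavePath writes that data to the container's file path, printing whether it succeeded.
; CopyPath applies an offset to the points and loads the result as a plane mission through the Drone Mapper game mode.
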(fn ConstructionScript)

(fn GetMovingActorRotationat
  (params (InTime :type Float%20%28single-precision%29))
  (return "0, 0, 0"))

(fn GetActualPointData
  (bind _outpoints (Class|MapperContainerBase|GetPointsOfClass "/Game/DMA/Blueprints/BP_Point_Plane_Mission.BP_Point_Plane_Mission_C"))
  (for _array_element _outpoints
    (Utilities|Array|Add (LocalVariables|GetDataLocal) (Variables|/Game/DMA/Blueprints/BP_Point_Plane_Mission.BP_Point_Plane_Mission_C|GetPointData _array_element)))
  (return (LocalVariables|GetDataLocal)))

(fn SavePath
  (bind _data (CallFunction|GetActualPointData))
  (bind _returnvalue (Class|KulaginStatics|SavePlanePointstoFile (Variables|Default|GetFilePath) _data))
  (Development|PrintString (Utilities|String|Append "Kulagin: SavePath for Plane Mission is " (Utilities|String|SelectString "VALID" "FAILED" _returnvalue)))
  (return true))

(fn CopyPath
  (params (Offset :type Vector :default "0, 0, 0"))
  (bind _data (CallFunction|GetActualPointData))
  (Class|KulaginStatics|AddPlaneMissionPointsOffset _data Offset)
  (Default|LoadPlaneMission (CallFunction|GetDroneMapperGamemode) (Utilities|Struct|MakePlaneMissionPointList (Variables|Default|GetFilePath) _data "()" "()"))
  (return true))