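; BP_Plane_Mission_Point is a numbered waypoint in a plane mission path, owned by a parent container.
; Moving it rewrites its geographic point struct and recalculates container timings, while struct updates reposition the actor.
; It stretches a segment toward TargetActor, with a danger-zone cylinder masked through a per-point render target.
; Line traces drive toggleable axis projection beams and decals, plus a red or yellow marker for first or last points.
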(event Custom|ToggleProjection_1
  (params (bEnabled :type Boolean))
  (CallFunction|ToggleProjectionOld bEnabled))

(event EventBeginPlay
  (bind _returnvalue (Rendering|CreateRenderTarget2D 512 512 "RTF_RGBA16f"))
  (bind _output_get (Variables|Default|SetCrossRenderTarget_0 _returnvalue))
  (Rendering|ClearRenderTarget2D _output_get)
  (bind _returnvalue_2 (Rendering|Material|CreateDynamicMaterialInstance "/Game/DMA/MaterialLibrary/M_Cross_01.M_Cross_01" "None" :!class /Script/Engine.KismetMaterialLibrary))
  (bind _output_get_2 (Variables|Default|SetCrossMaterial_0 _returnvalue_2))
  (Rendering|Material|SetTextureParameterValue _output_get_2 "RenderTarget" (Variables|Default|GetCrossRenderTarget_0))
  (Rendering|Material|SetMaterial (Variables|Default|GetCylinder_0) 0 (Variables|Default|GetCrossMaterial_0)))

(event Collision|EventActorBeginOverlap
  (params (OtherActor :type Actor%20Object%20Reference)))

(event EventTick
  (params (DeltaSeconds :type Float%20%28single-precision%29))
  (bind _returnvalue (Transformation|GetActorLocation))
  (if (Variables|Default|GetbIsFirstLast_0)
    (CallFunction|UpdateFirstLast0))
  (if (Variables|Default|GetbIsProjectionEnabled_0)
    (CallFunction|UpdateProjection0))
  (if (Math|Vector|NotEqual(Vector) (Variables|Default|GetPrevLocation_0) _returnvalue 0.1)
    (Variables|Default|SetPrevLocation_0 _returnvalue)
    (CallFunction|ChangePointStruct))
  (bind _targetactor (Variables|Default|GetTargetActor)
    (:then
      (if (Math|Vector|NotEqual(Vector) (Variables|Default|GetTargetPrevLocation_0) (Transformation|GetActorLocation _targetactor) 0.1)
        (Variables|Default|SetTargetPrevLocation_0 (Variables|Default|GetTargetPrevLocation_0))
        (CallFunction|CreatePlane)))
    (:else
      (Rendering|SetVisibility (Variables|Default|GetPlane_0) false false))))

(fn ConstructionScript)

(fn CreatePlane
  (bind _returnvalue (Transformation|GetActorLocation))
  (bind _planeroot_0 (Variables|Default|GetPlaneRoot_0))
  (bind _targetactor (Variables|Default|GetTargetActor))
  (bind _returnvalue_2 (Transformation|GetActorLocation _targetactor))
  (bind _returnvalue_3 (Math|Vector|Distance(Vector) _returnvalue _returnvalue_2))
  (bind _returnvalue_4 (Math|Rotator|FindLookatRotation _returnvalue _returnvalue_2))
  (bind (_roll _pitch _yaw) (Math|Rotator|BreakRotator _returnvalue_4))
  (bind _returnvalue_5 (/ _returnvalue_3 1e+02))
  (Rendering|SetVisibility (Variables|Default|GetPlane_0) true false)
  (Transformation|SetWorldScale3D _planeroot_0 (Math|Vector|MakeVector 1.0 1.0 _returnvalue_5))
  (Transformation|SetWorldRotation _planeroot_0 (Math|Rotator|MakeRotator 0.0 _pitch _yaw) false false)
  (Transformation|SetRelativeLocation (Variables|Default|GetCylinder_0) (Math|Vector|MakeVector (* _returnvalue_5 5e+01) 0.0 0.0) false false))

(fn IntBacktoMap
  (params (SourceString :type String) (InInt :type Integer))
  (bind _returnvalue (Utilities|String|Left SourceString 1))
  (bind _returnvalue_2 (Utilities|String|ToString(Integer) InInt))
  (bind _returnvalue_3 (Utilities|String|Left _returnvalue_2 1))
  (bind _returnvalue_4 (Utilities|String|RightChop _returnvalue_2 1))
  (bind _returnvalue_5 (Utilities|String|Append _returnvalue _returnvalue_3 "." _returnvalue_4))
  (bind _returnvalue_6 (Utilities|String|Reverse _returnvalue_5))
  (bind _returnvalue_7 (Utilities|String|GetCharacterArrayfromString _returnvalue_6))
  (bind _array_element (Utilities|Array|ForEachLoopwithBreak _returnvalue_7 :!label _label)
    (:LoopBody
      (if (Utilities|Enum|Equal(Enum) _array_element "0")
        (Math|Integer|IncrementInt (LocalVariables|GetZeroCount))
        (else
          (goto _label Break))))
    (:Completed
      (return (Utilities|String|LeftChop (Utilities|String|Reverse (Utilities|String|JoinStringArray _returnvalue_7 "")) (LocalVariables|GetZeroCount))))))

(fn ChangePointStruct
  ;[1 1 1] If location changed laclulate new Lat and Lon
  (if (not (Variables|Default|GetbStaticPointStruct_0))
    (Class|KulaginStatics|UEtoPlaneMissionPoint (Variables|Default|GetPointStruct) (Transformation|GetActorLocation) (Variables|Default|GetStartAlt_0))
    (Default|CalculatePointsTimes (Variables|Default|GetParentContainer_0))))

(fn SetPointID
  (params (Value :type Integer%20%28by%20ref%29))
  (bind _output_get (Variables|Default|SetPointID Value))
  (Rendering|Components|TextRender|SetText (Variables|Default|GetTextRender_0) (Utilities|Text|ToText(Integer) _output_get)))

(fn OnPointStructUpdated
  (Development|PrintString "Kulagin: On Point Struct Updated")
  (bind _returnvalue (Class|KulaginStatics|PlaneMissionPointtoUE (Variables|Default|GetPointStruct) (Variables|Default|GetStartAlt_0)))
  (Transformation|SetActorLocation _returnvalue false false)
  (Variables|Default|SetPrevLocation_0 (Transformation|GetActorLocation)))

(fn SetMaterialBp
  (params (NewMaterial :type Material%20Interface%20Object%20Reference)))

(fn UpdateProjection0
  (for (_array_element _array_index) (Utilities|Array|MakeArray (Variables|Default|GetProjectionZMinusRoot_0) (Variables|Default|GetProjectionXMinusRoot_0) (Variables|Default|GetProjectionXPlusRoot_0) (Variables|Default|GetProjectionYMinusRoot_0) (Variables|Default|GetProjectionYPlusRoot_0))
    (CallFunction|UpdateProjectionComponents0 _array_element (Utilities|Array|Get(acopy) (Utilities|Array|MakeArray (Variables|Default|GetProjectionZMinusDecal_0) (Variables|Default|GetProjectionXMinusDecal_0) (Variables|Default|GetProjectionXPlusDecal_0) (Variables|Default|GetProjectionYMinusDecal_0) (Variables|Default|GetProjectionYPlusDecal_0)) _array_index))))

(fn ToggleProjectionOld
  (params (bEnabled :type Boolean))
  (Class|MapperContainerBase|SetTimelineIsHighlighted (Variables|Default|GetParentContainer_0) bEnabled)
  (if (Math|Boolean|NotEqual(Boolean) bEnabled (Variables|Default|GetbIsProjectionEnabled_0))
    (Variables|Default|SetbIsProjectionEnabled_0 bEnabled)
    (for (_array_element _array_index) (Utilities|Array|MakeArray (Variables|Default|GetProjectionZMinusRoot_0) (Variables|Default|GetProjectionXMinusRoot_0) (Variables|Default|GetProjectionXPlusRoot_0) (Variables|Default|GetProjectionYMinusRoot_0) (Variables|Default|GetProjectionYPlusRoot_0))
      (Development|SetHiddeninGame _array_element (not (and (Variables|/Script/Kulagin.MapperContainerBase|GetbIsPathVisible (Variables|Default|GetParentContainer_0)) (Variables|Default|GetbIsProjectionEnabled_0))) true)
      (Development|SetHiddeninGame (Utilities|Array|Get(acopy) (Utilities|Array|MakeArray (Variables|Default|GetProjectionZMinusDecal_0) (Variables|Default|GetProjectionXMinusDecal_0) (Variables|Default|GetProjectionXPlusDecal_0) (Variables|Default|GetProjectionYMinusDecal_0) (Variables|Default|GetProjectionYPlusDecal_0)) _array_index) (not (and (Variables|/Script/Kulagin.MapperContainerBase|GetbIsPathVisible (Variables|Default|GetParentContainer_0)) (Variables|Default|GetbIsProjectionEnabled_0))) true))))

(fn UpdateFirstLast0
  (CallFunction|UpdateProjectionComponents0 (Variables|Default|GetProjectionFirstLastRoot_0) (Variables|Default|GetProjectionFirstLastDecal_0)))

(fn UpdateProjectionComponents0
  (params (Root :type Scene%20Component%20Object%20Reference) (Decal :type Scene%20Component%20Object%20Reference))
  (bind _returnvalue (Transformation|GetActorLocation))
  (bind (_outhit _returnvalue_2) (Collision|LineTraceForObjects _returnvalue (+ _returnvalue (* (Math|Vector|GetForwardVector Root) 1e+05)) (Utilities|Array|MakeArray "ObjectTypeQuery1") true 0 "None"))
  (Transformation|SetWorldScale3D Root (Math|Vector|MakeVector (Math|Float|SelectFloat (/ (Math|Vector|Distance(Vector) (.ImpactPoint (Collision|BreakHitResult _outhit)) (Transformation|GetActorLocation)) 1e+02) 1e+03 _returnvalue_2) 1.0 1.0))
  (Development|SetHiddeninGame Decal (not _returnvalue_2) false)
  (if _returnvalue_2
    (Transformation|SetWorldLocation Decal (.ImpactPoint (Collision|BreakHitResult _outhit)) false false)))

(fn SetFirst0
  (Variables|Default|SetbIsFirstLast_0 true)
  (Rendering|Material|SetMaterial (Variables|Default|GetProjectionFirstLast_0) 0 "/Game/DMA/MaterialLibrary/MI_Projection_01_Red.MI_Projection_01_Red")
  (Development|SetHiddeninGame (Variables|Default|GetProjectionFirstLast_0) false false)
  (Rendering|Components|Decal|SetDecalMaterial (Variables|Default|GetProjectionFirstLastDecal_0) "/Game/DMA/MaterialLibrary/MI_Projection_Decal_01_Red.MI_Projection_Decal_01_Red")
  (Development|SetHiddeninGame (Variables|Default|GetProjectionFirstLastDecal_0) false false))

(fn SetLast0
  (Variables|Default|SetbIsFirstLast_0 true)
  (Rendering|Material|SetMaterial (Variables|Default|GetProjectionFirstLast_0) 0 "/Game/DMA/MaterialLibrary/MI_Projection_01_Yellow.MI_Projection_01_Yellow")
  (Development|SetHiddeninGame (Variables|Default|GetProjectionFirstLast_0) false false)
  (Rendering|Components|Decal|SetDecalMaterial (Variables|Default|GetProjectionFirstLastDecal_0) "/Game/DMA/MaterialLibrary/MI_Projection_Decal_01_Yellow.MI_Projection_Decal_01_Yellow")
  (Development|SetHiddeninGame (Variables|Default|GetProjectionFirstLastDecal_0) false false))

(fn SetNormal0
  (Variables|Default|SetbIsFirstLast_0 false)
  (Development|SetHiddeninGame (Variables|Default|GetProjectionFirstLast_0) true false)
  (Development|SetHiddeninGame (Variables|Default|GetProjectionFirstLastDecal_0) true false))

(fn GetPrevious0
  (bind _pointid (Variables|Default|GetPointID))
  (bind _returnvalue (- _pointid 1))
  (bind _outpoints (Class|MapperContainerBase|GetPointsOfClass (Variables|Default|GetParentContainer_0) "BP_Plane_Mission_Point_C"))
  (if (Utilities|Array|IsValidIndex _outpoints _returnvalue)
    (return (Utilities|Array|Get(acopy) _outpoints _returnvalue))
    (else
      (return 0))))

(fn UpdateSpeed0
  (params (NewTargetTime :type Float%20%28single-precision%29)))

(fn SetMaterial0
  (params (NewMaterial :type Material%20Interface%20Object%20Reference) (NewMaterial_ERROR_DUPLICATE_0 :type Material%20Interface%20Object%20Reference) (NewMaterial_ERROR_DUPLICATE_1 :type Material%20Interface%20Object%20Reference) (NewMaterial :type Material%20Interface%20Object%20Reference))
  (Rendering|Material|SetMaterial (Variables|Default|GetSphere_0) 0 NewMaterial)
  (Rendering|Material|SetMaterial (Variables|Default|GetPlane_0) 0 NewMaterial)
  (return true false))

(fn UpdateCrossRadius0
  (bind _parentcontainer_0 (Variables|Default|GetParentContainer_0))
  (bind _returnvalue (Class|MapperContainerBase|GetDangerZoneRadiusUU _parentcontainer_0))
  (bind _returnvalue_2 (/ _returnvalue 1e+02))
  (Transformation|SetRelativeScale3D (Variables|Default|GetCylinder_0) (Math|Vector|MakeVector _returnvalue_2 _returnvalue_2 1.0)))

(fn UpdateCrossCylinder0
  (Utilities|IsValid (Variables|Default|GetParentContainer_0)
    (:Is%20Valid
      (bind _output_get (LocalVariables|SetPrevLocal (CallFunction|GetPrevious0)))
      (Utilities|IsValid _output_get
        (:Is%20Valid
          (LocalVariables|SetStartTimeLocal 0.0)
          (LocalVariables|SetEndTimeLocal (Variables|Default|GetEnterTime_0))
          (Class|MapperPointBase|SetDangerZoneMask (Variables|Default|GetCrossRenderTarget_0) (LocalVariables|GetStartTimeLocal) (LocalVariables|GetEndTimeLocal) (Variables|/Script/Kulagin.MapperContainerBase|GetDangerZones (Variables|Default|GetParentContainer_0))))))))

(fn UpdateCrossVisibility0
  (Development|SetHiddeninGame (Variables|Default|GetCylinder_0) (not (Variables|/Script/Kulagin.MapperContainerBase|GetbIsDangerZoneVisible (Variables|Default|GetParentContainer_0))) false))

(fn UpdatePathVisibility0
  (Development|SetHiddeninGame (Variables|Default|GetSphere_0) (not (Variables|/Script/Kulagin.MapperContainerBase|GetbIsPathVisible (Variables|Default|GetParentContainer_0))) true))