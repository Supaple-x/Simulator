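; Point container for a logged drone path that replays the flight by moving DroneActor along BP_Point_Log actors.
; Tick advances CurrentTime while unpaused, and SetMovingActor applies the transform linearly interpolated between the points bracketing that time, caching the last index to shorten forward searches.
; Parent overrides handle path visibility, color and highlighting through a shared material instance, timeline widget highlighting, and removal from the game mode.
; Drone spawning and material creation nodes are disconnected here.
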(event EventBeginPlay)

(event Collision|EventActorBeginOverlap
  (params (OtherActor :type Actor%20Object%20Reference)))

(event EventTick
  (params (DeltaSeconds :type Float%20%28single-precision%29))
  (if (not (Variables|Default|GetbIsPaused))
    (bind _output_get (Variables|Default|SetCurrentTime (+ DeltaSeconds (Variables|Default|GetCurrentTime))))
    (CallFunction|SetMovingActor _output_get)))

(fn ConstructionScript)

(fn SetWorldTrackIsHighlighted
  (params (bNewIsHighlighted :type Boolean))
  (|CallParentFunction bNewIsHighlighted)
  (Rendering|Material|SetScalarParameterValue (Variables|Default|GetPathMaterialInstance) "Lines" (Math|Float|SelectFloat 1.0 0.0 bNewIsHighlighted) :!class /Script/Engine.MaterialInstanceDynamic)
  (return bNewIsHighlighted))

(fn SetTimelineIsHighlighted
  (params (bNewIsHighlighted :type Boolean))
  (|CallParentFunction bNewIsHighlighted)
  (bind _asw_mission_timeline (Utilities|Casting|CastToW_Mission_Timeline (Variables|Default|GetTimelineWidget))
    (:then
      (bind _output_get (Variables|/Game/DMA/UI/Widgets/W_Mission_Timeline.W_Mission_Timeline_C|SetbIsHighlighted _asw_mission_timeline bNewIsHighlighted))
      (return _output_get))
    (:CastFailed
      (return false))))

(fn SetPointsMaterial
  (|CallParentFunction)
  (for _array_element (Variables|Default|GetPointActors)
    (Class|MapperPointBase|SetMaterial _array_element (Variables|Default|GetPathMaterialInstance)))
  (return true))

(fn SetPointsColor
  (params (NewColor :type Linear%20Color%20Structure))
  (|CallParentFunction NewColor)
  (Rendering|Material|SetVectorParameterValue (Variables|Default|GetPathMaterialInstance) "Color" NewColor :!class /Script/Engine.MaterialInstanceDynamic)
  (return true))

(fn RemovePath
  (bind _returnvalue (Class|KulaginStatics|GetMapperGameMode))
  (bind _pointcontainers (Variables|/Script/Kulagin.MapperGameMode|GetPointContainers _returnvalue))
  (|CallParentFunction)
  (Utilities|IsValid (Variables|Default|GetTimelineWidget)
    (:Is%20Valid
      (Widget|RemovefromParent (Variables|Default|GetTimelineWidget)))
    (:Is%20Not%20Valid
      _))
  (Variables|Default|SetTimelineWidget 0)
  (Utilities|Array|RemoveIndex _pointcontainers (Utilities|Array|FindItem _pointcontainers self))
  (for _array_element (Variables|Default|GetPointActors)
    (Actor|DestroyActor _array_element))
  (Actor|DestroyActor (Variables|Default|GetDroneActor))
  (Actor|DestroyActor)
  (return true))

(fn GetTotalTime
  (bind _pointactors (Variables|Default|GetPointActors))
  (bind _asbp_point_log (Utilities|Casting|CastToBP_Point_Log (Utilities|Array|Get(acopy) _pointactors (Utilities|Array|LastIndex _pointactors))))
  (return (.Time (Utilities|Struct|BreakLogPoint (Variables|/Game/DMA/Blueprints/BP_Point_Log.BP_Point_Log_C|GetLogPointStruct _asbp_point_log)))))

(fn SetPathVisibility
  (params (bNewIsVisible :type Boolean))
  (|CallParentFunction bNewIsVisible)
  (Variables|Default|SetbIsPathVisible bNewIsVisible)
  (for _array_element (Variables|Default|GetPointActors)
    (Rendering|SetActorHiddenInGame _array_element (not (Variables|Default|GetbIsPathVisible))))
  (return (Variables|Default|GetbIsPathVisible)))

(fn SetPaused
  (params (bNewIsPaused :type Boolean))
  (|CallParentFunction bNewIsPaused)
  (bind _output_get (Variables|Default|SetbIsPaused bNewIsPaused))
  (Actor|Tick|SetActorTickEnabled (not _output_get))
  (return _output_get))

(fn SetMovingActor
  (params (NewTime :type Float%20%28single-precision%29))
  (bind _output_get (Variables|Default|SetCurrentTime NewTime))
  (|CallParentFunction NewTime)
  (bind _transform (CallFunction|GetTransformatTime _output_get))
  (bind _returnvalue (Transformation|SetActorTransform (Variables|Default|GetDroneActor) _transform))
  (return _returnvalue))

(fn GetTransformatTime
  (params (TimeIn :type Float%20%28single-precision%29))
  (bind _pointactors (Variables|Default|GetPointActors))
  (bind _pointactors_2 (Variables|Default|GetPointActors))
  (LocalVariables|SetStartIndex (Math|Integer|Clamp(Integer) (Math|Integer|SelectInt (Variables|Default|GetLastCheckedIndex) 1 (> TimeIn (Variables|Default|GetLastCheckedTime))) 1 (- (Utilities|Array|LastIndex (Variables|Default|GetPointActors)) 1)))
  (Variables|Default|SetLastCheckedTime TimeIn)
  (if (<= TimeIn 0.0)
    (LocalVariables|SetSecondLocal (.AsBP%20Point%20Log (Utilities|Casting|CastToBP_Point_Log (Utilities|Array|Get(acopy) (Variables|Default|GetPointActors)))))
    (elif (>= TimeIn (CallFunction|GetTotalTime))
      (LocalVariables|SetSecondLocal (.AsBP%20Point%20Log (Utilities|Casting|CastToBP_Point_Log (Utilities|Array|Get(acopy) _pointactors_2 (Utilities|Array|LastIndex _pointactors_2)))))
      (else
        (for _index (range (LocalVariables|GetStartIndex) (Utilities|Array|LastIndex (Variables|Default|GetPointActors)))
          (Variables|Default|SetLastCheckedIndex _index)
          (LocalVariables|SetFirstLocal (.AsBP%20Point%20Log (Utilities|Casting|CastToBP_Point_Log (Utilities|Array|Get(acopy) _pointactors (- _index 1)))))
          (LocalVariables|SetSecondLocal (.AsBP%20Point%20Log (Utilities|Casting|CastToBP_Point_Log (Utilities|Array|Get(acopy) _pointactors _index))))
          (if (and (<= (Utilities|Struct|BreakLogPoint (Variables|/Game/DMA/Blueprints/BP_Point_Log.BP_Point_Log_C|GetLogPointStruct (LocalVariables|GetFirstLocal))) TimeIn) (>= (Utilities|Struct|BreakLogPoint (Variables|/Game/DMA/Blueprints/BP_Point_Log.BP_Point_Log_C|GetLogPointStruct (LocalVariables|GetSecondLocal))) TimeIn))
            (bind _output_get (LocalVariables|SetLocalAlpha (Math|Float|Clamp(Float) (/ (- TimeIn (Utilities|Struct|BreakLogPoint (Variables|/Game/DMA/Blueprints/BP_Point_Log.BP_Point_Log_C|GetLogPointStruct (LocalVariables|GetFirstLocal)))) (- (Utilities|Struct|BreakLogPoint (Variables|/Game/DMA/Blueprints/BP_Point_Log.BP_Point_Log_C|GetLogPointStruct (LocalVariables|GetSecondLocal))) (Utilities|Struct|BreakLogPoint (Variables|/Game/DMA/Blueprints/BP_Point_Log.BP_Point_Log_C|GetLogPointStruct (LocalVariables|GetFirstLocal))))))))
            (return (Math|Transform|MakeTransform (Math|Interpolation|Ease "Linear" (LocalVariables|GetLocalAlpha) (Transformation|GetActorLocation (LocalVariables|GetFirstLocal)) (Transformation|GetActorLocation (LocalVariables|GetSecondLocal))) (Math|Interpolation|Ease "Linear" (LocalVariables|GetLocalAlpha) (Math|Rotator|MakeRotator (.Roll (Utilities|Struct|BreakLogPoint (Variables|/Game/DMA/Blueprints/BP_Point_Log.BP_Point_Log_C|GetLogPointStruct (LocalVariables|GetFirstLocal)))) (.Pitch (Utilities|Struct|BreakLogPoint (Variables|/Game/DMA/Blueprints/BP_Point_Log.BP_Point_Log_C|GetLogPointStruct (LocalVariables|GetFirstLocal)))) (.Yaw (Utilities|Struct|BreakLogPoint (Variables|/Game/DMA/Blueprints/BP_Point_Log.BP_Point_Log_C|GetLogPointStruct (LocalVariables|GetFirstLocal))))) (Math|Rotator|MakeRotator (.Roll (Utilities|Struct|BreakLogPoint (Variables|/Game/DMA/Blueprints/BP_Point_Log.BP_Point_Log_C|GetLogPointStruct (LocalVariables|GetSecondLocal)))) (.Pitch (Utilities|Struct|BreakLogPoint (Variables|/Game/DMA/Blueprints/BP_Point_Log.BP_Point_Log_C|GetLogPointStruct (LocalVariables|GetSecondLocal)))) (.Yaw (Utilities|Struct|BreakLogPoint (Variables|/Game/DMA/Blueprints/BP_Point_Log.BP_Point_Log_C|GetLogPointStruct (LocalVariables|GetSecondLocal))))) true) (Transformation|GetActorScale3D (Variables|Default|GetDroneActor)))))))))
  (return (Math|Transform|MakeTransform (Transformation|GetActorLocation (LocalVariables|GetSecondLocal)) (Math|Rotator|MakeRotator (.Roll (Utilities|Struct|BreakLogPoint (Variables|/Game/DMA/Blueprints/BP_Point_Log.BP_Point_Log_C|GetLogPointStruct (LocalVariables|GetSecondLocal)))) (.Pitch (Utilities|Struct|BreakLogPoint (Variables|/Game/DMA/Blueprints/BP_Point_Log.BP_Point_Log_C|GetLogPointStruct (LocalVariables|GetSecondLocal)))) (.Yaw (Utilities|Struct|BreakLogPoint (Variables|/Game/DMA/Blueprints/BP_Point_Log.BP_Point_Log_C|GetLogPointStruct (LocalVariables|GetSecondLocal))))) (Transformation|GetActorScale3D (Variables|Default|GetDroneActor)))))

(fn StartMoving
  (|CallParentFunction)
  (bind _returnvalue (CallFunction|SetMovingActor 0.0))
  (return _returnvalue))

(fn GetLocationatTime
  (params (TimeIn :type Float%20%28single-precision%29))
  (bind _transform (CallFunction|GetTransformatTime TimeIn))
  (return (.location _transform)))