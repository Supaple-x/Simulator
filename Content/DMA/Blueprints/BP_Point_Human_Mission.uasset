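; Mission waypoint actor for a human mission, holding a point data struct and mirroring it in the world.
; It moves itself to the location converted from that data and start altitude, and can copy data from a mission list entry or another human mission point.
; Unless the point is static, the reverse update has its converter fed zero location and altitude rather than the actor's, then has the parent interactive container recalculate point times.
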(fn ConstructionScript)

(fn UpdateActorfromData
  (Development|PrintString "Kulagin: UpdateActorFromData for Drone Point")
  (bind _returnvalue (Class|KulaginStatics|HumanMissionPointtoUE (Variables|Default|GetPointData) (Variables|Default|GetStartAlt)))
  (Transformation|SetActorLocation _returnvalue false false)
  (Variables|Default|SetPrevLocation (Transformation|GetActorLocation))
  (return true))

(fn UpdateDatafromActor
  (if (not (Variables|Default|GetbStaticPointStruct))
    (Class|KulaginStatics|UEtoHumanMissionPoint (Variables|Default|GetPointData) "0, 0, 0" 0.0)
    (bind _asbp_container_interactive (Utilities|Casting|CastToBP_Container_Interactive (Variables|Default|GetParentContainer)))
    (Default|CalculatePointsTimes _asbp_container_interactive)
    (return true)))

(fn SetDatafromList
  (params (List :type Mission%20Point%20List%20Structure%20%28by%20ref%29) (Index :type Integer))
  (if (and (Utilities|Enum|Equal(Enum) (.type List) "PCT_HumanMission") (Utilities|Array|IsValidIndex (.humanpoints List) Index))
    (Variables|Default|SetPointData (Utilities|Array|Get(acopy) (.humanpoints List) Index))
    (return true)
    (else
      (return false))))

(fn SetDatafromPoint
  (params (Point :type Mapper%20Point%20Base%20Object%20Reference))
  (bind _asbp_point_human_mission (Utilities|Casting|CastToBP_Point_Human_Mission Point)
    (:then
      (Variables|Default|SetPointData (Variables|BP_Point_Human_Mission_C|GetPointData _asbp_point_human_mission))
      (return true))
    (:CastFailed
      (return false))))