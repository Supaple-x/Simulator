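; BP_Point_Plane_Mission is an interactive waypoint actor for a plane (drone) mission route, linking stored point data to a position in the world.
; It converts between PointData and actor location using the start altitude, and moving it makes the parent container recalculate point times unless the point's data is static.
; Data can be copied from a mission list or another point, and speed to the point comes from distance and time difference to the previous waypoint.
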(fn ConstructionScript)

(fn UpdateActorfromData
  (Development|PrintString "Kulagin: UpdateActorFromData for Drone Point")
  (bind _returnvalue (Class|KulaginStatics|PlaneMissionPointtoUE (Variables|Default|GetPointData) (Variables|Default|GetStartAlt)))
  (Transformation|SetActorLocation _returnvalue false false)
  (Variables|Default|SetPrevLocation (Transformation|GetActorLocation))
  (return true))

(fn UpdateDatafromActor
  (if (not (Variables|Default|GetbStaticPointStruct))
    (Class|KulaginStatics|UEtoPlaneMissionPoint (Variables|Default|GetPointData) (Transformation|GetActorLocation) (Variables|Default|GetStartAlt))
    (bind _asbp_container_interactive (Utilities|Casting|CastToBP_Container_Interactive (Variables|Default|GetParentContainer)))
    (Default|CalculatePointsTimes _asbp_container_interactive)
    (return true)))

(fn SetDatafromList
  (params (List :type Mission%20Point%20List%20Structure%20%28by%20ref%29) (Index :type Integer))
  (if (and (Utilities|Enum|Equal(Enum) (.type List) "PCT_PlaneMission") (Utilities|Array|IsValidIndex (.planepoints List) Index))
    (Variables|Default|SetPointData (Utilities|Array|Get(acopy) (.planepoints List) Index))
    (return true)
    (else
      (return false))))

(fn SetDatafromPoint
  (params (Point :type Mapper%20Point%20Base%20Object%20Reference))
  (bind _asbp_point_plane_mission (Utilities|Casting|CastToBP_Point_Plane_Mission Point)
    (:then
      (Variables|Default|SetPointData (Variables|BP_Point_Plane_Mission_C|GetPointData _asbp_point_plane_mission))
      (return true))
    (:CastFailed
      (return false))))

(fn GetSpeedtoPoint
  (params (CurrentLocation :type Vector%20%28by%20ref%29 :default "0, 0, 0"))
  (bind _previous (Class|MapperPointInteractive|GetPreviousOfClass "BP_Point_Plane_Mission_C"))
  (Utilities|IsValid _previous
    (:Is%20Valid
      (return (/ (Transformation|GetDistanceTo _previous) (Math|Float|Absolute(Float) (- (.time (Variables|Default|GetPointData)) (.time (Variables|BP_Point_Plane_Mission_C|GetPointData _previous)))))))
    (:Is%20Not%20Valid
      (return 1.0))))