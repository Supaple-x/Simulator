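; Interactive mission path container that owns an ordered set of waypoints and spawns the moving actor (with a child drone) that travels along them.
; Point enter times derive from distance, target speed and waits, while editing a point's time clamps it between neighbors, re-solves segment speeds and refreshes the timeline widget.
; Time queries linearly interpolate position for scrubbing.
; Parent overrides forward pause, visibility, danger-zone, highlight and color changes to points, actor and a shared dynamic material.
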(event EventBeginPlay
  (bind _returnvalue (Game|SpawnActorfromClass "/Game/DMA/Blueprints/Core/BP_Moving_Actor.BP_Moving_Actor_C" (Math|Transform|MakeTransform "0, 0, 0" "0, 0, 0" "1,1,1") "AlwaysSpawn" 0 0))
  (Variables|/Game/DMA/Blueprints/Core/BP_Moving_Actor.BP_Moving_Actor_C|SetAttachedToContainer _returnvalue self)
  (Variables|Default|SetMovingActor _returnvalue)
  (bind _returnvalue_2 (Rendering|Material|CreateDynamicMaterialInstance "/Game/DMA/MaterialLibrary/M_Metal_Brushed_Nickel.M_Metal_Brushed_Nickel" "None" :!class /Script/Engine.KismetMaterialLibrary))
  (Variables|Default|SetPathMaterialInstance _returnvalue_2))

(event Collision|EventActorBeginOverlap
  (params (OtherActor :type Actor%20Object%20Reference)))

(event EventTick
  (params (DeltaSeconds :type Float%20%28single-precision%29)))

(fn ConstructionScript)

(fn UpdateFirstLastPoint
  (bind _outpoints (Class|MapperContainerBase|GetPointsOfClass "/Script/Kulagin.MapperPointInteractive"))
  (for (_array_element _array_index) _outpoints
    (if (== _array_index 0)
      (Class|MapperPointInteractive|SetFirst _array_element)
      (elif (== _array_index (Utilities|Array|LastIndex _outpoints))
        (Class|MapperPointInteractive|SetLast _array_element)
        (else
          (Class|MapperPointInteractive|SetNormal _array_element))))))

(fn CalculatePointsTimes
  (bind _outpoints (Class|MapperContainerBase|GetPointsOfClass "/Script/Kulagin.MapperPointInteractive"))
  (LocalVariables|SetInteractivePointsLocal _outpoints)
  (if (Utilities|Array|IsValidIndex (LocalVariables|GetInteractivePointsLocal))
    (Variables|/Script/Kulagin.MapperPointInteractive|SetEnterTime (Utilities|Array|Get(acopy) (LocalVariables|GetInteractivePointsLocal)) 0.0)
    (for _index (range 1 (Utilities|Array|LastIndex (Variables|Default|GetPointActors)))
      (Variables|/Script/Kulagin.MapperPointInteractive|SetEnterTime (Utilities|Array|Get(acopy) (LocalVariables|GetInteractivePointsLocal) _index) (+ (Class|MapperPointInteractive|GetLeaveTime (Utilities|Array|Get(acopy) (LocalVariables|GetInteractivePointsLocal) (- _index 1))) (/ (Transformation|GetDistanceTo (Utilities|Array|Get(acopy) (LocalVariables|GetInteractivePointsLocal) (- _index 1)) (Utilities|Array|Get(acopy) (LocalVariables|GetInteractivePointsLocal) _index)) (CallFunction|GetTargetSpeed (Transformation|GetActorLocation (Utilities|Array|Get(acopy) (LocalVariables|GetInteractivePointsLocal) (- _index 1))) (Utilities|Array|Get(acopy) (LocalVariables|GetInteractivePointsLocal) _index))))))
    (Variables|Default|SetTotalTime (Class|MapperPointInteractive|GetEnterTime (Utilities|Array|Get(acopy) (LocalVariables|GetInteractivePointsLocal) (Utilities|Array|LastIndex (LocalVariables|GetInteractivePointsLocal)))))
    (Interactive|UpdateTimeline)
    (return)))

(fn UpdatePointTime
  (params (Point :type Mapper%20Point%20Interactive%20Object%20Reference) (NewTime :type Float%20%28single-precision%29))
  (Utilities|IsValid Point
    (:Is%20Valid
      (LocalVariables|SetLocalPoint Point)
      (LocalVariables|SetLocalNewTime NewTime)
      (if (Utilities|Array|IsValidIndex (Variables|Default|GetPointActors))
        (if (and (Class|MapperPointInteractive|IsFirst (LocalVariables|GetLocalPoint)) (Class|MapperPointInteractive|IsLast (LocalVariables|GetLocalPoint)))
          (Interactive|UpdateTimeline)
          (elif (Class|MapperPointInteractive|IsFirst (LocalVariables|GetLocalPoint))
            (bind _output_get (LocalVariables|SetLocalNewTime (Math|Float|Min(Float) (LocalVariables|GetLocalNewTime) (Class|MapperPointInteractive|GetEnterTime (Class|MapperPointInteractive|GetNextOfClass (LocalVariables|GetLocalPoint) "/Script/Kulagin.MapperPointInteractive")))))
            (Class|MapperPointInteractive|UpdateSpeed (Class|MapperPointInteractive|GetNextOfClass (LocalVariables|GetLocalPoint) "/Script/Kulagin.MapperPointInteractive") (- (Class|MapperPointInteractive|GetEnterTime (Class|MapperPointInteractive|GetNextOfClass (LocalVariables|GetLocalPoint) "/Script/Kulagin.MapperPointInteractive")) _output_get))
            (Interactive|CalculatePointsTimes)
            (elif (Class|MapperPointInteractive|IsLast (LocalVariables|GetLocalPoint))
              (bind _output_get_2 (LocalVariables|SetLocalNewTime (Math|Float|Max(Float) (LocalVariables|GetLocalNewTime) (Class|MapperPointInteractive|GetLeaveTime (Class|MapperPointInteractive|GetPreviousOfClass (LocalVariables|GetLocalPoint) "/Script/Kulagin.MapperPointInteractive")))))
              (Class|MapperPointInteractive|UpdateSpeed (LocalVariables|GetLocalPoint) (- _output_get_2 (Class|MapperPointInteractive|GetLeaveTime (Class|MapperPointInteractive|GetPreviousOfClass (LocalVariables|GetLocalPoint) "/Script/Kulagin.MapperPointInteractive"))))
              (Interactive|CalculatePointsTimes)
              (else
                (bind _output_get_3 (LocalVariables|SetLocalNewTime (Math|Float|Clamp(Float) (LocalVariables|GetLocalNewTime) (Class|MapperPointInteractive|GetLeaveTime (Class|MapperPointInteractive|GetPreviousOfClass (LocalVariables|GetLocalPoint) "/Script/Kulagin.MapperPointInteractive")) (- (Class|MapperPointInteractive|GetEnterTime (Class|MapperPointInteractive|GetNextOfClass (LocalVariables|GetLocalPoint) "/Script/Kulagin.MapperPointInteractive")) (Class|MapperPointInteractive|GetWaitTime (LocalVariables|GetLocalPoint))))))
                (Class|MapperPointInteractive|UpdateSpeed (LocalVariables|GetLocalPoint) (- _output_get_3 (Class|MapperPointInteractive|GetLeaveTime (Class|MapperPointInteractive|GetPreviousOfClass (LocalVariables|GetLocalPoint) "/Script/Kulagin.MapperPointInteractive"))))
                (Class|MapperPointInteractive|UpdateSpeed (Class|MapperPointInteractive|GetNextOfClass (LocalVariables|GetLocalPoint) "/Script/Kulagin.MapperPointInteractive") (- (Class|MapperPointInteractive|GetEnterTime (Class|MapperPointInteractive|GetNextOfClass (LocalVariables|GetLocalPoint) "/Script/Kulagin.MapperPointInteractive")) (+ (LocalVariables|GetLocalNewTime) (Class|MapperPointInteractive|GetWaitTime (LocalVariables|GetLocalPoint)))))
                (Interactive|CalculatePointsTimes)))))
        (else
          (Interactive|UpdateTimeline :!label _label))))
    (:Is%20Not%20Valid
      (goto _label))))

(fn UpdateTimeline
  (bind _asw_mission_timeline (Utilities|Casting|CastToW_Mission_Timeline (Variables|Default|GetTimelineWidget)))
  (Default|UpdateTimeline _asw_mission_timeline)
  (bind _asbp_main_pawn (Utilities|Casting|CastToBP_Main_Pawn (Game|Player|GetPlayerPawn 0)))
  (Default|CalculateZoom (Variables|/Game/DMA/UI/Widgets/MenuWidget.MenuWidget_C|GetMissionsScroll (Variables|/Game/DMA/Blueprints/Core/BP_Main_Pawn.BP_Main_Pawn_C|GetMenuWidget _asbp_main_pawn)))
  (Default|CalculateMaxTime (Variables|/Game/DMA/UI/Widgets/MenuWidget.MenuWidget_C|GetMissionsScroll (Variables|/Game/DMA/Blueprints/Core/BP_Main_Pawn.BP_Main_Pawn_C|GetMenuWidget _asbp_main_pawn))))

(fn GetTargetPointat
  (params (InTime :type Float%20%28single-precision%29))
  (return (Class|MapperPointInteractive|GetNextOfClass (Interactive|GetPointat InTime) "/Script/Kulagin.MapperPointInteractive")))

(fn GetMovingActorRotationat
  (params (InTime :type Float%20%28single-precision%29))
  (return "0, 0, 0"))

(fn GetPointat
  (params (InTime :type Float%20%28single-precision%29))
  (bind _pointindex (Interactive|GetPointIndexat InTime))
  (bind _outpoints (Class|MapperContainerBase|GetPointsOfClass "/Script/Kulagin.MapperPointInteractive"))
  (if (Utilities|Array|IsValidIndex _outpoints _pointindex)
    (return (Utilities|Array|Get(acopy) _outpoints _pointindex))))

(fn GetPointIndexat
  (params (InTime :type Float%20%28single-precision%29))
  (bind _pointactors (Variables|Default|GetPointActors))
  (bind _returnvalue (Utilities|Array|LastIndex _pointactors))
  (bind _outpoints (Class|MapperContainerBase|GetPointsOfClass "/Script/Kulagin.MapperPointInteractive"))
  (for _index (range 0 (- _returnvalue 1))
    (if (and (>= InTime (Class|MapperPointInteractive|GetEnterTime (Utilities|Array|Get(acopy) _outpoints _index))) (< InTime (Class|MapperPointInteractive|GetEnterTime (Utilities|Array|Get(acopy) _outpoints (+ _index 1)))))
      (return _index)))
  (return _returnvalue))

(fn SetWorldTrackIsHighlighted
  (params (bNewIsHighlighted :type Boolean))
  (|CallParentFunction bNewIsHighlighted)
  (Rendering|Material|SetScalarParameterValue (Variables|Default|GetPathMaterialInstance) "Lines" (Math|Float|SelectFloat 1.0 0.0 bNewIsHighlighted) :!class /Script/Engine.MaterialInstanceDynamic)
  (return bNewIsHighlighted))

(fn SetTimelineIsHighlighted
  (params (bNewIsHighlighted :type Boolean))
  (|CallParentFunction bNewIsHighlighted)
  (bind _asw_mission_timeline (Utilities|Casting|CastToW_Mission_Timeline (Variables|Default|GetTimelineWidget))
    (:then
      (bind _output_get (Variables|/Game/DMA/UI/Widgets/W_Mission_Timeline.W_Mission_Timeline_C|SetbIsHighlighted _asw_mission_timeline bNewIsHighlighted))
      (return _output_get))
    (:CastFailed
      (return false))))

(fn StartMoving
  (bind _movingactor (Variables|Default|GetMovingActor))
  (|CallParentFunction)
  (Utilities|IsValid _movingactor
    (:Is%20Valid
      (Default|StartMoving _movingactor)
      (return true))
    (:Is%20Not%20Valid
      (return false))))

(fn SetPointsMaterial
  (|CallParentFunction)
  (for _array_element (Variables|Default|GetPointActors)
    (Class|MapperPointBase|SetMaterial _array_element (Variables|Default|GetPathMaterialInstance)))
  (return true))

(fn SetPointsColor
  (params (NewColor :type Linear%20Color%20Structure))
  (|CallParentFunction NewColor)
  (Rendering|Material|SetVectorParameterValue (Variables|Default|GetPathMaterialInstance) "Color" NewColor :!class /Script/Engine.MaterialInstanceDynamic)
  (return true))

(fn SetMovingActor
  (params (NewTime :type Float%20%28single-precision%29))
  (|CallParentFunction 0.0)
  (LocalVariables|SetCurrentTime NewTime)
  (bind _outpoints (Class|MapperContainerBase|GetPointsOfClass "/Script/Kulagin.MapperPointInteractive"))
  (for _index (range 1 (Utilities|Array|LastIndex _outpoints))
    (if (< (LocalVariables|GetCurrentTime) (Class|MapperPointInteractive|GetEnterTime (Utilities|Array|Get(acopy) _outpoints _index)))
      (Variables|/Game/DMA/Blueprints/Core/BP_Moving_Actor.BP_Moving_Actor_C|SetTargetPoint (Variables|Default|GetMovingActor) (Utilities|Array|Get(acopy) _outpoints _index))
      (Transformation|SetActorLocation (Variables|Default|GetMovingActor) (Math|Interpolation|Ease "Linear" (Math|Float|Absolute(Float) (/ (- (Class|MapperPointInteractive|GetEnterTime (Utilities|Array|Get(acopy) _outpoints _index)) (LocalVariables|GetCurrentTime)) (- (Class|MapperPointInteractive|GetLeaveTime (Utilities|Array|Get(acopy) _outpoints (- _index 1))) (Class|MapperPointInteractive|GetEnterTime (Utilities|Array|Get(acopy) _outpoints _index))))) (Transformation|GetActorLocation (Utilities|Array|Get(acopy) _outpoints _index)) (Transformation|GetActorLocation (Utilities|Array|Get(acopy) _outpoints (- _index 1)))) false false)
      (Transformation|SetActorRotation (Variables|Default|GetMovingActor) (Interactive|GetMovingActorRotationat (LocalVariables|GetCurrentTime)) :!label _label)
      (Variables|/Game/DMA/Blueprints/Core/BP_Moving_Actor.BP_Moving_Actor_C|SetCurrentPoint (Variables|Default|GetMovingActor) (+ (Interactive|GetPointIndexat (LocalVariables|GetCurrentTime)) 1))
      (Variables|/Game/DMA/Blueprints/Core/BP_Moving_Actor.BP_Moving_Actor_C|SetTargetPoint (Variables|Default|GetMovingActor) (Interactive|GetTargetPointat (LocalVariables|GetCurrentTime)))
      (return false)
      (elif (and (>= (LocalVariables|GetCurrentTime) (Class|MapperPointInteractive|GetEnterTime (Utilities|Array|Get(acopy) _outpoints _index))) (<= (LocalVariables|GetCurrentTime) (Class|MapperPointInteractive|GetLeaveTime (Utilities|Array|Get(acopy) _outpoints _index))))
        (Variables|/Game/DMA/Blueprints/Core/BP_Moving_Actor.BP_Moving_Actor_C|SetTargetPoint (Variables|Default|GetMovingActor) (Utilities|Array|Get(acopy) _outpoints _index))
        (Transformation|SetActorLocation (Variables|Default|GetMovingActor) (Transformation|GetActorLocation (Utilities|Array|Get(acopy) _outpoints _index)) false false)
        (goto _label))))
  (Transformation|SetActorLocation (Variables|Default|GetMovingActor) (Transformation|GetActorLocation (Utilities|Array|Get(acopy) _outpoints)) false false)
  (Transformation|SetActorRotation (Variables|Default|GetMovingActor) (Interactive|GetMovingActorRotationat (LocalVariables|GetCurrentTime)))
  (Variables|/Game/DMA/Blueprints/Core/BP_Moving_Actor.BP_Moving_Actor_C|SetCurrentPoint (Variables|Default|GetMovingActor) (+ (Interactive|GetPointIndexat (LocalVariables|GetCurrentTime)) 1))
  (Variables|/Game/DMA/Blueprints/Core/BP_Moving_Actor.BP_Moving_Actor_C|SetTargetPoint (Variables|Default|GetMovingActor) (Interactive|GetTargetPointat (LocalVariables|GetCurrentTime)))
  (return false))

(fn SetPaused
  (params (bNewIsPaused :type Boolean))
  (bind _returnvalue (|CallParentFunction bNewIsPaused))
  (bind _output_get (Variables|/Game/DMA/Blueprints/Core/BP_Moving_Actor.BP_Moving_Actor_C|SetPaused? (Variables|Default|GetMovingActor) _returnvalue))
  (return _output_get))

(fn SetPathVisibility
  (params (bNewIsVisible :type Boolean))
  (|CallParentFunction bNewIsVisible)
  (bind _outpoints (Class|MapperContainerBase|GetPointsOfClass "/Game/DMA/Blueprints/BP_Point_Interactive.BP_Point_Interactive_C"))
  (for _array_element _outpoints
    (Class|MapperPointInteractive|UpdatePathVisibility _array_element))
  (return (Variables|Default|GetbIsPathVisible)))

(fn RemovePath
  (bind _returnvalue (Class|KulaginStatics|GetMapperGameMode))
  (bind _pointcontainers (Variables|/Script/Kulagin.MapperGameMode|GetPointContainers _returnvalue))
  (|CallParentFunction)
  (Utilities|IsValid (Variables|Default|GetTimelineWidget)
    (:Is%20Valid
      (Widget|RemovefromParent (Variables|Default|GetTimelineWidget)))
    (:Is%20Not%20Valid
      _))
  (Variables|Default|SetTimelineWidget 0)
  (Utilities|Array|RemoveIndex _pointcontainers (Utilities|Array|FindItem _pointcontainers self))
  (for _array_element (Variables|Default|GetPointActors)
    (Actor|DestroyActor _array_element))
  (Actor|DestroyActor (Variables|Default|GetMovingActor))
  (Actor|DestroyActor)
  (return true))

(fn GetTotalTime
  (return (Variables|Default|GetTotalTime)))

(fn GetLocationatTime
  (params (TimeIn :type Float%20%28single-precision%29))
  (bind _pointactors (Variables|Default|GetPointActors))
  (bind _outpoints (Class|MapperContainerBase|GetPointsOfClass "/Script/Kulagin.MapperPointInteractive"))
  (for _index (range 1 (Utilities|Array|LastIndex _pointactors))
    (if (< TimeIn (Class|MapperPointInteractive|GetEnterTime (Utilities|Array|Get(acopy) _outpoints _index)))
      (return (Math|Interpolation|Ease "Linear" (Math|Float|Absolute(Float) (/ (- (Class|MapperPointInteractive|GetEnterTime (Utilities|Array|Get(acopy) _outpoints _index)) TimeIn) (- (Class|MapperPointInteractive|GetLeaveTime (Utilities|Array|Get(acopy) _outpoints (- _index 1))) (Class|MapperPointInteractive|GetEnterTime (Utilities|Array|Get(acopy) _outpoints _index))))) (Transformation|GetActorLocation (Utilities|Array|Get(acopy) _outpoints _index)) (Transformation|GetActorLocation (Utilities|Array|Get(acopy) _outpoints (- _index 1)))))
      (elif (and (>= TimeIn (Class|MapperPointInteractive|GetEnterTime (Utilities|Array|Get(acopy) _outpoints _index))) (<= TimeIn (Class|MapperPointInteractive|GetLeaveTime (Utilities|Array|Get(acopy) _outpoints _index))))
        (return (Transformation|GetActorLocation (Utilities|Array|Get(acopy) _outpoints _index))))))
  (return (Transformation|GetActorLocation (Utilities|Array|Get(acopy) _pointactors))))

(fn UpdateDangerZones
  (bind _returnvalue (|CallParentFunction))
  (if _returnvalue
    (bind _outpoints (Class|MapperContainerBase|GetPointsOfClass "/Game/DMA/Blueprints/BP_Point_Interactive.BP_Point_Interactive_C"))
    (for _array_element _outpoints
      (Class|MapperPointInteractive|UpdateCrossCylinder _array_element))
    (return true)
    (else
      (return false))))

(fn GetPoint
  (params (Index :type Integer))
  (bind _pointactors (Variables|Default|GetPointActors))
  (if (Utilities|Array|IsValidIndex _pointactors Index)
    (bind _asmapper_point_interactive (Utilities|Casting|CastToMapperPointInteractive (Utilities|Array|Get(acopy) _pointactors Index)))
    (return _asmapper_point_interactive)))

(fn GetActorsIgnoreCrossing
  (bind _output_get (LocalVariables|SetIgnoreLocal (|CallParentFunction)))
  (Utilities|Array|AppendArray _output_get (Variables|Default|GetPointActors))
  (Utilities|Array|Add (LocalVariables|GetIgnoreLocal) (Variables|Default|GetMovingActor))
  (Utilities|Array|Add (LocalVariables|GetIgnoreLocal) (Variables|/Game/DMA/Blueprints/Core/BP_Moving_Actor.BP_Moving_Actor_C|GetChildDrone (Variables|Default|GetMovingActor)))
  (return (LocalVariables|GetIgnoreLocal)))

(fn UpdateCrossRadius
  (bind _outpoints (Class|MapperContainerBase|GetPointsOfClass "/Script/Kulagin.MapperPointInteractive"))
  (for _array_element _outpoints
    (Class|MapperPointInteractive|UpdateCrossRadius _array_element)))

(fn SetDangerZoneVisibility
  (params (bNewIsVisible :type Boolean))
  (|CallParentFunction bNewIsVisible)
  (bind _outpoints (Class|MapperContainerBase|GetPointsOfClass "/Script/Kulagin.MapperPointInteractive"))
  (for _array_element _outpoints
    (Class|MapperPointInteractive|UpdateCrossVisibility _array_element))
  (return (Variables|Default|GetbIsDangerZoneVisible)))

(fn SetMovingActorVisibility
  (params (bNewIsVisible :type Boolean))
  (|CallParentFunction bNewIsVisible)
  (Default|SetMovingActorVisible (Variables|Default|GetMovingActor) (Variables|Default|GetbIsMovingActorVisible))
  (return (Variables|Default|GetbIsMovingActorVisible)))

(fn DropMovingActor
  (|CallParentFunction)
  (bind _returnvalue (Class|MapperDroneBase|DropMovingActor (Variables|Default|GetMovingActor)))
  (return _returnvalue))

(fn RiseMovingActor
  (|CallParentFunction)
  (bind _returnvalue (Class|MapperDroneBase|RiseMovingActor (Variables|Default|GetMovingActor)))
  (return _returnvalue))