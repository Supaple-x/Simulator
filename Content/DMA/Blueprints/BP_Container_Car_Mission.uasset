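; Mission container for a car path in the drone mapper, which spawns a RED_NVO actor on BeginPlay as its moving actor and creates a brushed nickel material instance for the path.
; The moving actor's rotation faces from the current point toward the next interactive point, or keeps its current rotation.
; Saving and offset copying reuse Plane Mission point types and functions, writing to file or loading the copy through the game mode.
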(event EventBeginPlay
  (bind _returnvalue (Game|SpawnActorfromClass "/Game/Graphics/REN_NVO_73/RED_NVO.RED_NVO_C" (Math|Transform|MakeTransform "0, 0, 0" "0, 0, 0" "1,1,1") "AlwaysSpawn" 0 0))
  (Variables|/Game/DMA/Blueprints/Core/BP_Moving_Actor.BP_Moving_Actor_C|SetAttachedToContainer _returnvalue self)
  (Variables|Default|SetMovingActor _returnvalue)
  (bind _returnvalue_2 (Rendering|Material|CreateDynamicMaterialInstance "/Game/DMA/MaterialLibrary/M_Metal_Brushed_Nickel.M_Metal_Brushed_Nickel" "None" :!class /Script/Engine.KismetMaterialLibrary))
  (Variables|Default|SetPathMaterialInstance _returnvalue_2))

(fn ConstructionScript)

(fn GetMovingActorRotationat
  (params (InTime :type Float%20%28single-precision%29))
  (bind _point (CallFunction|GetPointat InTime))
  (LocalVariables|SetFirstLocal _point)
  (LocalVariables|SetSecondLocal (Class|MapperPointInteractive|GetNextOfClass _point "/Script/Kulagin.MapperPointInteractive"))
  (Utilities|IsValid (LocalVariables|GetFirstLocal)
    (:Is%20Valid
      (Utilities|IsValid (LocalVariables|GetSecondLocal)
        (:Is%20Valid
          (return (Math|Rotator|FindLookatRotation (Transformation|GetActorLocation (LocalVariables|GetFirstLocal)) (Transformation|GetActorLocation (LocalVariables|GetSecondLocal)))))
        (:Is%20Not%20Valid
          _)))
    (:Is%20Not%20Valid
      _))
  (return (Transformation|GetActorRotation (Variables|Default|GetMovingActor))))

(fn GetActualPointData
  (bind _outpoints (Class|MapperContainerBase|GetPointsOfClass "/Game/DMA/Blueprints/BP_Point_Plane_Mission.BP_Point_Plane_Mission_C"))
  (for _array_element _outpoints
    (Utilities|Array|Add (LocalVariables|GetDataLocal) (Variables|/Game/DMA/Blueprints/BP_Point_Plane_Mission.BP_Point_Plane_Mission_C|GetPointData _array_element)))
  (return (LocalVariables|GetDataLocal)))

(fn SavePath
  (bind _data (CallFunction|GetActualPointData))
  (bind _returnvalue (Class|KulaginStatics|SavePlanePointstoFile (Variables|Default|GetFilePath) _data))
  (Development|PrintString (Utilities|String|Append "Kulagin: SavePath for Plane Mission is " (Utilities|String|SelectString "VALID" "FAILED" _returnvalue)))
  (return true))

(fn CopyPath
  (params (Offset :type Vector :default "0, 0, 0"))
  (bind _data (CallFunction|GetActualPointData))
  (Class|KulaginStatics|AddPlaneMissionPointsOffset _data Offset)
  (Default|LoadPlaneMission (CallFunction|GetDroneMapperGamemode) (Utilities|Struct|MakePlaneMissionPointList (Variables|Default|GetFilePath) _data "()" "()"))
  (return true))