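; Drone mission path container that spawns the moving drone travelling its path and can display it as a swarm.
; With multiple drones, it hides the lead drone and attaches spawned copies to it in a centred grid set by row size and spacing.
; Setting changes clamp values and update each drone's spotlight and smoke.
; It also derives yaw from point POI headings, saves points to file and loads offset copies through the game mode.
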(event EventDestroyed
  (|CallParentFunction)
  (CallFunction|ClearSwarm))

(event EventBeginPlay
  (bind _returnvalue (Game|SpawnActorfromClass "/Game/DMA/Blueprints/Core/BP_Moving_Actor_Drone.BP_Moving_Actor_Drone_C" (Math|Transform|MakeTransform "0, 0, 0" "0, 0, 0" "1,1,1") "AlwaysSpawn" 0 0))
  (Variables|/Game/DMA/Blueprints/Core/BP_Moving_Actor.BP_Moving_Actor_C|SetAttachedToContainer _returnvalue self)
  (bind _output_get (Variables|Default|SetMovingActorDrone _returnvalue))
  (Variables|Default|SetMovingActor _output_get)
  (bind _returnvalue_2 (Rendering|Material|CreateDynamicMaterialInstance "/Game/DMA/MaterialLibrary/M_Metal_Brushed_Nickel.M_Metal_Brushed_Nickel" "None" :!class /Script/Engine.KismetMaterialLibrary))
  (Variables|Default|SetPathMaterialInstance _returnvalue_2))

(fn ConstructionScript)

(fn GetMovingActorRotationat
  (params (InTime :type Float%20%28single-precision%29))
  (bind _asbp_point_drone_mission (Utilities|Casting|CastToBP_Point_Drone_Mission (CallFunction|GetPointat InTime)))
  (Utilities|IsValid (Class|MapperPointInteractive|GetNextOfClass _asbp_point_drone_mission "/Game/DMA/Blueprints/BP_Point_Drone_Mission.BP_Point_Drone_Mission_C")
    (:Is%20Valid
      (return (Math|Rotator|MakeRotator 0.0 0.0 (.poiHeading (Utilities|Struct|BreakMissionPoint (Variables|/Game/DMA/Blueprints/BP_Point_Drone_Mission.BP_Point_Drone_Mission_C|GetPointData (Class|MapperPointInteractive|GetNextOfClass _asbp_point_drone_mission "/Game/DMA/Blueprints/BP_Point_Drone_Mission.BP_Point_Drone_Mission_C")))))))
    (:Is%20Not%20Valid
      (return (Math|Rotator|MakeRotator 0.0 0.0 (.poiHeading (Utilities|Struct|BreakMissionPoint (Variables|/Game/DMA/Blueprints/BP_Point_Drone_Mission.BP_Point_Drone_Mission_C|GetPointData _asbp_point_drone_mission))))))))

(fn GetActualPointData
  (bind _outpoints (Class|MapperContainerBase|GetPointsOfClass "/Game/DMA/Blueprints/BP_Point_Drone_Mission.BP_Point_Drone_Mission_C"))
  (for _array_element _outpoints
    (Utilities|Array|Add (LocalVariables|GetDataLocal) (Variables|/Game/DMA/Blueprints/BP_Point_Drone_Mission.BP_Point_Drone_Mission_C|GetPointData _array_element)))
  (return (LocalVariables|GetDataLocal)))

(fn SavePath
  (bind _data (CallFunction|GetActualPointData))
  (bind _returnvalue (Class|KulaginStatics|SavePointstoFile (Variables|Default|GetFilePath) _data))
  (Development|PrintString (Utilities|String|Append "Kulagin: SavePath for Drone Mission is " (Utilities|String|SelectString "VALID" "FAILED" _returnvalue)))
  (return true))

(fn CopyPath
  (params (Offset :type Vector :default "0, 0, 0"))
  (bind _data (CallFunction|GetActualPointData))
  (Class|KulaginStatics|AddMissionPointsOffset _data Offset)
  (Default|LoadMission (CallFunction|GetDroneMapperGamemode) (Utilities|Struct|MakeMissionPointList (Variables|Default|GetFilePath) "PCT_Mission" "()" "()" _data (Utilities|Array|MakeArray "") (Utilities|Array|MakeArray "") (Utilities|Array|MakeArray "")))
  (return true))

(fn OnNumberOfDronesChanged
  (params (NewNumberOfDrones :type Integer))
  (bind _output_get (Variables|Default|SetDronesCount (Math|Integer|Max(Integer) NewNumberOfDrones 1)))
  (CallFunction|ClearSwarm)
  (if (> _output_get 1)
    (CallFunction|RespawnSwarm)
    (CallFunction|RelocateSwarm))
  (CallFunction|SetMovingActorVisibility (Variables|Default|GetbIsMovingActorVisible))
  (CallFunction|UpdateAllDrones))

(fn OnLightStrengthChanged
  (params (NewLightStrength :type Float%20%28single-precision%29))
  (Variables|Default|SetLightStrength (Math|Float|Clamp(Float) NewLightStrength 0.0 1e+05))
  (CallFunction|UpdateAllDrones))

(fn OnLightAngleChanged
  (params (NewLightAngle :type Float%20%28single-precision%29))
  (Variables|Default|SetLightAngle (Math|Float|Clamp(Float) NewLightAngle 0.0 9e+01))
  (CallFunction|UpdateAllDrones))

(fn OnLightTemperatureChanged
  (params (NewLightTemperature :type Float%20%28single-precision%29))
  (Variables|Default|SetLightTemp (Math|Float|Clamp(Float) NewLightTemperature 1.7e+03 1.2e+04))
  (CallFunction|UpdateAllDrones))

(fn OnNumberOfDronesinOneRowChanged
  (params (NewNumberInOneRow :type Integer))
  (Variables|Default|SetDronesInRow (Math|Integer|Max(Integer) NewNumberInOneRow 1))
  (CallFunction|RelocateSwarm))

(fn OnDistanceBetweenDronesChanged
  (params (NewDistance :type Float%20%28single-precision%29))
  (Variables|Default|SetDistance (Math|Float|Max(Float) NewDistance 1e+02))
  (CallFunction|RelocateSwarm))

(fn RelocateSwarm
  (LocalVariables|SetCountX (Variables|Default|GetDronesInRow))
  (LocalVariables|SetCountY (Math|Float|Ceil (/ (Math|Conversions|ToFloat(Integer) (Variables|Default|GetDronesCount)) (Math|Conversions|ToFloat(Integer) (Variables|Default|GetDronesInRow)))))
  (LocalVariables|SetBeginLocation (* (Math|Vector|MakeVector (* (- (LocalVariables|GetCountX) 1) (Variables|Default|GetDistance)) (* (- (LocalVariables|GetCountY) 1) (Variables|Default|GetDistance)) 0.0) -0.5))
  (for _index (range 0 (- (LocalVariables|GetCountX) 1))
    (LocalVariables|SetIndexX _index)
    (for _index_2 (range 0 (- (LocalVariables|GetCountY) 1))
      (LocalVariables|SetIndexY _index_2)
      (bind _result (Math|Integer|IncrementInt (LocalVariables|GetDroneIndex))
        (:%20%20
          (if (Utilities|Array|IsValidIndex (Variables|Default|GetSwarmDrones) _result)
            (Transformation|SetActorRelativeLocation (Utilities|Array|Get(acopy) (Variables|Default|GetSwarmDrones) (LocalVariables|GetDroneIndex)) (Math|Vector|MakeVector (Class|KulaginStatics|LifetoUU (.x (* (+ (* (Math|Vector|MakeVector (Math|Conversions|ToFloat(Integer) (LocalVariables|GetIndexX)) (Math|Conversions|ToFloat(Integer) (LocalVariables|GetIndexY)) 0.0) (Variables|Default|GetDistance)) (LocalVariables|GetBeginLocation)) 0.01))) (Class|KulaginStatics|LifetoUU (.y (* (+ (* (Math|Vector|MakeVector (Math|Conversions|ToFloat(Integer) (LocalVariables|GetIndexX)) (Math|Conversions|ToFloat(Integer) (LocalVariables|GetIndexY)) 0.0) (Variables|Default|GetDistance)) (LocalVariables|GetBeginLocation)) 0.01))) 0.0))
            (else
              (return))))))))

(fn RespawnSwarm
  (for _index (range 1 (Variables|Default|GetDronesCount))
    (bind _returnvalue (Game|SpawnActorfromClass "/Game/DMA/Blueprints/Core/BP_Moving_Actor_Drone.BP_Moving_Actor_Drone_C" (Transformation|GetActorTransform (Variables|Default|GetMovingActor)) "AlwaysSpawn" 0 0))
    (Utilities|Array|Add (Variables|Default|GetSwarmDrones) _returnvalue)
    (Transformation|AttachActorToActor _returnvalue (Variables|Default|GetMovingActor) "None" "KeepWorld" "KeepWorld" "KeepWorld" true)))

(fn ClearSwarm
  (for _array_element (Variables|Default|GetSwarmDrones)
    (Actor|DestroyActor _array_element))
  (Utilities|Array|Clear (Variables|Default|GetSwarmDrones)))

(fn SetMovingActorVisibility
  (params (bNewIsVisible :type Boolean))
  (bind _returnvalue (|CallParentFunction bNewIsVisible))
  (Default|SetMovingActorVisible (Variables|Default|GetMovingActorDrone) (and _returnvalue (<= (Variables|Default|GetDronesCount) 1)))
  (for _array_element (Variables|Default|GetSwarmDrones)
    (Default|SetMovingActorVisible _array_element _returnvalue))
  (return _returnvalue))

(fn UpdateAllDrones
  (if (> (Variables|Default|GetDronesCount) 1)
    (for _array_element (Variables|Default|GetSwarmDrones)
      (CallFunction|UpdateDrone _array_element))
    (else
      (CallFunction|UpdateDrone (Variables|Default|GetMovingActorDrone)))))

(fn OnLightEnabledChanged
  (params (bNewEnabled :type Boolean))
  (Variables|Default|SetbLightEnabled bNewEnabled)
  (CallFunction|UpdateAllDrones))

(fn OnSmokeEnabledChanged
  (params (bNewSmokeEnabled :type Boolean))
  (Variables|Default|SetbSmokeEnabled bNewSmokeEnabled)
  (CallFunction|UpdateAllDrones))

(fn UpdateDrone
  (params (Drone :type BP%20Moving%20Actor%20Drone%20Object%20Reference))
  (bind _spotlight (Variables|/Game/DMA/Blueprints/Core/BP_Moving_Actor_Drone.BP_Moving_Actor_Drone_C|GetSpotLight Drone))
  (bind _particlesystem (Variables|/Game/DMA/Blueprints/Core/BP_Moving_Actor_Drone.BP_Moving_Actor_Drone_C|GetParticleSystem Drone))
  (Rendering|Lighting|SetOuterConeAngle _spotlight (Variables|Default|GetLightAngle))
  (Class|LightComponent|SetTemperature _spotlight (Variables|Default|GetLightTemp))
  (Rendering|Components|Light|SetIntensity _spotlight (Variables|Default|GetLightStrength))
  (Development|SetHiddeninGame _spotlight (not (Variables|Default|GetbLightEnabled)) false)
  (if (Variables|Default|GetbSmokeEnabled)
    (Components|Activation|Activate _particlesystem true)
    (else
      (Components|Activation|Deactivate _particlesystem))))