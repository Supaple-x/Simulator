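; Car prop Blueprint with configurable paint tint and roughness, applied in the construction script; the event graph has no active logic.
; It creates dynamic material instances on three slots of the Car component and feeds them the ColorTint and RougnessPower variables.
; The NewRoofMaterial flag swaps the third slot's source to an alternate material, though the parameter calls reference only the instance from the default-material branch.
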(event EventBeginPlay)

(event Collision|EventActorBeginOverlap
  (params (OtherActor :type Actor%20Object%20Reference)))

(event EventTick
  (params (DeltaSeconds :type Float%20%28single-precision%29)))

(fn ConstructionScript
  (bind _car (Variables|Default|GetCar))
  (bind _color_tint (Variables|Default|GetColor_Tint))
  (bind _rougness_power (Variables|Default|GetRougness_Power))
  (Utilities|FlowControl|Sequence
    (:then_0
      (bind _returnvalue (Rendering|Material|CreateDynamicMaterialInstance _car 9 (Rendering|Material|GetMaterial _car 9) "None" :!class /Script/Engine.PrimitiveComponent))
      (Rendering|Material|SetVectorParameterValue _returnvalue "Color_Tint" _color_tint :!class /Script/Engine.MaterialInstanceDynamic)
      (Rendering|Material|SetScalarParameterValue _returnvalue "Rougness_Power" _rougness_power :!class /Script/Engine.MaterialInstanceDynamic))
    (:then_1
      (bind _returnvalue_2 (Rendering|Material|CreateDynamicMaterialInstance _car 10 (Rendering|Material|GetMaterial _car 10) "None" :!class /Script/Engine.PrimitiveComponent))
      (Rendering|Material|SetVectorParameterValue _returnvalue_2 "Color_Tint" _color_tint :!class /Script/Engine.MaterialInstanceDynamic)
      (Rendering|Material|SetScalarParameterValue _returnvalue_2 "Rougness_Power" _rougness_power :!class /Script/Engine.MaterialInstanceDynamic))
    (:then_2
      (if (Variables|Default|GetNew_Roof_Material)
        (Rendering|Material|CreateDynamicMaterialInstance (Variables|Default|GetCar) 11 "/Game/IPU/Maps/IPU/Car/dff62f9c_dds_005.dff62f9c_dds_005" "None" :!class /Script/Engine.PrimitiveComponent)
        (else
          (bind _returnvalue_3 (Rendering|Material|CreateDynamicMaterialInstance _car 11 (Rendering|Material|GetMaterial _car 11) "None" :!class /Script/Engine.PrimitiveComponent))))
      (Rendering|Material|SetVectorParameterValue _returnvalue_3 "Color_Tint" _color_tint :!class /Script/Engine.MaterialInstanceDynamic)
      (Rendering|Material|SetScalarParameterValue _returnvalue_3 "Rougness_Power" _rougness_power :!class /Script/Engine.MaterialInstanceDynamic))))