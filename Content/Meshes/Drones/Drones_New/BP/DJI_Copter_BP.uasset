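; DJI copter drone Blueprint that animates six spinning propeller components.
; BeginPlay builds a yaw-only rotation rate from ScrewsSpeed.
; Each Tick, ScrewAddRotation scales that rate by delta time and applies it as relative rotation to all six propellers, keeping the spin frame-rate independent.
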(event EventBeginPlay
  (|CallParentFunction)
  (Variables|Default|SetRotation_Screw (Math|Rotator|MakeRotator 0.0 0.0 (Variables|Default|GetScrews_Speed))))

(event EventTick
  (params (DeltaSeconds :type Float%20%28single-precision%29))
  (|CallParentFunction DeltaSeconds)
  (CallFunction|ScrewAddRotation DeltaSeconds))

(fn ConstructionScript)

(fn ScrewAddRotation
  (params (TimeDelta :type Float%20%28single-precision%29))
  (bind _rotation_screw (Variables|Default|GetRotation_Screw))
  (bind _returnvalue (* _rotation_screw TimeDelta))
  (Transformation|AddRelativeRotation (Variables|Default|GetDJI_vint) _returnvalue false false)
  (Transformation|AddRelativeRotation (Variables|Default|GetDJI_vint2) _returnvalue false false)
  (Transformation|AddRelativeRotation (Variables|Default|GetDJI_vint3) _returnvalue false false)
  (Transformation|AddRelativeRotation (Variables|Default|GetDJI_vint5) _returnvalue false false)
  (Transformation|AddRelativeRotation (Variables|Default|GetDJI_vint6) _returnvalue false false)
  (Transformation|AddRelativeRotation (Variables|Default|GetDJI_vint1) _returnvalue false false))