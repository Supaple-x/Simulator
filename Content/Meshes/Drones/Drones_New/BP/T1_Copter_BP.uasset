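; T1 copter drone Blueprint that spins four rotor meshes and can switch its body in and out of physics simulation.
; BeginPlay builds a yaw rate from ScrewsSpeed, and Tick applies it to each screw, scaled by delta time.
; DropMovingActor enables physics on the body mesh.
; RiseMovingActor disables it, resets the body's relative transform and reattaches it to the capsule.
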(event EventBeginPlay
  (|CallParentFunction)
  (Variables|Default|SetRotation_Screw (Math|Rotator|MakeRotator 0.0 0.0 (Variables|Default|GetScrews_Speed))))

(event EventTick
  (params (DeltaSeconds :type Float%20%28single-precision%29))
  (|CallParentFunction DeltaSeconds)
  (CallFunction|ScrewAddRotation DeltaSeconds))

(fn ConstructionScript)

(fn ScrewAddRotation
  (params (TimeDelta :type Float%20%28single-precision%29))
  (bind _rotation_screw (Variables|Default|GetRotation_Screw))
  (bind _returnvalue (* _rotation_screw TimeDelta))
  (Transformation|AddRelativeRotation (Variables|Default|Gett1_Screw4) _returnvalue false false)
  (Transformation|AddRelativeRotation (Variables|Default|Gett1_Screw3) _returnvalue false false)
  (Transformation|AddRelativeRotation (Variables|Default|Gett1_Screw2) _returnvalue false false)
  (Transformation|AddRelativeRotation (Variables|Default|Gett1_Screw1) _returnvalue false false))

(fn DropMovingActor
  (Physics|SetSimulatePhysics (Variables|Default|Gett1_body1) true)
  (return true))

(fn RiseMovingActor
  (Physics|SetSimulatePhysics (Variables|Default|Gett1_body1) false)
  (Transformation|SetRelativeLocationAndRotation (Variables|Default|Gett1_body1) "0, 0, 0" "0,-90.000000, 0" false false)
  (Transformation|AttachComponentToComponent (Variables|Default|Gett1_body1) (Variables|Default|GetCapsuleComponent) "None" "KeepRelative" "KeepRelative" "KeepRelative" true)
  (return true))