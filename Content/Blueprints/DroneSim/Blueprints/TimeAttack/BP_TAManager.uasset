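; Time-attack manager for the drone sim: runs the countdown, lap race, results and level restart.
; Gathers checkpoints by their Index, highlights the next one and points a drone-camera arrow at it; passing the last starts a new lap or ends the race.
; Tick drives countdown and timer through Delays, adding fixed 0.01 steps rather than DeltaSeconds, so timing depends on frame rate.
; Best lap and total times persist via BP_TAHighScores.
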(event Custom|Timer%20Tick
  (if (Variables|Default|GetIsTiming)
    (Utilities|FlowControl|Delay 0.01)
    (Variables|Default|SetTotal%20Time (+ (Variables|Default|GetTotal%20Time) 0.01))
    (Variables|Default|SetCurrent%20Lap%20Time (+ (Variables|Default|GetCurrent%20Lap%20Time) 0.01))))

(event Custom|Countdown%20Tick
  (if (Variables|Default|GetNeed%20Countdown)
    (if (> (Variables|Default|GetCountdown) 0)
      (Utilities|FlowControl|Delay 1.0)
      (Audio|PlaySound2D (Variables|Default|GetCountdown%20Sound) 1.0 1.0 0.0 0 0)
      (Math|Integer|DecrementInt (Variables|Default|GetCountdown))
      (else
        (Utilities|FlowControl|Delay 1.0)
        (Audio|PlaySound2D (Variables|Default|GetStart%20Sound) 1.0 1.0 0.0 0 0)
        (CallFunction|StartRace)))))

(event Custom|Arrow%20Tick
  (params (Delta :type Float%20%28single-precision%29))
  (Transformation|SetWorldRotation (Variables|Default|GetArrow) (Math|Interpolation|RInterpTo (Transformation|GetWorldRotation (Variables|Default|GetArrow)) (Math|Rotator|FindLookatRotation (Transformation|GetWorldLocation (Variables|Default|GetArrow)) (Transformation|GetActorLocation (Variables|Default|GetNext%20Checkpoint))) Delta 4.0) false false))

(event EventTick
  (params (DeltaSeconds :type Float%20%28single-precision%29))
  (CallFunction|ArrowTick DeltaSeconds)
  (CallFunction|TimerTick)
  (CallFunction|CountdownTick))

(event EventBeginPlay
  (Input|EnableInput (Game|GetPlayerController 0))
  (Input|DisableInput (Game|Player|GetPlayerPawn 0) (Game|GetPlayerController 0))
  (CallFunction|LoadScores)
  (bind _outactors (Actor|GetAllActorsOfClass "/Game/Blueprints/DroneSim/Blueprints/TimeAttack/BP_TACheckpoint.BP_TACheckpoint_C"))
  (for _array_element _outactors
    (Utilities|Array|SetArrayElem (Variables|Default|GetCheckpoints) (Variables|/Game/Blueprints/DroneSim/Blueprints/TimeAttack/BP_TACheckpoint.BP_TACheckpoint_C|GetIndex _array_element) _array_element true))
  (CallFunction|SetNextCheckpoint)
  (bind _returnvalue (UserInterface|CreateWidget "/Game/Blueprints/DroneSim/Blueprints/TimeAttack/HUD_TimeAttack.HUD_TimeAttack_C"))
  (UserInterface|Viewport|AddtoViewport _returnvalue 0)
  (bind _returnvalue_2 (AddComponent|AddArrowComponent true))
  (Variables|Default|SetArrow _returnvalue_2)
  (bind _outactors_2 (Actor|GetAllActorswithTag "Drone"))
  (Transformation|AttachComponentToComponent (Variables|Default|GetArrow) (Utilities|Array|Get(acopy) (Actor|GetComponentsbyTag (Utilities|Array|Get(acopy) _outactors_2) "/Script/Engine.CameraComponent" "TPCamera")) "None" "KeepRelative" "KeepRelative" "KeepRelative" true)
  (Rendering|SetVisibility (Variables|Default|GetArrow) false false))

(event Input|KeyboardEvents|Enter
  (params (Key :type Key%20Structure))
  (:Pressed
    (CallFunction|PlayAgain)))

(event Input|GamepadEvents|GamepadSpecialRight
  (params (Key :type Key%20Structure))
  (:Pressed
    (CallFunction|PlayAgain)))

(fn ConstructionScript)

(fn SetNextCheckpoint
  (Utilities|IsValid (Variables|Default|GetNext%20Checkpoint)
    (:Is%20Valid
      (Utilities|IsValid (Utilities|Array|Get(acopy) (Variables|Default|GetCheckpoints) (+ (Variables|/Game/Blueprints/DroneSim/Blueprints/TimeAttack/BP_TACheckpoint.BP_TACheckpoint_C|GetIndex (Variables|Default|GetNext%20Checkpoint)) 1))
        (:Is%20Valid
          (Variables|Default|SetNext%20Checkpoint (Utilities|Array|Get(acopy) (Variables|Default|GetCheckpoints) (+ (Variables|/Game/Blueprints/DroneSim/Blueprints/TimeAttack/BP_TACheckpoint.BP_TACheckpoint_C|GetIndex (Variables|Default|GetNext%20Checkpoint)) 1))))
        (:Is%20Not%20Valid
          (CallFunction|NewLap))))
    (:Is%20Not%20Valid
      (Variables|Default|SetNext%20Checkpoint (Utilities|Array|Get(acopy) (Variables|Default|GetCheckpoints)))))
  (Rendering|Material|SetMaterial (Variables|/Game/Blueprints/DroneSim/Blueprints/TimeAttack/BP_TACheckpoint.BP_TACheckpoint_C|GetMesh (Variables|Default|GetNext%20Checkpoint)) 0 "/Game/Blueprints/DroneSim/Materials/TimeAttack/M_TranslucentGreen.M_TranslucentGreen")
  (Variables|/Game/Blueprints/DroneSim/Blueprints/TimeAttack/BP_TACheckpoint.BP_TACheckpoint_C|SetIsNextCheckpoint (Variables|Default|GetNext%20Checkpoint) true))

(fn StartTimer
  (Variables|Default|SetIsTiming true))

(fn StopTimer
  (Variables|Default|SetIsTiming false))

(fn NewLap
  (CallFunction|CheckBestLapTime)
  (Utilities|Array|SetArrayElem (Variables|Default|GetLap%20Times) (- (Variables|Default|GetCurrent%20Lap) 1) (Variables|Default|GetCurrent%20Lap%20Time) true)
  (Variables|Default|SetCurrent%20Lap%20Time 0.0)
  (if (< (Variables|Default|GetCurrent%20Lap) (Variables|Default|GetTotal%20Laps))
    (Math|Integer|IncrementInt (Variables|Default|GetCurrent%20Lap)
      (:%20%20
        (Variables|Default|SetNext%20Checkpoint (Utilities|Array|Get(acopy) (Variables|Default|GetCheckpoints)))))
    (else
      (CallFunction|EndRace))))

(fn EndRace
  (CallFunction|StopTimer)
  (Rendering|SetVisibility (Variables|Default|GetArrow) false false)
  (if (< (Variables|Default|GetTotal%20Time) (Variables|Default|GetBest%20Total%20Time))
    (Variables|Default|SetBest%20Total%20Time (Variables|Default|GetTotal%20Time)))
  (CallFunction|SaveScores)
  (Variables|Default|SetIsHUDVisible false)
  (Variables|Default|SetIsResultsVisible true))

(fn CheckBestLapTime
  (if (< (Variables|Default|GetCurrent%20Lap%20Time) (Variables|Default|GetBest%20Lap%20Time))
    (Variables|Default|SetBest%20Lap%20Time (Variables|Default|GetCurrent%20Lap%20Time))))

(fn CheckBestTotalTime)

(fn SaveScores
  (bind _returnvalue (SaveGame|CreateSaveGameObject "/Game/Blueprints/DroneSim/Blueprints/TimeAttack/BP_TAHighScores.BP_TAHighScores_C"))
  (Variables|Default|SetSave%20Game%20Instance _returnvalue)
  (Variables|/Game/Blueprints/DroneSim/Blueprints/TimeAttack/BP_TAHighScores.BP_TAHighScores_C|SetBest%20Lap%20Time (Variables|Default|GetSave%20Game%20Instance) (Variables|Default|GetBest%20Lap%20Time))
  (Variables|/Game/Blueprints/DroneSim/Blueprints/TimeAttack/BP_TAHighScores.BP_TAHighScores_C|SetBest%20Total%20Time (Variables|Default|GetSave%20Game%20Instance) (Variables|Default|GetBest%20Total%20Time))
  (SaveGame|SaveGametoSlot (Variables|Default|GetSave%20Game%20Instance) (Variables|/Game/Blueprints/DroneSim/Blueprints/TimeAttack/BP_TAHighScores.BP_TAHighScores_C|GetSave%20Slot%20Name (Variables|Default|GetSave%20Game%20Instance)) (Variables|/Game/Blueprints/DroneSim/Blueprints/TimeAttack/BP_TAHighScores.BP_TAHighScores_C|GetUser%20Index (Variables|Default|GetSave%20Game%20Instance))))

(fn LoadScores
  (bind _returnvalue (SaveGame|CreateSaveGameObject "/Game/Blueprints/DroneSim/Blueprints/TimeAttack/BP_TAHighScores.BP_TAHighScores_C"))
  (bind _output_get (Variables|Default|SetSave%20Game%20Instance _returnvalue))
  (bind _returnvalue_2 (SaveGame|LoadGamefromSlot (Variables|/Game/Blueprints/DroneSim/Blueprints/TimeAttack/BP_TAHighScores.BP_TAHighScores_C|GetSave%20Slot%20Name _output_get) (Variables|/Game/Blueprints/DroneSim/Blueprints/TimeAttack/BP_TAHighScores.BP_TAHighScores_C|GetUser%20Index _output_get)))
  (bind _asbp_tahigh_scores (Utilities|Casting|CastToBP_TAHighScores _returnvalue_2))
  (Variables|Default|SetSave%20Game%20Instance _asbp_tahigh_scores)
  (Variables|Default|SetBest%20Lap%20Time (Variables|/Game/Blueprints/DroneSim/Blueprints/TimeAttack/BP_TAHighScores.BP_TAHighScores_C|GetBest%20Lap%20Time (Variables|Default|GetSave%20Game%20Instance)))
  (Variables|Default|SetBest%20Total%20Time (Variables|/Game/Blueprints/DroneSim/Blueprints/TimeAttack/BP_TAHighScores.BP_TAHighScores_C|GetBest%20Total%20Time (Variables|Default|GetSave%20Game%20Instance))))

(fn StartRace
  (Rendering|SetVisibility (Variables|Default|GetArrow) true false)
  (Variables|Default|SetNeed%20Countdown false)
  (Variables|Default|SetIsCountdownVisible false)
  (Variables|Default|SetIsHUDVisible true)
  (CallFunction|StartTimer)
  (Input|EnableInput (Game|Player|GetPlayerPawn 0) (Game|GetPlayerController 0)))

(fn PlayAgain
  (bind _returnvalue (Game|GetCurrentLevelName true))
  (Game|OpenLevel(byName) (Utilities|String|StringToName _returnvalue)))