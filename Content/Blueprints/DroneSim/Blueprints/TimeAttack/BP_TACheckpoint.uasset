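; BP_TACheckpoint is a checkpoint actor for the drone sim's time attack mode, linked to the first BP_TAManager found at BeginPlay.
; When the player character overlaps it while it is the next checkpoint, it has the manager advance the sequence, turns translucent red, clears its flag and plays the checkpoint sound.
; The checkpoint with index zero also starts the manager's timer if it is not already running.
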(event OnComponentBeginOverlap(Collision)
  (params (OverlappedComponent :type Primitive%20Component%20Object%20Reference) (OtherActor :type Actor%20Object%20Reference) (OtherComp :type Primitive%20Component%20Object%20Reference) (OtherBodyIndex :type Integer) (bFromSweep :type Boolean) (SweepResult :type Hit%20Result%20Structure%20%28by%20ref%29))
  (bind _ascharacter (Utilities|Casting|CastToCharacter OtherActor))
  (if (and (== (Game|GetPlayerCharacter 0) _ascharacter) (Variables|Default|GetIsNextCheckpoint))
    (CallFunction|CheckTimer)
    (Default|SetNextCheckpoint (Variables|Default|GetManagerReference))
    (Rendering|Material|SetMaterial (Variables|Default|GetMesh) 0 "/Game/Blueprints/DroneSim/Materials/TimeAttack/M_TranslucentRed.M_TranslucentRed")
    (Variables|Default|SetIsNextCheckpoint false)
    (Audio|PlaySound2D (Variables|/Game/Blueprints/DroneSim/Blueprints/TimeAttack/BP_TAManager.BP_TAManager_C|GetCheckpoint%20Sound (Variables|Default|GetManagerReference)) 1.0 1.0 0.0 0 0)))

(event EventBeginPlay
  (bind _outactors (Actor|GetAllActorsOfClass "/Game/Blueprints/DroneSim/Blueprints/TimeAttack/BP_TAManager.BP_TAManager_C"))
  (Variables|Default|SetManagerReference (Utilities|Array|Get(acopy) _outactors)))

(fn ConstructionScript)

(fn CheckTimer
  (if (== (Variables|Default|GetIndex) 0)
    (if (not (Variables|/Game/Blueprints/DroneSim/Blueprints/TimeAttack/BP_TAManager.BP_TAManager_C|GetIsTiming (Variables|Default|GetManagerReference)))
      (Default|StartTimer (Variables|Default|GetManagerReference)))))