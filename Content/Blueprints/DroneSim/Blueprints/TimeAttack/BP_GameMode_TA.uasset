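; Game mode for the drone sim's Time Attack mode that gives each joining player a pawn at their own start point.
; On PostLogin, the authority spawns the default pawn at the PlayerStart indexed by SpawnOrder, possesses it with the new controller and increments the counter.
; The index has no wrap or bounds check, and the construction script only casts the current game mode to BP_GameMode without using the result.
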(event EventPostLogin
  (params (NewPlayer :type Player%20Controller%20Object%20Reference))
  (Networking|SwitchHasAuthority
    (:Authority
      (bind _outactors (Actor|GetAllActorsOfClass "/Script/Engine.PlayerStart"))
      (bind _returnvalue (Game|SpawnActorfromClass (Variables|Default|GetDefaultPawnClass) (Transformation|GetActorTransform (Utilities|Array|Get(acopy) _outactors (Variables|Default|GetSpawnOrder))) "AdjustIfPossibleButDontSpawnIfColliding" 0 0))
      (Pawn|Possess NewPlayer _returnvalue)
      (Variables|Default|SetSpawnOrder (+ (Variables|Default|GetSpawnOrder) 1)))))

(fn ConstructionScript
  (bind _returnvalue (Game|GetGameMode))
  (Utilities|IsValid _returnvalue
    (:Is%20Valid
      (Utilities|Casting|CastToBP_GameMode _returnvalue))))