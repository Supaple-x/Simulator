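; BP_Ragdoll is an ATV vehicle actor that stands in for the driver as a physics ragdoll.
; On BeginPlay it applies the driver skeletal mesh, reinitializing the pose.
; After a short delay, it blocks all collision channels except Camera, which it ignores, and enables physics simulation.
; It then launches the body with the Impulse variable, applied as a velocity change so mass is disregarded.
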(event EventBeginPlay
  (bind _mesh (Variables|Default|GetMesh))
  ;[1 1 1] Ragdoll Begin Play
  (Class|SkinnedMeshComponent|SetSkeletalMesh (Variables|Default|GetMesh) (Variables|Default|GetDriverSkeletalMesh) true)
  (Utilities|FlowControl|Delay 0.2)
  (Collision|SetCollisionResponsetoAllChannels _mesh "ECR_Block")
  (Collision|SetCollisionResponsetoChannel _mesh "ECC_Camera" "ECR_Ignore")
  (Physics|SetSimulatePhysics (Variables|Default|GetMesh) true)
  (Physics|AddImpulse (Variables|Default|GetMesh) (Variables|Default|GetImpulse) "None" true))

(fn ConstructionScript)