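; BP_BarrierSpline is a spline actor, apparently a path for BP_Barrier actors, that can conform its points to the terrain in the editor.
; When AlignToTerrain is set, the construction script makes each point a curve type and snaps it to the hit of a vertical Visibility trace spanning TraceH above and below.
; A disconnected branch for rebuilding all BP_Barrier actors is noted as crash-prone in construction; the event graph is empty.
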(event EventBeginPlay)

(event Collision|EventActorBeginOverlap
  (params (OtherActor :type Actor%20Object%20Reference)))

(event EventTick
  (params (DeltaSeconds :type Float%20%28single-precision%29)))

(fn ConstructionScript
  (bind _trace_h (Variables|Default|GetTrace_H))
  ;[1 1 1] Add Spline Points with terrain alignment if needed
  (if (Variables|Default|GetAlignToTerrain?)
    (for _index (range 0 (Spline|GetNumberOfSplinePoints (Variables|Default|GetSpline)))
      (Spline|SetSplinePointType (Variables|Default|GetSpline) _index "Curve" true)
      (bind (_outhit _returnvalue) (Collision|LineTraceByChannel (+ (Spline|GetLocationatSplinePoint (Variables|Default|GetSpline) _index "World") (Math|Vector|MakeVector 0.0 0.0 _trace_h)) (- (Spline|GetLocationatSplinePoint (Variables|Default|GetSpline) _index "World") (Math|Vector|MakeVector 0.0 0.0 _trace_h)) "TraceTypeQuery1" false 0 "ForDuration"))
      (if _returnvalue
        (Spline|SetLocationatSplinePoint (Variables|Default|GetSpline) _index (.Location (Collision|BreakHitResult _outhit)) "World" true)))))