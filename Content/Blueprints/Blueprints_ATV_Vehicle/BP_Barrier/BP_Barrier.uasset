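; BP_Barrier places barrier meshes along every BP_BarrierSpline actor in the level using one hierarchical instanced static mesh component.
; The construction script clears and rebuilds all instances, resetting a Refresh flag that acts as an editor button.
; FAddBarrier steps along each spline at that actor's spacing, aligning instances to spline rotation.
; An optional left row is offset along the right vector by lane size, without the Z offset.
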(event Custom|CreateBarriers
  (Components|StaticMesh|SetStaticMesh (Variables|Default|GetHISMC_Barrier) (Variables|Default|GetBarrierMesh))
  (Components|InstancedStaticMesh|ClearInstances (Variables|Default|GetHISMC_Barrier))
  (bind _outactors (Actor|GetAllActorsOfClass "/Game/Blueprints/Blueprints_ATV_Vehicle/BP_Barrier/BP_BarrierSpline.BP_BarrierSpline_C"))
  (for _array_element _outactors
    (Utilities|IsValid _array_element
      (:Is%20Valid
        (CallFunction|FAddBarrier (Variables|/Game/Blueprints/Blueprints_ATV_Vehicle/BP_Barrier/BP_BarrierSpline.BP_BarrierSpline_C|GetSpline _array_element) (Variables|/Game/Blueprints/Blueprints_ATV_Vehicle/BP_Barrier/BP_BarrierSpline.BP_BarrierSpline_C|GetDistance _array_element) (Variables|/Game/Blueprints/Blueprints_ATV_Vehicle/BP_Barrier/BP_BarrierSpline.BP_BarrierSpline_C|GetLaneSize _array_element) (Variables|/Game/Blueprints/Blueprints_ATV_Vehicle/BP_Barrier/BP_BarrierSpline.BP_BarrierSpline_C|GetAddLeftBarrier? _array_element) (Variables|/Game/Blueprints/Blueprints_ATV_Vehicle/BP_Barrier/BP_BarrierSpline.BP_BarrierSpline_C|GetLeftBarrierRightVector _array_element))))))

(fn ConstructionScript
  (CallFunction|CreateBarriers)
  (if (Variables|Default|GetRefresh)
    (Variables|Default|SetRefresh false)))

(fn FAddBarrier
  (params (Target :type Spline%20Component%20Object%20Reference) (BDistance :type Float%20%28single-precision%29) (LaneSize :type Float%20%28single-precision%29) (Add%20LeftBarrier? :type Boolean) (LeftBarrierRightVector :type Float%20%28single-precision%29))
  (LocalVariables|SetLV_CurrentSpline Target)
  (Components|StaticMesh|SetStaticMesh (Variables|Default|GetHISMC_Barrier) (Variables|Default|GetBarrierMesh))
  (for _index (range 0 (Math|Float|Truncate (/ (Spline|GetSplineLength (LocalVariables|GetLV_CurrentSpline)) BDistance)))
    (LocalVariables|SetLV_CurrentSplineDistance (* _index BDistance))
    (Class|InstancedStaticMeshComponent|AddInstanceWorldSpace (Variables|Default|GetHISMC_Barrier) (Math|Transform|MakeTransform (+ (Spline|GetLocationatDistanceAlongSpline (LocalVariables|GetLV_CurrentSpline) (LocalVariables|GetLV_CurrentSplineDistance) "World") (Math|Vector|MakeVector 0.0 0.0 (Variables|Default|GetMeshZ_Offset))) (Spline|GetRotationatDistanceAlongSpline (LocalVariables|GetLV_CurrentSpline) (LocalVariables|GetLV_CurrentSplineDistance) "World") "1,1,1"))
    (if Add%20LeftBarrier?
      (Class|InstancedStaticMeshComponent|AddInstanceWorldSpace (Variables|Default|GetHISMC_Barrier) (Math|Transform|MakeTransform (+ (Spline|GetLocationatDistanceAlongSpline (LocalVariables|GetLV_CurrentSpline) (LocalVariables|GetLV_CurrentSplineDistance) "World") (* (Class|SplineComponent|GetRightVectoratDistanceAlongSpline (LocalVariables|GetLV_CurrentSpline) (LocalVariables|GetLV_CurrentSplineDistance) "World") (* LaneSize LeftBarrierRightVector)) (Math|Vector|MakeVector 0.0 0.0 0.0)) (Spline|GetRotationatDistanceAlongSpline (LocalVariables|GetLV_CurrentSpline) (LocalVariables|GetLV_CurrentSplineDistance) "World") "1,1,1")))))