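; Race track actor for the ATV game that lays out AI target nodes along a spline and provides the start/finish trigger.
; The construction script either line-traces along the spline for landscape spline meshes, adding HISM targets and moving spline points to them, or spaces targets evenly along the spline.
; The box overlap starts an ATV's race and sizes its node array to the track, then signals lap completion on later overlaps.
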(event OnComponentBeginOverlap(Box)
  (params (OverlappedComponent :type Primitive%20Component%20Object%20Reference) (OtherActor :type Actor%20Object%20Reference) (OtherComp :type Primitive%20Component%20Object%20Reference) (OtherBodyIndex :type Integer) (bFromSweep :type Boolean) (SweepResult :type Hit%20Result%20Structure%20%28by%20ref%29))
  ;[1 1 1] This is the starting gate box overlap that will trigger an event on the atv
  (bind _asbp_atv (Utilities|Casting|CastToBP_ATV OtherActor))
  (if (Variables|/Game/Blueprints/Blueprints_ATV_Vehicle/ATV/Blueprints/BP_ATV.BP_ATV_C|GetRaceStarted _asbp_atv)
    (Default|CallEDLapCompleted _asbp_atv _asbp_atv)
    (else
      (Variables|/Game/Blueprints/Blueprints_ATV_Vehicle/ATV/Blueprints/BP_ATV.BP_ATV_C|SetRaceStarted _asbp_atv true)
      (for _index (range 0 (Variables|Default|GetNodesCreated))
        (Utilities|Array|SetArrayElem (Variables|/Game/Blueprints/Blueprints_ATV_Vehicle/ATV/Blueprints/BP_ATV.BP_ATV_C|GetFoundInstances _asbp_atv) _index false true)))))

(fn ConstructionScript
  (bind _spline1 (Variables|Default|GetSpline1))
  (bind _tracedistancelandscapesplines (Variables|Default|GetTraceDistanceLandscapeSplines))
  (bind _returnvalue (Spline|GetSplineLength _spline1))
  (if (Variables|Default|GetLandscapeSplineTrack?)
    ;[1 1 1] The track can be created using landscape spline components. this is made using this function
    ;;[1 1 1] Clear all found spline mesh components
    (Utilities|Array|Clear (Variables|Default|GetFoundSplineMeshC))
    (Utilities|Array|Resize (Variables|Default|GetFoundSplineMeshC) 0)
    (for _index (range 0 (Math|Float|Truncate (/ (Spline|GetSplineLength (Variables|Default|GetSpline1)) (Variables|Default|GetCheckDistance))))
      ;;[1 1 1] If the trace finds a spline mesh component it adds it to the array
      (bind (_outhit _returnvalue_2) (Collision|LineTraceByChannel (+ (Spline|GetLocationatDistanceAlongSpline (Variables|Default|GetSpline1) (* _index (Variables|Default|GetCheckDistance)) "World") (Math|Vector|MakeVector 0.0 0.0 _tracedistancelandscapesplines)) (- (Spline|GetLocationatDistanceAlongSpline (Variables|Default|GetSpline1) (* _index (Variables|Default|GetCheckDistance)) "World") (Math|Vector|MakeVector 0.0 0.0 _tracedistancelandscapesplines)) "TraceTypeQuery1" true 0 "ForOneFrame"))
      (if _returnvalue_2
        (bind _asspline_mesh_component (Utilities|Casting|CastToSplineMeshComponent (.HitComponent (Collision|BreakHitResult _outhit))))
        (Utilities|Array|AddUnique (Variables|Default|GetFoundSplineMeshC) _asspline_mesh_component)))
    ;;[1 1 1] For all components add an instance of the hismc that is used as target for the AI
    (for (_array_element _array_index) (Variables|Default|GetFoundSplineMeshC)
      (Class|InstancedStaticMeshComponent|AddInstanceWorldSpace (Variables|Default|GetHISMC_AI_TARGET) (Math|Transform|MakeTransform (+ (Transformation|GetWorldLocation _array_element) (Math|Vector|MakeVector 0.0 0.0 (Variables|Default|GetSplineZOffset))) "0, 0, 0" "1,1,1"))
      (if (!= _array_index 0)
        (Spline|SetLocationatSplinePoint (Variables|Default|GetSpline1) _array_index (Transformation|GetWorldLocation _array_element) "World" true)))
    (else
      ;[1 1 1] If you don't want to use landscape splines you can manually set the track
      (for _index_2 (range 0 (Math|Float|Truncate (/ (Spline|GetSplineLength (Variables|Default|GetSpline1)) (Variables|Default|GetCheckDistance))))
        (Class|InstancedStaticMeshComponent|AddInstanceWorldSpace (Variables|Default|GetHISMC_AI_TARGET) (Math|Transform|MakeTransform (Spline|GetLocationatDistanceAlongSpline (Variables|Default|GetSpline1) (* _index_2 (Variables|Default|GetCheckDistance)) "World") (Spline|GetRotationatDistanceAlongSpline (Variables|Default|GetSpline1) (Variables|Default|GetCheckDistance) "World") "1,1,1")))))
  ;[1 1 1] These are values to monitor your race track length
  (Variables|Default|SetTotalTrackDistanceCM _returnvalue)
  (Variables|Default|SetTrackLen%28ReadOnly%29 (Math|Conversions|ToFloat(Integer) (Math|Float|Round (/ _returnvalue 1e+02))))
  (Variables|Default|SetNodesCreated (Components|InstancedStaticMesh|GetInstanceCount (Variables|Default|GetHISMC_AI_TARGET)))
  (Components|Box|SetBoxExtent (Variables|Default|GetBox) (Variables|Default|GetStartingTriggerSize) true)
  (Transformation|SetRelativeRotation (Variables|Default|GetBox) (Math|Rotator|MakeRotator 0.0 0.0 (Variables|Default|GetStartingTriggerRotation_Z)) false false))