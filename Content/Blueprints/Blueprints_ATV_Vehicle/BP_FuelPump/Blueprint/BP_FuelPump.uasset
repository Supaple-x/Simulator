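; Two-sided fuel pump that automatically refuels BP_ATV vehicles stopped beside it.
; A one-second looping timer sphere-traces each side, adding fuel until the detected ATV is full, then resetting that side's handle.
; A fast timer snaps each active handle to one of the ATV's two refill arrows, chosen by the angle between vehicle and pump facing.
; The construction script resets both handles and places instanced meshes at regular intervals along a spline.
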(event Custom|CheckForATVS
  (CallFunction|FCheckR)
  (CallFunction|FCheckL))

(event Custom|MoveHandles
  ;[1 1 1] When Refilling the two fuel pumps are moved
  (CallFunction|FMoveHandleR)
  (CallFunction|FMoveHandleL))

(event EventBeginPlay
  ;[1 1 1] On Begin Play
  ;[1 1 1] CheckerTimer
  (Utilities|Time|SetTimerbyEvent (delegate Custom|CheckForATVS) 1.0 true)
  ;[1 1 1] Movement Timer
  (Utilities|Time|SetTimerbyEvent (delegate Custom|MoveHandles) 0.01 true))

(fn ConstructionScript
  (bind _nodesdistance (Variables|Default|GetNodesDistance))
  (bind _splinepath (Variables|Default|GetSplinePath))
  (Transformation|SetRelativeLocation (Variables|Default|GetSplinePath) (Variables|Default|GetPathStart) false false)
  (CallFunction|FReset1)
  (CallFunction|FReset2)
  (for _index (range 0 (Math|Float|Truncate (/ (Spline|GetSplineLength (Variables|Default|GetSplinePath)) (Variables|Default|GetNodesDistance))))
    (Class|InstancedStaticMeshComponent|AddInstanceWorldSpace (Variables|Default|GetHierarchicalInstancedStaticMesh) (Math|Transform|MakeTransform (Spline|GetLocationatDistanceAlongSpline _splinepath (* _index _nodesdistance) "World") (Spline|GetRotationatDistanceAlongSpline _splinepath _nodesdistance "World") "1,1,1"))))

(fn FReset1
  (bind _arrowstart1 (Variables|Default|GetArrowStart1))
  (bind _returnvalue (Transformation|GetWorldTransform _arrowstart1))
  (bind (_location _rotation) (Math|Transform|BreakTransform _returnvalue))
  (Transformation|SetWorldLocationAndRotation (Variables|Default|GetSM_FuelPump_Handle) _location _rotation false true))

(fn FReset2
  (bind _arrowstart2 (Variables|Default|GetArrowStart2))
  (bind _returnvalue (Transformation|GetWorldTransform _arrowstart2))
  (bind (_location _rotation) (Math|Transform|BreakTransform _returnvalue))
  (Transformation|SetWorldLocationAndRotation (Variables|Default|GetSM_FuelPump_Handle2) _location _rotation false true))

(fn FRefill
  (params (ATV :type BP%20ATV%20Object%20Reference))
  (Default|EventRestoreFuel ATV (Math|Integer|Clamp(Integer) (+ (Variables|/Game/Blueprints/Blueprints_ATV_Vehicle/ATV/Blueprints/BP_ATV.BP_ATV_C|GetFuel ATV) (Variables|Default|GetRefillAmountPerSec)) 0 (Variables|/Game/Blueprints/Blueprints_ATV_Vehicle/ATV/Blueprints/BP_ATV.BP_ATV_C|GetMaxFuel ATV))))

(fn FCheckR
  (bind _arrowcheck1 (Variables|Default|GetArrowCheck1))
  (bind _returnvalue (Transformation|GetWorldLocation _arrowcheck1))
  ;[1 1 1] From the Arrow 1 performs a sphere trace for objects (pawn) and check for atvs. If it founds one then it starts refilling. If fuel is greater than max fuel it stops refilling
  (bind (_outhit _returnvalue_2) (Collision|SphereTraceForObjects _returnvalue (+ _returnvalue "0.100000,0.100000,0.100000") (Variables|Default|GetSearchRadius) (Utilities|Array|MakeArray "ObjectTypeQuery3") false 0 "ForDuration"))
  (if _returnvalue_2
    (bind _asbp_atv (Utilities|Casting|CastToBP_ATV (.HitActor (Collision|BreakHitResult _outhit))))
    (Variables|Default|SetCurrentATV_R _asbp_atv)
    (if (< (Variables|/Game/Blueprints/Blueprints_ATV_Vehicle/ATV/Blueprints/BP_ATV.BP_ATV_C|GetFuel (Variables|Default|GetCurrentATV_R)) (Variables|/Game/Blueprints/Blueprints_ATV_Vehicle/ATV/Blueprints/BP_ATV.BP_ATV_C|GetMaxFuel (Variables|Default|GetCurrentATV_R)))
      (CallFunction|FRefill (Variables|Default|GetCurrentATV_R))
      (if (>= (Variables|/Game/Blueprints/Blueprints_ATV_Vehicle/ATV/Blueprints/BP_ATV.BP_ATV_C|GetFuel (Variables|Default|GetCurrentATV_R)) (Variables|/Game/Blueprints/Blueprints_ATV_Vehicle/ATV/Blueprints/BP_ATV.BP_ATV_C|GetMaxFuel (Variables|Default|GetCurrentATV_R)))
        (CallFunction|FReset1 :!label _label)
        (Variables|Default|SetCurrentATV_R 0))
      (else
        (goto _label)))
    (else
      (goto _label))))

(fn FCheckL
  (bind _arrowcheck2 (Variables|Default|GetArrowCheck2))
  (bind _returnvalue (Transformation|GetWorldLocation _arrowcheck2))
  ;[1 1 1] From the Arrow 2 performs a sphere trace for objects (pawn) and check for atvs. If it founds one then it starts refilling. If fuel is greater than max fuel it stops refilling
  (bind (_outhit _returnvalue_2) (Collision|SphereTraceForObjects _returnvalue (+ _returnvalue "0.100000,0.100000,0.100000") (Variables|Default|GetSearchRadius) (Utilities|Array|MakeArray "ObjectTypeQuery3") false 0 "ForDuration"))
  (if _returnvalue_2
    (bind _asbp_atv (Utilities|Casting|CastToBP_ATV (.HitActor (Collision|BreakHitResult _outhit))))
    (Variables|Default|SetCurrentATV_L _asbp_atv)
    (if (< (Variables|/Game/Blueprints/Blueprints_ATV_Vehicle/ATV/Blueprints/BP_ATV.BP_ATV_C|GetFuel (Variables|Default|GetCurrentATV_L)) (Variables|/Game/Blueprints/Blueprints_ATV_Vehicle/ATV/Blueprints/BP_ATV.BP_ATV_C|GetMaxFuel (Variables|Default|GetCurrentATV_L)))
      (CallFunction|FRefill (Variables|Default|GetCurrentATV_L))
      (if (>= (Variables|/Game/Blueprints/Blueprints_ATV_Vehicle/ATV/Blueprints/BP_ATV.BP_ATV_C|GetFuel (Variables|Default|GetCurrentATV_L)) (Variables|/Game/Blueprints/Blueprints_ATV_Vehicle/ATV/Blueprints/BP_ATV.BP_ATV_C|GetMaxFuel (Variables|Default|GetCurrentATV_L)))
        (CallFunction|FReset2 :!label _label)
        (Variables|Default|SetCurrentATV_L 0))
      (else
        (goto _label)))
    (else
      (goto _label))))

(fn FMoveHandleR
  (bind _currentatv_r (Variables|Default|GetCurrentATV_R))
  (bind _arrowcheck1 (Variables|Default|GetArrowCheck1))
  (bind _currentatv_r_2 (Variables|Default|GetCurrentATV_R))
  (bind _returnvalue (Math|Vector|GetForwardVector _arrowcheck1))
  (bind _arrowrefillpoint (Variables|/Game/Blueprints/Blueprints_ATV_Vehicle/ATV/Blueprints/BP_ATV.BP_ATV_C|GetArrowRefillPoint _currentatv_r_2))
  (bind _arrowrefill_l (Variables|/Game/Blueprints/Blueprints_ATV_Vehicle/ATV/Blueprints/BP_ATV.BP_ATV_C|GetArrowRefill_L _currentatv_r_2))
  (bind _sm_atv_body (Variables|/Game/Blueprints/Blueprints_ATV_Vehicle/ATV/Blueprints/BP_ATV.BP_ATV_C|GetSM_ATV_Body _currentatv_r))
  (bind _returnvalue_2 (Math|Vector|GetForwardVector _sm_atv_body))
  (bind _returnvalue_3 (Math|Vector|DotProduct _returnvalue_2 _returnvalue))
  (bind _returnvalue_4 (Class|KismetMathLibrary|DegAcos _returnvalue_3))
  (bind _returnvalue_5 (Math|Float|Absolute(Float) _returnvalue_4))
  (bind _returnvalue_6 (> _returnvalue_5 9e+01))
  (bind _returnvalue_7 (select _returnvalue_6 _arrowrefill_l _arrowrefillpoint))
  (bind _returnvalue_8 (Transformation|GetWorldTransform _returnvalue_7))
  (bind (_location _rotation) (Math|Transform|BreakTransform _returnvalue_8))
  (Utilities|IsValid (Variables|Default|GetCurrentATV_R)
    (:Is%20Valid
      (Transformation|SetWorldLocationAndRotation (Variables|Default|GetSM_FuelPump_Handle) _location _rotation false true))))

(fn FMoveHandleL
  (bind _currentatv_l (Variables|Default|GetCurrentATV_L))
  (bind _arrowcheck2 (Variables|Default|GetArrowCheck2))
  (bind _currentatv_l_2 (Variables|Default|GetCurrentATV_L))
  (bind _returnvalue (Math|Vector|GetForwardVector _arrowcheck2))
  (bind _arrowrefillpoint (Variables|/Game/Blueprints/Blueprints_ATV_Vehicle/ATV/Blueprints/BP_ATV.BP_ATV_C|GetArrowRefillPoint _currentatv_l_2))
  (bind _arrowrefill_l (Variables|/Game/Blueprints/Blueprints_ATV_Vehicle/ATV/Blueprints/BP_ATV.BP_ATV_C|GetArrowRefill_L _currentatv_l_2))
  (bind _sm_atv_body (Variables|/Game/Blueprints/Blueprints_ATV_Vehicle/ATV/Blueprints/BP_ATV.BP_ATV_C|GetSM_ATV_Body _currentatv_l))
  (bind _returnvalue_2 (Math|Vector|GetForwardVector _sm_atv_body))
  (bind _returnvalue_3 (Math|Vector|DotProduct _returnvalue_2 _returnvalue))
  (bind _returnvalue_4 (Class|KismetMathLibrary|DegAcos _returnvalue_3))
  (bind _returnvalue_5 (Math|Float|Absolute(Float) _returnvalue_4))
  (bind _returnvalue_6 (> _returnvalue_5 9e+01))
  (bind _returnvalue_7 (select _returnvalue_6 _arrowrefillpoint _arrowrefill_l))
  (bind _returnvalue_8 (Transformation|GetWorldTransform _returnvalue_7))
  (bind (_location _rotation) (Math|Transform|BreakTransform _returnvalue_8))
  (Utilities|IsValid (Variables|Default|GetCurrentATV_L)
    (:Is%20Valid
      (Transformation|SetWorldLocationAndRotation (Variables|Default|GetSM_FuelPump_Handle2) _location _rotation false true))))