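; Game mode for the drone simulation that spawns and possesses each joining player's chosen pawn: a drone, copter, SWAT character or ATV.
; After a short delay, PostLogin claims a free SpawnPoint, or creates one at the level's data-table start point, and spawns by the GameInstance's character index.
; BeginPlay hides target point actors.
; Helper functions send uncontrolled drones to a target location as a formation and update their trace data.
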(event EventBeginPlay
  (bind _outactors (Actor|GetAllActorsOfClass "/Game/Blueprints/DronesGroup_Blueprints/TargetPoints/TargetPoint_Actor.TargetPoint_Actor_C"))
  (for _array_element _outactors
    (Rendering|SetActorHiddenInGame _array_element true)))

(event EventPostLogin
  (params (NewPlayer :type Player%20Controller%20Object%20Reference))
  (Utilities|FlowControl|Delay 1.0)
  (bind _output_get (Variables|Default|SetSelectedSpawnPoint (CallFunction|FindFreeSpawnPoint)))
  (Utilities|IsValid _output_get
    (:Is%20Valid
      (Variables|/Game/Blueprints/DroneSim/Blueprints/SpawnPoint.SpawnPoint_C|SetbIsTaken (Variables|Default|GetSelectedSpawnPoint) true)
      (bind _aspmm_game_instance (Utilities|Casting|CastToPMM_GameInstance (Game|GetGameInstance)))
      (switch int (Variables|/Game/UI/ProMainMenuKit/Blueprints/PMM_GameInstance.PMM_GameInstance_C|GetSelectedCharacterIndex _aspmm_game_instance)
        (:0
          (bind _returnvalue (Game|SpawnActorfromClass "/Game/Blueprints/DroneSim/Blueprints/BP_Drone_01.BP_Drone_01_C" (Math|Transform|MakeTransform (Transformation|GetActorLocation (Variables|Default|GetSelectedSpawnPoint)) (Transformation|GetActorRotation (Variables|Default|GetSelectedSpawnPoint)) "1,1,1") "Undefined" 0 0 (Variables|Default|GetSelectedSpawnPoint) false true 0 :!label _label))
          (Pawn|Possess NewPlayer _returnvalue))
        (:1
          (goto _label))
        (:2
          (bind _returnvalue_2 (Game|SpawnActorfromClass "/Game/Blueprints/Swat_Soldier/Blueprint/SWAT_Character.SWAT_Character_C" (Math|Transform|MakeTransform (Transformation|GetActorLocation (Variables|Default|GetSelectedSpawnPoint)) (Transformation|GetActorRotation (Variables|Default|GetSelectedSpawnPoint)) "1,1,1") "Undefined" 0 0))
          (Pawn|Possess NewPlayer _returnvalue_2)
          (Variables|/Script/Engine.PlayerController|SetbShowMouseCursor NewPlayer false))
        (:3
          (bind _returnvalue_3 (Game|SpawnActorfromClass "/Game/Blueprints/Blueprints_ATV_Vehicle/ATV/Blueprints/BP_ATV.BP_ATV_C" (Math|Transform|MakeTransform (Transformation|GetActorLocation (Variables|Default|GetSelectedSpawnPoint)) (Transformation|GetActorRotation (Variables|Default|GetSelectedSpawnPoint)) "1,1,1") "Undefined" 0 false false (Variables|Default|GetSelectedSpawnPoint) 0))
          (Pawn|Possess NewPlayer _returnvalue_3))
        (:4
          (bind _returnvalue_4 (Game|SpawnActorfromClass "/Game/Meshes/Drones/Drones_New/BP/DJI_Copter_BP.DJI_Copter_BP_C" (Math|Transform|MakeTransform (Transformation|GetActorLocation (Variables|Default|GetSelectedSpawnPoint)) (Transformation|GetActorRotation (Variables|Default|GetSelectedSpawnPoint)) "1,1,1") "AlwaysSpawn" 0 0 (Variables|Default|GetSelectedSpawnPoint) false true 0))
          (Pawn|Possess NewPlayer _returnvalue_4))
        (:5
          (bind _returnvalue_5 (Game|SpawnActorfromClass "/Game/Meshes/Drones/Drones_New/BP/T1_Copter_BP.T1_Copter_BP_C" (Math|Transform|MakeTransform (Transformation|GetActorLocation (Variables|Default|GetSelectedSpawnPoint)) (Transformation|GetActorRotation (Variables|Default|GetSelectedSpawnPoint)) "1,1,1") "AlwaysSpawn" 0 0 (Variables|Default|GetSelectedSpawnPoint) false true 0))
          (Pawn|Possess NewPlayer _returnvalue_5))))))

(fn ConstructionScript)

(fn CreateAIFormation
  (bind _outactors (Actor|GetAllActorsOfClass "/Game/Blueprints/DroneSim/Blueprints/BP_Drone_01.BP_Drone_01_C"))
  (bind _outactors_2 (Actor|GetAllActorsOfClass "/Game/Blueprints/DroneAI/TargetLocation.TargetLocation_C"))
  (for _array_element _outactors
    (if (not (Class|Pawn|IsControlled _array_element))
      (Utilities|Array|Add (Variables|Default|GetDronesInFormation) _array_element)
      (Default|FlyingAIMovetoGivenPoint _array_element (Transformation|GetActorLocation (Utilities|Array|Get(acopy) _outactors_2))))))

(fn UpdateDronesTraceData
  (for (_array_element _array_index) (Variables|Default|GetDronesInFormation)
    (Class|CPPFuncLib|UpdateDroneTracesData (+ _array_index 1) (Variables|/Game/Blueprints/DroneSim/Blueprints/BP_Drone_01.BP_Drone_01_C|GetLocationData _array_element))))

(fn FindFreeSpawnPoint
  (bind _outactors (Actor|GetAllActorsOfClass "/Game/Blueprints/DroneSim/Blueprints/SpawnPoint.SpawnPoint_C"))
  (bind _array_element (Utilities|Array|ForEachLoopwithBreak _outactors)
    (:LoopBody
      (if (not (Variables|/Game/Blueprints/DroneSim/Blueprints/SpawnPoint.SpawnPoint_C|GetbIsTaken _array_element))
        (return _array_element)))
    (:Completed
      (bind _returnvalue (Utilities|GetDataTableRow "/Game/DMA/Data/DT_MapperLevelData.DT_MapperLevelData" (Variables|/Script/Kulagin.MapperGameInstance|GetLevelName (Class|KulaginStatics|GetMapperGameInstance)))
        (:then
          (LocalVariables|SetSpawnPointLoc (.startpoint _returnvalue)))
        (:RowNotFound
          (LocalVariables|SetSpawnPointLoc "0, 0, 0")))
      (bind _returnvalue_2 (Game|SpawnActorfromClass "/Game/Blueprints/DroneSim/Blueprints/SpawnPoint.SpawnPoint_C" (Math|Transform|MakeTransform (LocalVariables|GetSpawnPointLoc) "0, 0, 0" "1,1,1") "AlwaysSpawn" 0 0))
      (return _returnvalue_2))))